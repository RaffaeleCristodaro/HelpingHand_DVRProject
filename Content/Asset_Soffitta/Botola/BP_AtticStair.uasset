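; Attic hatch stair that starts by playing its close animation and can be opened once through an event.
; Opening plays the open animation and a sound, then sets a flag that Tick polls.
; Tick then drives timelines setting spot and point light intensities, clears the flag when the point light timeline finishes, and destroys the Cube component once.
; Focus events toggle custom depth on the stair mesh for highlighting.
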(event Custom|EventCloseBotola
  ;[1 1 1] Animation and Sound
  (Utilities|FlowControl|DoOnce false
    (:Completed
      (Components|Animation|PlayAnimation (Variables|Default|GetSM_AtticStair) "/Game/Asset_Soffitta/Botola/Anim_AtticStair_Close.Anim_AtticStair_Close" false))))

(event Custom|EventOpenBotola
  ;[1 1 1] Animation and Sound
  (Utilities|FlowControl|DoOnce false
    (:Completed
      (Components|Animation|PlayAnimation (Variables|Default|GetSM_AtticStair) "/Game/Asset_Soffitta/Botola/Anim_AtticStair_Open.Anim_AtticStair_Open" false)
      (Audio|PlaySoundatLocation 0 "0, 0, 0" "0, 0, 0" 1.0 1.0 0.0 0 0 0 0)
      (Variables|Default|SetActivateLight? true))))

(event EventTick
  (params (DeltaSeconds :type Float%20%28single-precision%29))
  (bind _spotlight (Variables|Default|GetSpotLight))
  ;[1 1 1] Event tick
  (if (Variables|Default|GetActivateLight?)
    (Utilities|FlowControl|Sequence
      (:then_0
        (bind _lightintensity (Timeline|SpotLightIntensity Play)
          (:Update
            (Utilities|IsValid _spotlight
              (:Is%20Valid
                (Rendering|Components|Light|SetIntensity (Variables|/Script/Engine.Light|GetLightComponent _spotlight) _lightintensity))))))
      (:then_1
        (for _array_element (Variables|Default|GetPointsLight)
          (bind _lightintensity_2 (Timeline|PointLightIntensity Play)
            (:Update
              (Utilities|IsValid _array_element
                (:Is%20Valid
                  (Rendering|Components|Light|SetIntensity (Variables|/Script/Engine.Light|GetLightComponent _array_element) _lightintensity_2))))
            (:Finished
              (Variables|Default|SetActivateLight? false)))))
      (:then_2
        (Utilities|FlowControl|DoOnce false
          (:Completed
            (Components|DestroyComponent (Variables|Default|GetCube))))))))

(event EventBeginPlay
  ;[1 1 1] Initialize
  (CallFunction|EventCloseBotola))

(fn ConstructionScript)

(fn BeginFocus
  (Rendering|SetRenderCustomDepth (Variables|Default|GetSM_AtticStair) true))

(fn EndFocus
  (Rendering|SetRenderCustomDepth (Variables|Default|GetSM_AtticStair) false))