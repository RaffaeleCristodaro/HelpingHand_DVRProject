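; BP_InteractiveGrabbablesParent is a parent Blueprint for interactive grabbable objects, holding the start state needed for respawning.
; SetRespawnVariables caches the location, rotation and scale of both the actor and its StaticMesh component in world space, storing the two separately.
; The construction script is empty, and this file shows neither the caller of that function nor the grab and respawn logic.
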(fn ConstructionScript)

(fn SetRespawnVariables
  (Variables|Default|SetActorStartLocation (Transformation|GetActorLocation))
  (Variables|Default|SetActorStartRotation (Transformation|GetActorRotation))
  (Variables|Default|SetPrimitiveComponentStartLocation (Transformation|GetWorldLocation (Variables|Default|GetStaticMesh)))
  (Variables|Default|SetPrimitiveComponentStartRotation (Transformation|GetWorldRotation (Variables|Default|GetStaticMesh)))
  (Variables|Default|SetActorInitialStartScale (Transformation|GetActorScale3D))
  (Variables|Default|SetComponentStaticMeshInitialStartScale (Transformation|GetWorldScale (Variables|Default|GetStaticMesh)))
  (return))