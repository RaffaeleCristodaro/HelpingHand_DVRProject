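; Piano actor with three keys, Do, Re and Mi, that sink and play their notes when Player 1 overlaps their collision.
; Each Tick checks every key's overlap and uses MoveComponentTo to ease the button down or back up, clamped between shared min and max offsets.
; A DoOnce per key fires its 2D sound once the clamped target reaches the halfway point, and re-arms when the target returns to the top.
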(event EventBeginPlay
  ;[1 1 1] Initialize
  (bind _pg1 (CallFunction|GetPlayer1))
  (Variables|Default|SetPG1 _pg1))

(event EventTick
  (params (DeltaSeconds :type Float%20%28single-precision%29))
  (bind _maxoffsetbuttons (Variables|Default|GetMaxOffsetButtons))
  (bind _minoffsetbuttons (Variables|Default|GetMinOffsetButtons))
  (bind _minoffsetbuttons_2 (Variables|Default|GetMinOffsetButtons))
  (bind _maxoffsetbuttons_2 (Variables|Default|GetMaxOffsetButtons))
  (bind _button_mi (Variables|Default|GetButton_Mi))
  (bind _button_mi_2 (Variables|Default|GetButton_Mi))
  (bind _minoffsetbuttons_3 (Variables|Default|GetMinOffsetButtons))
  (bind _maxoffsetbuttons_3 (Variables|Default|GetMaxOffsetButtons))
  (bind _maxoffsetbuttons_4 (Variables|Default|GetMaxOffsetButtons))
  (bind _minoffsetbuttons_4 (Variables|Default|GetMinOffsetButtons))
  (bind _maxoffsetbuttons_5 (Variables|Default|GetMaxOffsetButtons))
  (bind _minoffsetbuttons_5 (Variables|Default|GetMinOffsetButtons))
  (bind _maxoffsetbuttons_6 (Variables|Default|GetMaxOffsetButtons))
  (bind _button_re (Variables|Default|GetButton_Re))
  (bind _button_re_2 (Variables|Default|GetButton_Re))
  (bind _button_do (Variables|Default|GetButton_Do))
  (bind _button_do_2 (Variables|Default|GetButton_Do))
  (bind _minoffsetbuttons_6 (Variables|Default|GetMinOffsetButtons))
  (bind _returnvalue (Transformation|GetRelativeTransform _button_do))
  (bind _returnvalue_2 (Transformation|GetRelativeTransform _button_do_2))
  (bind _returnvalue_3 (Transformation|GetRelativeTransform _button_mi))
  (bind _returnvalue_4 (Transformation|GetRelativeTransform _button_mi_2))
  (bind _returnvalue_5 (Transformation|GetRelativeTransform _button_re))
  (bind _returnvalue_6 (Transformation|GetRelativeTransform _button_re_2))
  (bind _returnvalue_7 (+ (.location _returnvalue) "0.000000,0.000000,3.000000"))
  (bind _returnvalue_8 (- (.location _returnvalue_3) "0.000000,0.000000,3.000000"))
  (bind _returnvalue_9 (+ (.location _returnvalue_4) "0.000000,0.000000,3.000000"))
  (bind _returnvalue_10 (- (.location _returnvalue_5) "0.000000,0.000000,3.000000"))
  (bind _returnvalue_11 (+ (.location _returnvalue_6) "0.000000,0.000000,3.000000"))
  (bind _returnvalue_12 (- (.location _returnvalue_2) "0.000000,0.000000,3.000000"))
  (bind _returnvalue_13 (Math|Float|Clamp(Float) (.z _returnvalue_7) _minoffsetbuttons_2 _maxoffsetbuttons_2))
  (bind _returnvalue_14 (Math|Float|Clamp(Float) (.z _returnvalue_12) _minoffsetbuttons _maxoffsetbuttons))
  (bind _returnvalue_15 (Math|Float|Clamp(Float) (.z _returnvalue_8) _minoffsetbuttons_6 _maxoffsetbuttons_4))
  (bind _returnvalue_16 (Math|Float|Clamp(Float) (.z _returnvalue_9) _minoffsetbuttons_3 _maxoffsetbuttons_3))
  (bind _returnvalue_17 (Math|Float|Clamp(Float) (.z _returnvalue_10) _minoffsetbuttons_5 _maxoffsetbuttons_6))
  (bind _returnvalue_18 (Math|Float|Clamp(Float) (.z _returnvalue_11) _minoffsetbuttons_4 _maxoffsetbuttons_5))
  ;[1 1 1] Event tick
  (Utilities|FlowControl|Sequence
    (:then_0
      (if (Collision|IsOverlappingActor (Variables|Default|GetCollision_Mi) (Variables|Default|GetPG1) :!class /Script/Engine.PrimitiveComponent)
        (Components|MoveComponentTo _button_mi (Math|Vector|MakeVector (.x _returnvalue_8) (.y _returnvalue_8) _returnvalue_15) (.rotation _returnvalue_3) false true (Variables|Default|GetOver%20Time) false)
        (if (<= _returnvalue_15 (/ (+ (Variables|Default|GetMinOffsetButtons) (Variables|Default|GetMaxOffsetButtons)) 2.0))
          (Utilities|FlowControl|DoOnce false :!label _label
            (:Completed
              (Audio|PlaySound2D "/Game/Blueprint_Grabbable/BP_Piano/3-Mi.3-Mi" 1.0 1.0 0.0 0 0))))
        (else
          (Components|MoveComponentTo _button_mi_2 (Math|Vector|MakeVector (.x _returnvalue_9) (.y _returnvalue_9) _returnvalue_16) (.rotation _returnvalue_4) false true (Variables|Default|GetOver%20Time) false)
          (if (>= _returnvalue_16 (Variables|Default|GetMaxOffsetButtons))
            (goto _label Reset)))))
    (:then_1
      (if (Collision|IsOverlappingActor (Variables|Default|GetCollision_Re) (Variables|Default|GetPG1) :!class /Script/Engine.PrimitiveComponent)
        (Components|MoveComponentTo _button_re (Math|Vector|MakeVector (.x _returnvalue_10) (.y _returnvalue_10) _returnvalue_17) (.rotation _returnvalue_5) false true (Variables|Default|GetOver%20Time) false)
        (if (<= _returnvalue_17 (/ (+ (Variables|Default|GetMinOffsetButtons) (Variables|Default|GetMaxOffsetButtons)) 2.0))
          (Utilities|FlowControl|DoOnce false :!label _label_2
            (:Completed
              (Audio|PlaySound2D "/Game/Blueprint_Grabbable/BP_Piano/2-Re.2-Re" 1.0 1.0 0.0 0 0))))
        (else
          (Components|MoveComponentTo _button_re_2 (Math|Vector|MakeVector (.x _returnvalue_11) (.y _returnvalue_11) _returnvalue_18) (.rotation _returnvalue_6) false true (Variables|Default|GetOver%20Time) false)
          (if (>= _returnvalue_18 (Variables|Default|GetMaxOffsetButtons))
            (goto _label_2 Reset)))))
    (:then_2
      (if (Collision|IsOverlappingActor (Variables|Default|GetCollision_Do) (Variables|Default|GetPG1) :!class /Script/Engine.PrimitiveComponent)
        (Components|MoveComponentTo _button_do_2 (Math|Vector|MakeVector (.x _returnvalue_12) (.y _returnvalue_12) _returnvalue_14) (.rotation _returnvalue_2) false true (Variables|Default|GetOver%20Time) false)
        (if (<= _returnvalue_14 (/ (+ (Variables|Default|GetMinOffsetButtons) (Variables|Default|GetMaxOffsetButtons)) 2.0))
          (Utilities|FlowControl|DoOnce false :!label _label_3
            (:Completed
              (Audio|PlaySound2D "/Game/Blueprint_Grabbable/BP_Piano/1-Do.1-Do" 1.0 1.0 0.0 0 0))))
        (else
          (Components|MoveComponentTo _button_do (Math|Vector|MakeVector (.x _returnvalue_7) (.y _returnvalue_7) _returnvalue_13) (.rotation _returnvalue) false true (Variables|Default|GetOver%20Time) false)
          (if (>= _returnvalue_13 (Variables|Default|GetMaxOffsetButtons))
            (goto _label_3 Reset)))))))

(fn ConstructionScript)