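; MainMenuUISpawner_BP is an actor that creates the main menu widget when play begins.
; BeginPlay reads GiocoHasBeenStarted from the GI_HelpingHand game instance, but both branches identically create a MainMenu_WG and assign it to UiSwitch through SetWidget.
; A DestroyMainMenuWidget event removes the menu by destroying the whole spawner actor.
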(event Custom|DestroyMainMenuWidget
  (bind _self self)
  ;[1 1 1] Destroy main menu
  (Utilities|IsValid _self
    (:Is%20Valid
      (Actor|DestroyActor _self))))

(event EventBeginPlay
  (bind _asgi_helping_hand (Utilities|Casting|CastToGI_HelpingHand (Game|GetGameInstance)))
  (if (Variables|/Game/Managers/GI_HelpingHand.GI_HelpingHand_C|GetGiocoHasBeenStarted? _asgi_helping_hand)
    (bind _mainmenúwidget (CallFunction|GetUiSwitch))
    (bind _returnvalue (UserInterface|CreateWidget "/Game/UIBlueprints/MainMenu/MainMenu_WG.MainMenu_WG_C"))
    (UserInterface|SetWidget _mainmenúwidget _returnvalue)
    (else
      (bind _mainmenúwidget_2 (CallFunction|GetUiSwitch))
      (bind _returnvalue_2 (UserInterface|CreateWidget "/Game/UIBlueprints/MainMenu/MainMenu_WG.MainMenu_WG_C"))
      (UserInterface|SetWidget _mainmenúwidget_2 _returnvalue_2))))

(fn ConstructionScript)