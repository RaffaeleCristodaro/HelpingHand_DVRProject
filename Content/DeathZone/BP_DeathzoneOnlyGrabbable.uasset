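; Death zone actor that respawns grabbable objects when they overlap its Box.
; Interactive grabbables are handed to the Game Manager for respawn and have their overlay material cleared.
; Rune mode tutorial spheres get special handling: overlay cleared, actor and sphere teleported to their stored start transforms, and linear velocity zeroed.
; A deactivation event switches the zone off by destroying the Box component.
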(event OnComponentBeginOverlap(Box)
  (params (OverlappedComponent :type Primitive%20Component%20Object%20Reference) (OtherActor :type Actor%20Object%20Reference) (OtherComp :type Primitive%20Component%20Object%20Reference) (OtherBodyIndex :type Integer) (bFromSweep :type Boolean) (SweepResult :type Hit%20Result%20Structure%20%28by%20ref%29))
  ;[1 1 1] Deathzone collisions
  (bind _asbp_interactive_grabbables_parent (Utilities|Casting|CastToBP_InteractiveGrabbablesParent OtherActor)
    (:then
      (Default|RespawnGrabbables (Variables|Default|GetGame%20Manager) _asbp_interactive_grabbables_parent)
      (Rendering|Material|SetOverlayMaterial (Variables|/Game/Blueprint_Grabbable/BP_InteractiveGrabbablesParent.BP_InteractiveGrabbablesParent_C|GetStaticMesh _asbp_interactive_grabbables_parent) 0 :!class /Script/Engine.MeshComponent))
    (:CastFailed
      (CallFunction|SpecialObjectRespawnGeneral OtherActor))))

(event Custom|DeathzoneOnlyGrabbableDeactivation
  (bind _box (Variables|Default|GetBox))
  ;[1 1 1] DeathzoneOnly
  (Utilities|IsValid _box
    (:Is%20Valid
      (Components|DestroyComponent _box))))

(event EventBeginPlay
  ;[1 1 1] initialize
  (bind _gamemanager (CallFunction|GetGameManager))
  (Variables|Default|SetGame%20Manager _gamemanager))

(fn ConstructionScript)

(fn SpecialObjectRespawnGeneral
  (params (SpecialObject :type Object%20Object%20Reference))
  (bind _asbp_rune_mode_sphere_tutorial (Utilities|Casting|CastToBP_RuneModeSphereTutorial SpecialObject)
    (:then
      (Rendering|Material|SetOverlayMaterial (Variables|/Game/Asset_CameraBambina/BP/BP_RuneModeSphereTutorial.BP_RuneModeSphereTutorial_C|GetSphere _asbp_rune_mode_sphere_tutorial) 0 :!class /Script/Engine.MeshComponent)
      (Transformation|SetActorLocationAndRotation _asbp_rune_mode_sphere_tutorial (Variables|/Game/Asset_CameraBambina/BP/BP_RuneModeSphereTutorial.BP_RuneModeSphereTutorial_C|GetActorStartLocation _asbp_rune_mode_sphere_tutorial) (Variables|/Game/Asset_CameraBambina/BP/BP_RuneModeSphereTutorial.BP_RuneModeSphereTutorial_C|GetActorStartRotation _asbp_rune_mode_sphere_tutorial) false true)
      (Transformation|SetWorldLocationAndRotation (Variables|/Game/Asset_CameraBambina/BP/BP_RuneModeSphereTutorial.BP_RuneModeSphereTutorial_C|GetSphere _asbp_rune_mode_sphere_tutorial) (Variables|/Game/Asset_CameraBambina/BP/BP_RuneModeSphereTutorial.BP_RuneModeSphereTutorial_C|GetSphereStartLocation _asbp_rune_mode_sphere_tutorial) (Variables|/Game/Asset_CameraBambina/BP/BP_RuneModeSphereTutorial.BP_RuneModeSphereTutorial_C|GetSphereStartRotation _asbp_rune_mode_sphere_tutorial) false true)
      (Physics|SetPhysicsLinearVelocity (Variables|/Game/Asset_CameraBambina/BP/BP_RuneModeSphereTutorial.BP_RuneModeSphereTutorial_C|GetSphere _asbp_rune_mode_sphere_tutorial) "0, 0, 0" false "None"))
    (:CastFailed
      (return))))