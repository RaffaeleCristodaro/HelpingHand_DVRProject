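; Monster spawn Blueprint for the dining room (SalaDaPranzo) that grows bubble actors and teleports PhysicMonster to two spawn locations.
; Two events set flags that Tick polls, with the first taking priority; neither flag is cleared here.
; Tick calls PlayFromStart on the matching timeline every frame it runs that branch.
; Each timeline scales its bubble on update and moves the monster when finished.
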(event Custom|SpawnMonsterSecondTime
  ;[1 1 1] Spawn monster second time
  (Variables|Bubble|SetSecondBubbleSpawn? true))

(event Custom|SpawnMonsterFirstTime
  ;[1 1 1] Spawn monster first time
  (Variables|Bubble|SetFirstBubbleSpawn? true))

(event EventTick
  (params (DeltaSeconds :type Float%20%28single-precision%29))
  ;[1 1 1] Event tick
  (if (Variables|Bubble|GetFirstBubbleSpawn?)
    (bind _bubblescale (Timeline|SpawnMosterBubble_1 PlayFromStart)
      (:Update
        (Transformation|SetActorScale3D (Utilities|Array|Get(acopy) (Variables|Bubble|GetMonsterSpawnBubble)) (Math|Vector|MakeVector _bubblescale _bubblescale _bubblescale)))
      (:Finished
        (Transformation|SetActorLocation (Variables|PhysicMonster|GetPhysicMonster) (Utilities|Array|Get(acopy) (Variables|PhysicMonster|GetMosterSpawnLocations)) false true)))
    (elif (Variables|Bubble|GetSecondBubbleSpawn?)
      (bind _bubblescale_2 (Timeline|SpawnMosterBubble_2 PlayFromStart)
        (:Update
          (Transformation|SetActorScale3D (Utilities|Array|Get(acopy) (Variables|Bubble|GetMonsterSpawnBubble) 1) (Math|Vector|MakeVector _bubblescale_2 _bubblescale_2 _bubblescale_2)))
        (:Finished
          (Transformation|SetActorLocation (Variables|PhysicMonster|GetPhysicMonster) (Utilities|Array|Get(acopy) (Variables|PhysicMonster|GetMosterSpawnLocations) 1) false true))))))

(fn ConstructionScript)