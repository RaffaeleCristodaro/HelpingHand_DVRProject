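; Trigger for a statue jump scare in the surreal dining room zone, which slides a referenced statue when the player enters its box.
; The first overlap by BP_PG3 sets a flag through a DoOnce, and Tick plays a timeline while that flag is set.
; The timeline's Speed track is used as the absolute world X, teleporting the statue with Y and Z unchanged until it finishes and clears the flag.
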(event OnComponentBeginOverlap(Box)
  (params (OverlappedComponent :type Primitive%20Component%20Object%20Reference) (OtherActor :type Actor%20Object%20Reference) (OtherComp :type Primitive%20Component%20Object%20Reference) (OtherBodyIndex :type Integer) (bFromSweep :type Boolean) (SweepResult :type Hit%20Result%20Structure%20%28by%20ref%29))
  ;[1 1 1] Overlap with PG3
  (Utilities|Casting|CastToBP_PG3 OtherActor)
  (Utilities|FlowControl|DoOnce false
    (:Completed
      (Variables|Default|SetCanMoveStatue? true))))

(event EventTick
  (params (DeltaSeconds :type Float%20%28single-precision%29))
  (bind _statuetomove (Variables|StatueRef|GetStatueToMove))
  (bind _returnvalue (Transformation|GetActorLocation _statuetomove))
  ;[1 1 1] Event tick
  (if (Variables|Default|GetCanMoveStatue?)
    (bind _speed (Timeline|MoveStatueTimeline Play)
      (:Update
        (Transformation|SetActorLocation _statuetomove (Math|Vector|MakeVector _speed (.y _returnvalue) (.z _returnvalue)) false true))
      (:Finished
        (Variables|Default|SetCanMoveStatue? false)))))

(fn ConstructionScript)