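; BP_ActorRaiser is a trigger for the surreal dining room zone that raises a set of actors once BP_PG3 overlaps its Box.
; While the flag is set, Tick teleports each of RaisingActors up by Speed per frame, not scaled by delta time, clamped to its ZFinalLocations entry.
; RestoreZLocation clears the flag and returns each actor to its ZStartlLocations height, with both height arrays matched by index.
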(event OnComponentBeginOverlap(Box)
  (params (OverlappedComponent :type Primitive%20Component%20Object%20Reference) (OtherActor :type Actor%20Object%20Reference) (OtherComp :type Primitive%20Component%20Object%20Reference) (OtherBodyIndex :type Integer) (bFromSweep :type Boolean) (SweepResult :type Hit%20Result%20Structure%20%28by%20ref%29))
  ;[1 1 1] Collision with PG3
  (Utilities|Casting|CastToBP_PG3 OtherActor)
  (Variables|Default|SetCanRaiseActors? true))

(event Custom|RestoreZLocation
  ;[1 1 1] Restore Z start loc
  (Variables|Default|SetCanRaiseActors? false)
  (for (_array_element _array_index) (Variables|ActorsRef|GetRaisingActors)
    (Transformation|SetActorLocation _array_element (Math|Vector|MakeVector (.x (Transformation|GetActorLocation _array_element)) (.y (Transformation|GetActorLocation _array_element)) (Utilities|Array|Get(acopy) (Variables|ActorsRef|GetZStartlLocations) _array_index)) false false)))

(event EventTick
  (params (DeltaSeconds :type Float%20%28single-precision%29))
  ;[1 1 1] Event tick
  (if (Variables|Default|GetCanRaiseActors?)
    (Utilities|FlowControl|DoOnce false :!label _label
      (:Completed
        (for (_array_element _array_index) (Variables|ActorsRef|GetRaisingActors)
          (Transformation|SetActorLocation _array_element (Math|Vector|MakeVector (.x (Transformation|GetActorLocation _array_element)) (.y (Transformation|GetActorLocation _array_element)) (Math|Float|Clamp(Float) (+ (.z (Transformation|GetActorLocation _array_element)) (Variables|ActorsRef|GetSpeed)) -1e+04 (Utilities|Array|Get(acopy) (Variables|ActorsRef|GetZFinalLocations) _array_index))) false true))
        (goto _label Reset)))))

(fn ConstructionScript)