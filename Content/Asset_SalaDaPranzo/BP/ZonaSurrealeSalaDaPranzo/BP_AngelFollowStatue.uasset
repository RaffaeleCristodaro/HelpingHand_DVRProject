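; Angel statue actor for the surreal dining room zone that turns in place to face the player.
; It caches the player through GetPlayer3 on BeginPlay, then every Tick computes a look-at yaw from its root toward the player's mesh.
; That world yaw is clamped between Min and Max and applied instantly to the root, keeping pitch and roll unchanged.
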(event EventBeginPlay
  ;[1 1 1] Initialize
  (bind _pg3 (CallFunction|GetPlayer3))
  (Variables|Default|SetPG3 _pg3))

(event EventTick
  (params (DeltaSeconds :type Float%20%28single-precision%29))
  (bind _defaultsceneroot (Variables|Default|GetDefaultSceneRoot))
  (bind _returnvalue (Transformation|GetWorldRotation _defaultsceneroot))
  ;[1 1 1] Event tick
  (Transformation|SetWorldRotation _defaultsceneroot (Math|Rotator|MakeRotator (.roll _returnvalue) (.pitch _returnvalue) (Math|Float|Clamp(Float) (.yaw (Math|Rotator|FindLookatRotation (Transformation|GetWorldLocation _defaultsceneroot) (Transformation|GetWorldLocation (Variables|/Script/Engine.Character|GetMesh (Variables|Default|GetPG3))))) (Variables|StatueRef|GetMin) (Variables|StatueRef|GetMax))) false true))

(fn ConstructionScript)