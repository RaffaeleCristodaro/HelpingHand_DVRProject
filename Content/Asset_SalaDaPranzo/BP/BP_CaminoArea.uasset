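; Dining-room fireplace trigger that reacts to the players' fire rune mode.
; A Box overlap, rechecked every Tick, tests PG1's rune-mode flags or PG3's active rune Niagara.
; PG1's failed check falls through to PG3's, even if PG3 is outside the box.
; A DoOnce then swaps a Camino material to a lamp instance and, after a short delay, destroys the MelmaDissolve actor.
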(event OnComponentBeginOverlap(Box)
  (params (OverlappedComponent :type Primitive%20Component%20Object%20Reference) (OtherActor :type Actor%20Object%20Reference) (OtherComp :type Primitive%20Component%20Object%20Reference) (OtherBodyIndex :type Integer) (bFromSweep :type Boolean) (SweepResult :type Hit%20Result%20Structure%20%28by%20ref%29))
  (bind _pg1 (Variables|Default|GetPG1))
  (bind _pg3 (Variables|Default|GetPG3))
  ;[1 1 1] Overlap with Fire rune mode
  (if (== OtherActor _pg1)
    (if (and (Variables|/Game/VRTemplate/Blueprints/VRPawn.VRPawn_C|GetIsRuneModeOn? _pg1) (or (Variables|/Game/VRTemplate/Blueprints/VRPawn.VRPawn_C|GetIsRuneModeOnParticlesOnRight? _pg1) (Variables|/Game/VRTemplate/Blueprints/VRPawn.VRPawn_C|GetIsRuneModeOnParticlesOnLeft? _pg1)))
      (Utilities|FlowControl|DoOnce false :!label _label
        (:Completed
          (Rendering|Material|SetMaterial (Variables|/Script/Engine.StaticMeshActor|GetStaticMeshComponent (Variables|Default|GetCamino)) 1 "/Game/Asset_Cucina/M_Master_Lampada_Inst1.M_Master_Lampada_Inst1")
          (Utilities|FlowControl|Delay 0.2)
          (Actor|DestroyActor (Variables|Default|GetMelmaDissolve))))
      (else
        (if (Components|Activation|IsActive (Variables|/Game/PG3/BP_PG3.BP_PG3_C|GetRuneModeNiagara _pg3)) :!label _label_2
          (goto _label))))
    (elif (== OtherActor _pg3)
      (goto _label_2))))

(event EventBeginPlay
  ;[1 1 1] Initialize
  (bind _pg3 (CallFunction|GetPlayer3))
  (Variables|Default|SetPG3 _pg3)
  (bind _pg1 (CallFunction|GetPlayer1))
  (Variables|Default|SetPG1 _pg1))

(event EventTick
  (params (DeltaSeconds :type Float%20%28single-precision%29))
  (bind _pg1 (Variables|Default|GetPG1))
  ;[1 1 1] Event tick
  (if (Collision|IsOverlappingActor (Variables|Default|GetBox) (Variables|Default|GetPG1) :!class /Script/Engine.PrimitiveComponent)
    ;[1 1 1] Overlap with Fire rune mode
    (if (and (Variables|/Game/VRTemplate/Blueprints/VRPawn.VRPawn_C|GetIsRuneModeOn? _pg1) (or (Variables|/Game/VRTemplate/Blueprints/VRPawn.VRPawn_C|GetIsRuneModeOnParticlesOnRight? _pg1) (Variables|/Game/VRTemplate/Blueprints/VRPawn.VRPawn_C|GetIsRuneModeOnParticlesOnLeft? _pg1)))
      (Utilities|FlowControl|DoOnce false :!label _label
        (:Completed
          (Rendering|Material|SetMaterial (Variables|/Script/Engine.StaticMeshActor|GetStaticMeshComponent (Variables|Default|GetCamino)) 1 "/Game/Asset_Cucina/M_Master_Lampada_Inst1.M_Master_Lampada_Inst1")
          (Utilities|FlowControl|Delay 0.2)
          (Actor|DestroyActor (Variables|Default|GetMelmaDissolve))))
      (else
        (if (Components|Activation|IsActive (Variables|/Game/PG3/BP_PG3.BP_PG3_C|GetRuneModeNiagara (Variables|Default|GetPG3))) :!label _label_2
          (goto _label))))
    (elif (Collision|IsOverlappingActor (Variables|Default|GetBox) (Variables|Default|GetPG3) :!class /Script/Engine.PrimitiveComponent)
      (goto _label_2))))

(fn ConstructionScript)