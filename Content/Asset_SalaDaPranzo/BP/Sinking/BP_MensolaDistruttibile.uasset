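; BP_MensolaDistruttibile is a destructible shelf that tips over after the player touches it.
; Overlap by the cached Player3 waits half a second, plays an optional fall sound and sets a flag.
; While flagged, Tick plays a Timeline that drives the mesh's pitch, clearing the flag when finished.
; RestoreMensolaEvent disables mesh physics, restores the transform saved at BeginPlay and resets the Timeline's time.
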(event OnComponentBeginOverlap(Box)
  (params (OverlappedComponent :type Primitive%20Component%20Object%20Reference) (OtherActor :type Actor%20Object%20Reference) (OtherComp :type Primitive%20Component%20Object%20Reference) (OtherBodyIndex :type Integer) (bFromSweep :type Boolean) (SweepResult :type Hit%20Result%20Structure%20%28by%20ref%29))
  (bind _soundfallmensola (Variables|Default|GetSoundFallMensola))
  ;[1 1 1] Player hit
  (if (== OtherActor (Variables|Default|GetPG3))
    (Utilities|FlowControl|Delay 0.5)
    (Variables|Default|SetCanStartFallingRotation? true)
    (Utilities|IsValid _soundfallmensola
      (:Is%20Valid
        (Audio|PlaySound2D _soundfallmensola 1.0 1.0 0.0 0 0)))))

(event Custom|RestoreMensolaEvent
  (bind _staticmesh (Variables|Default|GetStaticMesh))
  ;[1 1 1] Player hit
  (Physics|SetSimulatePhysics _staticmesh false)
  (Transformation|SetWorldLocation _staticmesh (Variables|Default|GetStaticMeshInitialLocation) false false)
  (Transformation|SetWorldRotation _staticmesh (Variables|Default|GetIntialWordlRotation) false false)
  (CallFunction|RestoreTimelineMensolaDistruttibile))

(event Custom|RestoreTimelineMensolaDistruttibile
  (bind _staticmesh (Variables|Default|GetStaticMesh))
  (bind _returnvalue (Transformation|GetWorldRotation _staticmesh))
  ;[1 1 1] Event tick
  (bind _rotationmensolafloat (Timeline|Timeline SetNewTime)
    (:Update
      (Transformation|SetWorldRotation _staticmesh (Math|Rotator|MakeRotator (.roll _returnvalue) _rotationmensolafloat (.yaw _returnvalue)) false false))
    (:Finished
      (Variables|Default|SetCanStartFallingRotation? false))))

(event EventBeginPlay
  (bind _staticmesh (Variables|Default|GetStaticMesh))
  ;[1 1 1] Initialize
  (bind _pg3 (CallFunction|GetPlayer3))
  (Variables|Default|SetPG3 _pg3)
  (Variables|Default|SetStaticMeshInitialLocation (Transformation|GetWorldLocation _staticmesh))
  (Variables|Default|SetIntialWordlRotation (Transformation|GetWorldRotation _staticmesh)))

(event EventTick
  (params (DeltaSeconds :type Float%20%28single-precision%29))
  (bind _staticmesh (Variables|Default|GetStaticMesh))
  (bind _returnvalue (Transformation|GetWorldRotation _staticmesh))
  ;[1 1 1] Event tick
  (if (Variables|Default|GetCanStartFallingRotation?)
    (bind _rotationmensolafloat (Timeline|Timeline Play)
      (:Update
        (Transformation|SetWorldRotation _staticmesh (Math|Rotator|MakeRotator (.roll _returnvalue) _rotationmensolafloat (.yaw _returnvalue)) false false))
      (:Finished
        (Variables|Default|SetCanStartFallingRotation? false)))))

(fn ConstructionScript)