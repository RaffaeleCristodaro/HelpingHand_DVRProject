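; BP_Sedia_2 is a dining-room chair that sinks while Player 3 overlaps its trigger box.
; Overlap events set a flag that Tick reads, restarting the sink Timeline from the start every frame or stopping it.
; Timeline updates subtract the curve value from the mesh's current Z, and its finish plays an optional sound.
; RestoreSinking returns the mesh to the height saved at BeginPlay.
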(event OnComponentBeginOverlap(Box)
  (params (OverlappedComponent :type Primitive%20Component%20Object%20Reference) (OtherActor :type Actor%20Object%20Reference) (OtherComp :type Primitive%20Component%20Object%20Reference) (OtherBodyIndex :type Integer) (bFromSweep :type Boolean) (SweepResult :type Hit%20Result%20Structure%20%28by%20ref%29))
  ;[1 1 1] Overlap PG3
  (if (== OtherActor (Variables|Default|GetPG3))
    (Variables|Sinking|SetStartSinking? true)))

(event OnComponentEndOverlap(Box)
  (params (OverlappedComponent :type Primitive%20Component%20Object%20Reference) (OtherActor :type Actor%20Object%20Reference) (OtherComp :type Primitive%20Component%20Object%20Reference) (OtherBodyIndex :type Integer))
  ;[1 1 1] Overlap PG3
  (if (== OtherActor (Variables|Default|GetPG3))
    (Variables|Sinking|SetStartSinking? false)))

(event EventBeginPlay
  ;[1 1 1] Intialize
  (Variables|Default|SetInitialZLocation (.z (Transformation|GetWorldLocation (Variables|Default|GetStaticMesh))))
  (bind _pg3 (CallFunction|GetPlayer3))
  (Variables|Default|SetPG3 _pg3))

(event EventTick
  (params (DeltaSeconds :type Float%20%28single-precision%29))
  (bind _staticmesh (Variables|Default|GetStaticMesh))
  (bind _sinksound (Variables|Sinking|GetSinkSound))
  (bind _returnvalue (Transformation|GetWorldLocation _staticmesh))
  ;[1 1 1] Event tick
  (if (Variables|Sinking|GetStartSinking?)
    (bind _sinkingcurve (Timeline|Timeline PlayFromStart)
      (:Update
        (Transformation|SetWorldLocation _staticmesh (Math|Vector|MakeVector (.x _returnvalue) (.y _returnvalue) (- (.z _returnvalue) _sinkingcurve)) false true))
      (:Finished
        (Utilities|IsValid _sinksound
          (:Is%20Valid
            (Audio|PlaySound2D _sinksound 1.0 1.0 0.0 0 0)))))
    (else
      (Timeline|Timeline Stop))))

(event EventRestoreSinking
  (bind _staticmesh (Variables|Default|GetStaticMesh))
  (bind _returnvalue (Transformation|GetWorldLocation _staticmesh))
  ;[1 1 1] Restore sinking override
  (Transformation|SetWorldLocation _staticmesh (Math|Vector|MakeVector (.x _returnvalue) (.y _returnvalue) (Variables|Default|GetInitialZLocation)) false false))

(fn ConstructionScript)