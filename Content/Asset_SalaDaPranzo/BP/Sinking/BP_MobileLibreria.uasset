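; Bookcase in the dining room (SalaDaPranzo) that sinks when an actor implementing BPI_PG3 enters its trigger box.
; After a delay, a timeline subtracts its curve value from the mesh's current Z each update, so descent accumulates, then plays a sink sound when finished.
; Leaving the box stops the timeline; both overlaps fire only once.
; RestoreSinking calls the parent, restores the starting height and re-arms both triggers.
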(event OnComponentBeginOverlap(Box)
  (params (OverlappedComponent :type Primitive%20Component%20Object%20Reference) (OtherActor :type Actor%20Object%20Reference) (OtherComp :type Primitive%20Component%20Object%20Reference) (OtherBodyIndex :type Integer) (bFromSweep :type Boolean) (SweepResult :type Hit%20Result%20Structure%20%28by%20ref%29))
  (bind _staticmesh (Variables|Default|GetStaticMesh))
  (bind _returnvalue (Transformation|GetWorldLocation _staticmesh))
  ;[1 1 1] Overlap PG3
  (if (Utilities|DoesObjectImplementInterface OtherActor "/Game/Managers/BlueprintInterfaces/BPI_PG3.BPI_PG3_C")
    (Utilities|FlowControl|DoOnce false
      (:Completed
        (Utilities|FlowControl|Delay (Variables|Default|GetDelay))
        (Components|Timeline|SetPlayRate (Variables|Default|GetSink_Anim) (Variables|Default|GetTime%20Sink))
        (bind _sinkingcurve (Timeline|Sink_Anim PlayFromStart)
          (:Update
            (Transformation|SetWorldLocation _staticmesh (Math|Vector|MakeVector (.x _returnvalue) (.y _returnvalue) (- (.z _returnvalue) _sinkingcurve)) false true))
          (:Finished
            (CallFunction|PlaySinkSound)))))))

(event OnComponentEndOverlap(Box)
  (params (OverlappedComponent :type Primitive%20Component%20Object%20Reference) (OtherActor :type Actor%20Object%20Reference) (OtherComp :type Primitive%20Component%20Object%20Reference) (OtherBodyIndex :type Integer))
  (bind _staticmesh (Variables|Default|GetStaticMesh))
  (bind _returnvalue (Transformation|GetWorldLocation _staticmesh))
  ;[1 1 1] Overlap PG3
  (if (Utilities|DoesObjectImplementInterface OtherActor "/Game/Managers/BlueprintInterfaces/BPI_PG3.BPI_PG3_C")
    (Utilities|FlowControl|DoOnce false
      (:Completed
        (bind _sinkingcurve (Timeline|Sink_Anim Stop)
          (:Update
            (Transformation|SetWorldLocation _staticmesh (Math|Vector|MakeVector (.x _returnvalue) (.y _returnvalue) (- (.z _returnvalue) _sinkingcurve)) false true))
          (:Finished
            (CallFunction|PlaySinkSound)))))))

(event Custom|ResetBeginOverlap
  (bind _staticmesh (Variables|Default|GetStaticMesh))
  (bind _returnvalue (Transformation|GetWorldLocation _staticmesh))
  ;[1 1 1] Overlap PG3
  (Utilities|FlowControl|DoOnce false) ; enters at Reset
)

(event Custom|ResetEndOverlap
  (bind _staticmesh (Variables|Default|GetStaticMesh))
  (bind _returnvalue (Transformation|GetWorldLocation _staticmesh))
  ;[1 1 1] Overlap PG3
  (Utilities|FlowControl|DoOnce false) ; enters at Reset
)

(event EventBeginPlay
  ;[1 0.1073 0.1073 1 50] Begin Play
  ;;[1 1 1] Set start Z location
  (Variables|Default|SetInitialZLocation (.z (Transformation|GetWorldLocation (Variables|Default|GetStaticMesh)))))

(event EventRestoreSinking
  (bind _staticmesh (Variables|Default|GetStaticMesh))
  (bind _returnvalue (Transformation|GetWorldLocation _staticmesh))
  ;[0.9848 0.03478 1 1 50] Interface
  ;;[1 1 1] Restore sinking
  (|CallParentFunction)
  (Transformation|SetWorldLocation _staticmesh (Math|Vector|MakeVector (.x _returnvalue) (.y _returnvalue) (Variables|Default|GetInitialZLocation)) false false)
  (CallFunction|ResetEndOverlap)
  (CallFunction|ResetBeginOverlap))

(fn ConstructionScript)