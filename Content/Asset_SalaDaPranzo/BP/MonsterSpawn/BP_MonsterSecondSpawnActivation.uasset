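; Trigger actor in the dining room (Sala da Pranzo) that switches the monster over to its second spawn setup.
; When the cached player first overlaps the box, a DoOnce assigns the new spawner and bubble spawn references to PhysicMonster and calls its DespawnMonster.
; It then destroys the old bubble spawn and old spawner if they are still valid.
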(event OnComponentBeginOverlap(Box)
  (params (OverlappedComponent :type Primitive%20Component%20Object%20Reference) (OtherActor :type Actor%20Object%20Reference) (OtherComp :type Primitive%20Component%20Object%20Reference) (OtherBodyIndex :type Integer) (bFromSweep :type Boolean) (SweepResult :type Hit%20Result%20Structure%20%28by%20ref%29))
  (bind _physicmonster (Variables|Default|GetPhysicMonster))
  (bind _oldbubblemonsterspawn (Variables|Default|GetOldBubbleMonsterSpawn))
  (bind _oldmonsterspawnersalapranzo (Variables|Default|GetOldMonsterSpawnerSalaPranzo))
  ;[1 1 1] Begin overlap
  (if (== OtherActor (Variables|Default|GetPG3))
    (Utilities|FlowControl|DoOnce false
      (:Completed
        (Variables|/Game/Enemies/EnemyPhisyc/BP_PhysicMonster.BP_PhysicMonster_C|SetBP_MonsterSpawnerSalaPranzo _physicmonster (Variables|Default|GetNewMonsterSpawnerSalaPranzo))
        (Variables|/Game/Enemies/EnemyPhisyc/BP_PhysicMonster.BP_PhysicMonster_C|SetBubbleMonsterSpawn _physicmonster (Variables|Default|GetNewBubbleMonsterSpawn))
        (Default|DespawnMonster _physicmonster)
        (Utilities|IsValid _oldbubblemonsterspawn
          (:Is%20Valid
            (Actor|DestroyActor _oldbubblemonsterspawn))
          (:Is%20Not%20Valid
            _))
        (Utilities|IsValid _oldmonsterspawnersalapranzo
          (:Is%20Valid
            (Actor|DestroyActor _oldmonsterspawnersalapranzo)))))))

(event EventBeginPlay
  ;[1 1 1] Initialize
  (bind _pg3 (CallFunction|GetPlayer3))
  (Variables|Default|SetPG3 _pg3))

(fn ConstructionScript)