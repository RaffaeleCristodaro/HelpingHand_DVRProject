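; Bubble actor for a monster spawn, with a pop-out animation and a player respawn point.
; BubblePopOutAnim plays a timeline that drives uniform scale by a multiplier, then hides the actor and fires OnAnimationFinished.
; BubblePopInAnim restores the scale cached at BeginPlay and unhides it.
; The construction script moves an editor sphere to the debug respawn offset and stores its world position as PlayerSpawnLocation.
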(event Custom|BubblePopInAnim
  ;[0 0 0 1 50] Custom Events
  ;;[1 1 1] Reset Animation
  (Transformation|SetActorScale3D (Variables|Default|GetInitialScaleBubble))
  (Rendering|SetActorHiddenInGame false))

(event Custom|BubblePopOutAnim
  ;[0 0 0 1 50] Custom Events
  ;;[1 1 1] Start Animation
  (bind _bubblescale (Timeline|Timeline PlayFromStart)
    (:Update
      (Transformation|SetActorScale3D (Math|Vector|MakeVector (* _bubblescale (Variables|Default|GetScaleMultiplier)) (* _bubblescale (Variables|Default|GetScaleMultiplier)) (* _bubblescale (Variables|Default|GetScaleMultiplier)))))
    (:Finished
      (Rendering|SetActorHiddenInGame true)
      (Default|CallOnAnimationFinished))))

(event EventBeginPlay
  ;[1 0.09896 0.09896 1 50] BEgin Play
  (Variables|Default|SetInitialScaleBubble (Transformation|GetActorScale3D)))

(fn ConstructionScript
  (Transformation|SetRelativeLocation (Variables|Default|GetEditor_PhereCheck) (Variables|Editables|GetDebugPlayerRespawnLocation) false false)
  (Variables|Default|SetPlayerSpawnLocation (Transformation|GetWorldLocation (Variables|Default|GetEditor_PhereCheck))))