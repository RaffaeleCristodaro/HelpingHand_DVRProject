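; Handler that manages the physics monster's despawn and respawn at checkpoint spawner triggers.
; A checkpoint update destroys the previous trigger, stores the new one and despawns the monster.
; Spawning plays the trigger's bubble pop-out, then moves the monster there, respawns it and flings listed meshes with random impulses, once until ResetState.
; Getters lazily cache, find or spawn the normal and giant monsters, though only the normal one is used here.
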(event Custom|DespawnMonster
  ;[1 1 1] Despawn Monster
  (bind _physicmonsterref (CallFunction|GetPhysicMonsterRef))
  (Default|DespawnMonster _physicmonsterref))

(event Custom|UpdateMonsterCheckpoint
  (params (NewCheckpointTrigger :type BP%20Monster%20Trigger%20Object%20Reference))
  ;[1 1 1] Update Monster Checkpoint
  (Utilities|IsValid (Variables|Editable|GetCurrent_SpawnerTrigger)
    (:Is%20Valid
      (Actor|DestroyActor (Variables|Editable|GetCurrent_SpawnerTrigger)))
    (:Is%20Not%20Valid
      _))
  (Variables|Editable|SetCurrent_SpawnerTrigger NewCheckpointTrigger)
  (CallFunction|DespawnMonster))

(event Custom|ResetMeshThrow
  ;[1 1 1] Monster Spawn
  ;;[1 1 1] Explosion around monster
  (Utilities|FlowControl|DoOnce false) ; enters at Reset
)

(event Custom|SpawnMonster
  ;[1 1 1] Monster Spawn
  (EventDispatchers|AssignOnAnimationFinished (Variables|/Game/Asset_SalaDaPranzo/BP/MonsterSpawn/BP_MonsterTrigger.BP_MonsterTrigger_C|GetRef_Bubble (Variables|Editable|GetCurrent_SpawnerTrigger)) (delegate Custom|OnAnimationFinished_Event))
  (Default|BubblePopOutAnim (Variables|/Game/Asset_SalaDaPranzo/BP/MonsterSpawn/BP_MonsterTrigger.BP_MonsterTrigger_C|GetRef_Bubble (Variables|Editable|GetCurrent_SpawnerTrigger))))

(event Custom|OnAnimationFinished_Event
  ;[1 1 1] Monster Spawn
  (bind _physicmonsterref (CallFunction|GetPhysicMonsterRef))
  (Transformation|SetActorLocation _physicmonsterref (Transformation|GetActorLocation (Variables|/Game/Asset_SalaDaPranzo/BP/MonsterSpawn/BP_MonsterTrigger.BP_MonsterTrigger_C|GetRef_Bubble (Variables|Editable|GetCurrent_SpawnerTrigger))) false false)
  (Default|RespawnMonster _physicmonsterref)
  ;;[1 1 1] Explosion around monster
  (Utilities|FlowControl|DoOnce false
    (:Completed
      (if (Utilities|Array|IsNotEmpty (Variables|MeshToThrow|GetStaticMeshActorsToThrow))
        (for _array_element (Variables|MeshToThrow|GetStaticMeshActorsToThrow)
          (Utilities|IsValid (Variables|/Script/Engine.StaticMeshActor|GetStaticMeshComponent _array_element)
            (:Is%20Valid
              (Physics|AddImpulse (Variables|/Script/Engine.StaticMeshActor|GetStaticMeshComponent _array_element) (* (Math|Random|RandomUnitVector) (Variables|MeshToThrow|GetImpulseForce)) "None" false))))))))

(event EventResetState
  ;[1 0 0.9151 1 50] Interface
  ;;[1 1 1] Reset State
  (CallFunction|ResetMeshThrow))

(fn ConstructionScript)

(fn GetPhysicMonsterRef
  (Variables|References|GetRef_Physic%20Monster
    (:then
      _)
    (:else
      (bind _returnvalue (Actor|GetActorOfClass "/Game/Enemies/EnemyPhisyc/BP_PhysicMonster.BP_PhysicMonster_C"))
      (Variables|References|SetRef_Physic%20Monster _returnvalue)
      (Variables|References|GetRef_Physic%20Monster
        (:then
          _)
        (:else
          (bind _returnvalue_2 (Game|SpawnActorfromClass "/Game/Enemies/EnemyPhisyc/BP_PhysicMonster.BP_PhysicMonster_C" (Math|Transform|MakeTransform "0, 0, 0" "0, 0, 0" "1.000000,1.000000,1.000000") "Undefined" 0 0))
          (Variables|References|SetRef_Physic%20Monster _returnvalue_2)))))
  (return (Variables|References|GetRef_Physic%20Monster)))

(fn GetPhysicGiantMonsterRef
  (Variables|References|GetReg_PhysicGiantMonster
    (:then
      _)
    (:else
      (bind _returnvalue (Actor|GetActorOfClass "/Game/Enemies/EnemyPhysicSurreale/BP_PhysicMonsterGigante.BP_PhysicMonsterGigante_C"))
      (Variables|References|SetReg_PhysicGiantMonster _returnvalue)
      (Variables|References|GetReg_PhysicGiantMonster
        (:then
          _)
        (:else
          (bind _returnvalue_2 (Game|SpawnActorfromClass "/Game/Enemies/EnemyPhysicSurreale/BP_PhysicMonsterGigante.BP_PhysicMonsterGigante_C" (Math|Transform|MakeTransform "0, 0, 0" "0, 0, 0" "1.000000,1.000000,1.000000") "Undefined" 0 0))
          (Variables|References|SetReg_PhysicGiantMonster _returnvalue_2)))))
  (return (Variables|References|GetReg_PhysicGiantMonster)))