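; BP_MonsterTrigger is a one-shot box trigger that drives monster events when an actor implementing BPI_PG3 enters it.
; TriggerType selects spawning the monster, updating its checkpoint, having it grab PG3, or setting a giant monster action.
; Monster calls route through a lazily cached BP_MonsterSpawnHandler, and ResetState re-arms the trigger.
; The construction script stores the grab location from a debug component's world position.
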(event OnComponentBeginOverlap(Box)
  (params (OverlappedComponent :type Primitive%20Component%20Object%20Reference) (OtherActor :type Actor%20Object%20Reference) (OtherComp :type Primitive%20Component%20Object%20Reference) (OtherBodyIndex :type Integer) (bFromSweep :type Boolean) (SweepResult :type Hit%20Result%20Structure%20%28by%20ref%29))
  ;[0 0.5334 1 1 50] Overlap
  (if (Utilities|DoesObjectImplementInterface OtherActor "/Game/Managers/BlueprintInterfaces/BPI_PG3.BPI_PG3_C")
    (Utilities|FlowControl|DoOnce false
      (:Completed
        (switch Utilities|FlowControl|Switch|SwitchonE_MonsterTriggerActions (Variables|Editables|GetTriggerType)
          (:NewEnumerator0
            ;;[1 1 1] Spawn Monster
            (bind _monsterspawnhandlerref (CallFunction|GetMonsterSpawnHandler))
            (Default|SpawnMonster _monsterspawnhandlerref))
          (:NewEnumerator1
            ;;[1 1 1] Update Checkpoint
            (bind _monsterspawnhandlerref_2 (CallFunction|GetMonsterSpawnHandler))
            (Default|UpdateMonsterCheckpoint _monsterspawnhandlerref_2 self))
          (:NewEnumerator4
            ;;[1 1 1] Grab PG3
            (bind _monsterspawnhandlerref_3 (CallFunction|GetMonsterSpawnHandler))
            (Default|GrabPG3 (Variables|/Game/Asset_SalaDaPranzo/BP/MonsterSpawn/BP_MonsterSpawnHandler.BP_MonsterSpawnHandler_C|GetRef_Physic%20Monster _monsterspawnhandlerref_3) (Variables|Default|GetMonsterGrabPG3Location)))
          (:NewEnumerator3
            ;;[1 1 1] Giant monster action
            (bind _monsterspawnhandlerref_4 (CallFunction|GetMonsterSpawnHandler))
            (bind _monstergiantref (Default|GetPhysicGiantMonsterRef _monsterspawnhandlerref_4))
            (Transformation|SetMobility (Variables|/Script/Engine.Character|GetCapsuleComponent _monstergiantref) "Movable")
            (Default|SetCurrentMonsterGiantAction _monstergiantref (Variables|GiantMonster|GetGiantMonsterAction))
            (Transformation|SetActorLocationAndRotation (Variables|GiantMonster|GetPhysicMonsterGiganteNewLocation) (Variables|GiantMonster|GetPhysicMonsterGiganteNewRotation) false true)))))))

(event Custom|ResetTrigger
  ;[0 0.5334 1 1 50] Overlap
  (Utilities|FlowControl|DoOnce false) ; enters at Reset
)

(event EventResetState
  ;[0.8629 0.02084 1 1 50] Interface
  ;;[1 1 1] Reset Trigger
  (CallFunction|ResetTrigger))

(fn ConstructionScript
  (Variables|Default|SetMonsterGrabPG3Location (Transformation|GetWorldLocation (Variables|Default|GetMonsterPG3GrabLocationDebug))))

(fn GetMonsterSpawnHandler
  (Variables|Default|GetRef_Monster%20Spawn%20Handler
    (:then
      _)
    (:else
      (bind _returnvalue (Actor|GetActorOfClass "/Game/Asset_SalaDaPranzo/BP/MonsterSpawn/BP_MonsterSpawnHandler.BP_MonsterSpawnHandler_C"))
      (Variables|Default|SetRef_Monster%20Spawn%20Handler _returnvalue)))
  (return (Variables|Default|GetRef_Monster%20Spawn%20Handler)))