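; BP_Melma is a slime hazard that changes the PG3 player's speed and drowns them after a time limit.
; Interface overlap calls, gated by two DoOnce nodes that re-arm each other, start and clear the drowning and elapsed-time timers.
; Exit restores speed and mesh position and updates the player's TimeInMelma, which shortens DrowningTime on entry if already flagged in slime.
; Timeout triggers death through the game mode, while a timeline sinks the player mesh.
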(event Custom|OnDrownPlayer
  ;[0 0 0 1 50] Custom Events
  ;;[1 1 1] On Drown player
  (Utilities|Time|ClearandInvalidateTimerbyHandle (Variables|Frameworks|GetCheckTimeInMelmaTimerHandler))
  (Default|LocalPlayerDeath (Variables|References|GetRef_GameMode) "NewEnumerator1")
  (bind _drown (Timeline|DrownAnim PlayFromStart)
    (:Update
      (Default|SetPGMeshNewLocation (Variables|References|GetRef_PG3) (Math|Vector|Lerp(Vector) (Variables|/Game/PG3/BP_PG3.BP_PG3_C|GetStartMeshRelativeLocation (Variables|References|GetRef_PG3)) (- (Variables|/Game/PG3/BP_PG3.BP_PG3_C|GetStartMeshRelativeLocation (Variables|References|GetRef_PG3)) (Math|Vector|MakeVector 0.0 0.0 (Variables|Sinking|GetDrown_Z_Offset))) _drown) false))))

(event Custom|OverlapBeginWithPlayer
  (bind _ref_pg3 (Variables|References|GetRef_PG3))
  ;[0 0 0 1 50] Custom Events
  ;;[1 1 1] Overlap PG3
  (Utilities|FlowControl|DoOnce false
    (:Completed
      (if (Default|GetIsinMelma? _ref_pg3)
        (Variables|Sinking|SetDrowningTime (- (Variables|Sinking|GetDrowningTime) (Variables|/Game/PG3/BP_PG3.BP_PG3_C|GetTimeInMelma _ref_pg3)))
        (else
          (Default|SetIsinMelma (Variables|References|GetRef_PG3) true)
          (Default|SetPlayerSpeedMultiplier (Variables|References|GetRef_PG3) (Variables|Sinking|GetPlayerSpeedInMelmaMultiplier))))
      (bind _returnvalue (Utilities|Time|SetTimerbyFunctionName 0 "OnDrownPlayer" (Variables|Sinking|GetDrowningTime)))
      (Variables|Frameworks|SetSinkPlayerTimerHandler _returnvalue)
      (bind _returnvalue_2 (Utilities|Time|SetTimerbyFunctionName 0 "UpdateCurrentTimeInMelma" 0.01 true))
      (Variables|Frameworks|SetCheckTimeInMelmaTimerHandler _returnvalue_2)
      (CallFunction|RestoreMelmaInteractionEnd))))

(event Custom|OverlapEndWithPlayer
  (bind _ref_pg3 (Variables|References|GetRef_PG3))
  ;[0 0 0 1 50] Custom Events
  ;;[1 1 1] Exit Overlap PG3
  (Utilities|FlowControl|DoOnce false
    (:Completed
      (Utilities|Time|ClearandInvalidateTimerbyHandle (Variables|Frameworks|GetCheckTimeInMelmaTimerHandler))
      (Utilities|Time|ClearandInvalidateTimerbyHandle (Variables|Frameworks|GetSinkPlayerTimerHandler))
      (Variables|/Game/PG3/BP_PG3.BP_PG3_C|SetTimeInMelma (Variables|References|GetRef_PG3) (+ (Variables|/Game/PG3/BP_PG3.BP_PG3_C|GetTimeInMelma (Variables|References|GetRef_PG3)) (- (Variables|Sinking|GetDrowningTime) (Variables|Frameworks|GetCurrentTimeInMelma))))
      (Default|SetIsinMelma _ref_pg3 false)
      (Default|ResetMeshRelativeLocation _ref_pg3)
      (Default|SetPlayerSpeedMultiplier (Variables|References|GetRef_PG3) 1.0)
      (CallFunction|RestoreMelmaInteractionBegin))))

(event Custom|RestoreMelmaInteraction_Begin
  (bind _ref_pg3 (Variables|References|GetRef_PG3))
  ;[0 0 0 1 50] Custom Events
  ;;[1 1 1] Overlap PG3
  (Utilities|FlowControl|DoOnce false) ; enters at Reset
)

(event Custom|UpdateCurrentTimeInMelma
  ;[0 0 0 1 50] Custom Events
  ;;[1 1 1] Update Current time in melma
  (Variables|Frameworks|SetCurrentTimeInMelma (Math|Float|Clamp(Float) (+ (Variables|Frameworks|GetCurrentTimeInMelma) 0.01) 0.0 (Variables|Sinking|GetDrowningTime))))

(event Custom|RestoreMelmaInteraction_End
  (bind _ref_pg3 (Variables|References|GetRef_PG3))
  ;[0 0 0 1 50] Custom Events
  ;;[1 1 1] Exit Overlap PG3
  (Utilities|FlowControl|DoOnce false) ; enters at Reset
)

(event EventEndPlayerOverlap
  ;[0.8943 0 1 1 50] Interface
  ;;[1 1 1] End Overlap
  (CallFunction|OverlapEndwithPlayer))

(event EventBeginPlayerOverlap
  ;[0.8943 0 1 1 50] Interface
  ;;[1 1 1] Begin Overlap
  (CallFunction|OverlapBeginwithPlayer))

(event EventBeginPlay
  ;[1 0.08646 0.08646 1 50] Begin Play
  (bind _gamemoderef (Class|BPIGameMode|GetGameModeRef(Message) (Game|GetGameMode)))
  (bind _output_get (Variables|References|SetRef_GameMode _gamemoderef))
  (Variables|References|SetRef_PG3 (Default|GetPG3Ref _output_get)))

(fn ConstructionScript)