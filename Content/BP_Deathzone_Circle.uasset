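; Circle deathzone actor with a capsule trigger that sends the player (BP_PG3) and, optionally, grabbable objects back to respawn through the Game Manager.
; On player overlap, a DoOnce gate calls RespawnPlayers with configurable teleport and transform settings, then resets after a short delay.
; In levels flagged for sinking objects, it also restores those objects after the delay.
; Other overlapping grabbables are respawned if enabled, and their overlay material is cleared.
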(event OnComponentBeginOverlap(Capsule)
  (params (OverlappedComponent :type Primitive%20Component%20Object%20Reference) (OtherActor :type Actor%20Object%20Reference) (OtherComp :type Primitive%20Component%20Object%20Reference) (OtherBodyIndex :type Integer) (bFromSweep :type Boolean) (SweepResult :type Hit%20Result%20Structure%20%28by%20ref%29))
  ;[1 1 1] Deathzone collisions
  (Utilities|Casting|CastToBP_PG3 OtherActor
    (:then
      (Utilities|FlowControl|DoOnce false :!label _label
        (:Completed
          (Default|RespawnPlayers (Variables|Default|GetGame%20Manager) (Variables|RespawnPlayerLocation|GetForcedTeleportWhereToRespawn) (Variables|RespawnPlayerLocation|GetTeleportWhereToRespawn) (Variables|RespawnPlayerLocation|GetPG3RespawnLocation) (Variables|RespawnPlayerLocation|GetPG3RespawnRotation))
          (Utilities|FlowControl|Delay 1.0)
          (if (Variables|Sinking|GetIsLevelWhereObjectsSinks?)
            (for _array_element (Variables|Sinking|GetSinkingObjects)
              (Utilities|IsValid _array_element
                (:Is%20Valid
                  (Default|RestoreSinking _array_element))))
            (goto _label Reset)
            (else
              (goto _label Reset))))))
    (:CastFailed
      (if (Variables|GrabbableDeathzone|GetIsDeathzoneForGrabbable?)
        (bind _asbp_interactive_grabbables_parent (Utilities|Casting|CastToBP_InteractiveGrabbablesParent OtherActor))
        (Default|RespawnGrabbables (Variables|Default|GetGame%20Manager) _asbp_interactive_grabbables_parent)
        (Rendering|Material|SetOverlayMaterial (Variables|/Game/Blueprint_Grabbable/BP_InteractiveGrabbablesParent.BP_InteractiveGrabbablesParent_C|GetStaticMesh _asbp_interactive_grabbables_parent) 0 :!class /Script/Engine.MeshComponent)))))

(event EventBeginPlay
  ;[0 1 0.06679] initialize
  (bind _gamemanager (CallFunction|GetGameManager))
  (Variables|Default|SetGame%20Manager _gamemanager))

(fn ConstructionScript)