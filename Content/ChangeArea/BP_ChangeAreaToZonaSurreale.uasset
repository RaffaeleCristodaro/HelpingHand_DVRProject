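; BP_ChangeAreaToZonaSurreale is a trigger that moves the game into the Zona Surreale level when PG3 enters its box.
; The one-shot overlap makes PG3 faint, waits for the fall animation, attaches a fader to PG1's camera, then has GameManager change level.
; A GameInstance flag records the trip, so on return BeginPlay teleports PG1 and PG3 to return points and disables the trigger.
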(event OnComponentBeginOverlap(Box)
  (params (OverlappedComponent :type Primitive%20Component%20Object%20Reference) (OtherActor :type Actor%20Object%20Reference) (OtherComp :type Primitive%20Component%20Object%20Reference) (OtherBodyIndex :type Integer) (bFromSweep :type Boolean) (SweepResult :type Hit%20Result%20Structure%20%28by%20ref%29))
  ;[1 1 1] Collision with PG3
  (bind _asbp_pg3 (Utilities|Casting|CastToBP_PG3 OtherActor))
  (Variables|Default|SetPG3 _asbp_pg3)
  (if (Variables|ChangeAreaSurrealeRef|GetCanStartCollision?)
    (Utilities|FlowControl|DoOnce false
      (:Completed
        (Variables|/Game/PG3/BP_PG3.BP_PG3_C|SetIsFainting?_1 (Variables|Default|GetPG3) true)
        (Variables|/Game/PG3/BP_PG3.BP_PG3_C|SetIsDying? (Variables|Default|GetPG3) true)
        (CallFunction|ChangeAreaZonaSurrealeEvent)))))

(event Custom|ChangeAreaZonaSurrealeEvent
  ;[1 1 1] Change into zona surreale event
  (Utilities|Time|SetTimerbyEvent (delegate Custom|ChangeAreaZonaSurrealeTimerEvent) (Variables|ChangeAreaSurrealeRef|GetTimeForPG3FallAnimation)))

(event Custom|ChangeAreaZonaSurrealeTimerEvent
  (bind _pg1 (Variables|Default|GetPG1))
  (bind _camera (Variables|/Game/VRTemplate/Blueprints/VRPawn.VRPawn_C|GetCamera _pg1))
  ;[1 1 1] Change into zona surreale event
  (bind _returnvalue (Game|SpawnActorfromClass "/Game/ChangeArea/BP_Fader.BP_Fader_C" (Math|Transform|MakeTransform (Transformation|GetWorldLocation _camera) "0, 0, 0" "1.000000,1.000000,1.000000") "AlwaysSpawn" 0 0))
  (Transformation|AttachComponentToComponent _returnvalue _camera "None" "SnapToTarget" "SnapToTarget" "KeepRelative" true)
  (Default|ChangeLevel (Variables|Default|GetGame%20Manager) (Variables|ChangeAreaSurrealeRef|GetLevelNameZonaSurreale) (Variables|ChangeAreaSurrealeRef|GetLoading%20Time))
  (Variables|/Game/Managers/GI_HelpingHand.GI_HelpingHand_C|SetIsPG1ReturnedFromZonaSurreale? (Variables|Default|GetGIHelping%20Hand) true))

(event EventBeginPlay
  ;[1 1 1] Intialize
  (bind _gamemanager (CallFunction|GetGameManager))
  (Variables|Default|SetGame%20Manager _gamemanager)
  (bind _pg1 (CallFunction|GetPlayer1))
  (Variables|Default|SetPG1 _pg1)
  (bind _pg3 (CallFunction|GetPlayer3))
  (bind _asgi_helping_hand (Utilities|Casting|CastToGI_HelpingHand (Game|GetGameInstance)))
  (bind _output_get (Variables|Default|SetGIHelping%20Hand _asgi_helping_hand))
  (if (Variables|/Game/Managers/GI_HelpingHand.GI_HelpingHand_C|GetIsPG1ReturnedFromZonaSurreale? _output_get)
    (Variables|/Game/Managers/GI_HelpingHand.GI_HelpingHand_C|SetIsPG1ReturnedFromZonaSurreale? _output_get false)
    (Transformation|Teleport (Variables|Default|GetPG1) (Variables|ChangeAreaSurrealeRef|GetReturnFromZonaSurrealeLocationPG1) (Variables|ChangeAreaSurrealeRef|GetReturnFromZonaSurrealeRotationPG1))
    (Transformation|SetActorLocationAndRotation _pg3 (Variables|ChangeAreaSurrealeRef|GetReturnFromZonaSurrealeLocationPG3) (Variables|ChangeAreaSurrealeRef|GetReturnFromZonaSurrealeRotationPG3) false true)
    (Transformation|SetRelativeLocation (Variables|/Script/Engine.Character|GetMesh _pg3) (Math|Vector|MakeVector (.x (Variables|/Script/Engine.SceneComponent|GetRelativeLocation (Variables|/Script/Engine.Character|GetMesh _pg3))) (.y (Variables|/Script/Engine.SceneComponent|GetRelativeLocation (Variables|/Script/Engine.Character|GetMesh _pg3))) (Variables|/Game/PG3/BP_PG3.BP_PG3_C|GetStart%20ZRelative%20Location _pg3)) false false)
    (Variables|ChangeAreaSurrealeRef|SetCanStartCollision? false)))

(fn ConstructionScript)