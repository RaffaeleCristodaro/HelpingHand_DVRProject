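; BP_ChangeArea is a trigger volume that moves the game to another level when a BP_PG3 actor enters its box.
; On begin play it caches the game manager and Player 1.
; The first valid overlap, gated by DoOnce, attaches a spawned fader to Player 1's camera, blocks pause menu creation and spawns a loading screen spawner.
; It then passes its target level and loading time to the game manager's ChangeLevel.
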(event OnComponentBeginOverlap(Box)
  (params (OverlappedComponent :type Primitive%20Component%20Object%20Reference) (OtherActor :type Actor%20Object%20Reference) (OtherComp :type Primitive%20Component%20Object%20Reference) (OtherBodyIndex :type Integer) (bFromSweep :type Boolean) (SweepResult :type Hit%20Result%20Structure%20%28by%20ref%29))
  (bind _pg1 (Variables|Default|GetPG1))
  (bind _camera (Variables|/Game/Characters/VRPawn.VRPawn_C|GetCamera _pg1))
  ;[1 1 1] Change area when colliding with PG3
  (Utilities|Casting|CastToBP_PG3 OtherActor)
  (Utilities|FlowControl|DoOnce false
    (:Completed
      (bind _returnvalue (Game|SpawnActorfromClass "/Game/ChangeArea/BP_Fader.BP_Fader_C" (Math|Transform|MakeTransform (Transformation|GetWorldLocation _camera) "0, 0, 0" "1.000000,1.000000,1.000000") "AlwaysSpawn" 0 0))
      (Transformation|AttachComponentToComponent _returnvalue _camera "None" "SnapToTarget" "SnapToTarget" "KeepRelative" true)
      (Variables|/Game/Managers/BP_GameManager.BP_GameManager_C|SetCanCreatePauseMenu? (Variables|Default|GetGame%20Manager) false)
      (Game|SpawnActorfromClass "/Game/UIBlueprints/UIDiGioco/BP_LoadingScreenSpawner.BP_LoadingScreenSpawner_C" (Math|Transform|MakeTransform "0, 0, 0" "0, 0, 0" "1.000000,1.000000,1.000000") "Undefined" 0 0)
      (Default|ChangeLevel (Variables|Default|GetGame%20Manager) (Variables|Default|GetLevel%20to%20Open) (Variables|Default|GetLoadingTime)))))

(event EventBeginPlay
  ;[1 1 1] Initialize
  (bind _gamemanager (CallFunction|GetGameManager))
  (Variables|Default|SetGame%20Manager _gamemanager)
  (bind _pg1 (CallFunction|GetPlayer1))
  (Variables|Default|SetPG1 _pg1))

(fn ConstructionScript)