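; BP_Fader is an actor that fades a sphere's material in or out when it spawns, likely for area transitions.
; After a short delay, BeginPlay creates a dynamic material instance and the FadeIn flag selects one of two looping timers that step its Alpha parameter.
; Fade-in lowers Alpha and destroys the actor at zero.
; The slower fade-out raises Alpha until a limit, leaving the actor alive.
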(event Custom|FadeInEventFader
  ;[1 1 1] FadeIn
  (Utilities|Time|SetTimerbyEvent (delegate Custom|FadeIn) 0.1 true))

(event Custom|FadeIn
  ;[1 1 1] FadeIn
  (Rendering|Material|SetScalarParameterValue (Variables|Default|GetDinamicMaterial) "Alpha" (Variables|Default|GetFadeValue) :!class /Script/Engine.MaterialInstanceDynamic)
  (bind _output_get (Variables|Default|SetFadeValue (- (Variables|Default|GetFadeValue) 0.15)))
  (if (<= _output_get 0.0)
    (Utilities|FlowControl|DoOnce false
      (:Completed
        (Actor|DestroyActor)))))

(event Custom|FadeOutEventFader
  ;[1 1 1] Fade out
  (Utilities|Time|SetTimerbyEvent (delegate Custom|FadeOut) 0.1 true))

(event Custom|FadeOut
  ;[1 1 1] Fade out
  (if (Variables|Default|GetContinueFadeOut?)
    (Rendering|Material|SetScalarParameterValue (Variables|Default|GetDinamicMaterial) "Alpha" (Variables|Default|GetFadeValue) :!class /Script/Engine.MaterialInstanceDynamic)
    (bind _output_get (Variables|Default|SetFadeValue (+ (Variables|Default|GetFadeValue) 0.03)))
    (if (>= _output_get 2.0)
      (Variables|Default|SetContinueFadeOut? false))))

(event EventBeginPlay
  (bind _sphere (Variables|Default|GetSphere))
  ;[1 1 1] Initialize
  (Utilities|FlowControl|Delay 0.1)
  (bind _returnvalue (Rendering|Material|CreateDynamicMaterialInstance _sphere 0 (Rendering|Material|GetMaterial _sphere 0) "None" :!class /Script/Engine.PrimitiveComponent))
  (Variables|Default|SetDinamicMaterial _returnvalue)
  (if (Variables|Default|GetFadeIn?)
    (CallFunction|FadeinEventFader)
    (else
      (CallFunction|FadeOutEventFader))))

(fn ConstructionScript)