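; BP_Falo1 is a campfire that a player lights by entering its sphere with rune mode effects active.
; The overlap accepts a VRPawn with either hand's rune Niagara active, or a BP_PG3 with its rune Niagara active.
; A shared DoOnce then activates the fire Niagara, swaps the material, plays a campfire sound at world origin and sets a flag.
; Tick reads that flag to play a timeline raising the point light's intensity.
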(event OnComponentBeginOverlap(Sphere)
  (params (OverlappedComponent :type Primitive%20Component%20Object%20Reference) (OtherActor :type Actor%20Object%20Reference) (OtherComp :type Primitive%20Component%20Object%20Reference) (OtherBodyIndex :type Integer) (bFromSweep :type Boolean) (SweepResult :type Hit%20Result%20Structure%20%28by%20ref%29))
  ;[1 1 1] Collision with flame powers
  (bind _asvrpawn (Utilities|Casting|CastToVRPawn OtherActor)
    (:then
      (if (or (Components|Activation|IsActive (Variables|/Game/Characters/VRPawn.VRPawn_C|GetNiagaraRuneModeRight _asvrpawn)) (Components|Activation|IsActive (Variables|/Game/Characters/VRPawn.VRPawn_C|GetNiagaraRuneModeLeft _asvrpawn)))
        (Utilities|FlowControl|DoOnce false :!label _label
          (:Completed
            (Components|Activation|Activate (Variables|Default|GetNiagara) false)
            (Rendering|Material|SetMaterial (Variables|Default|GetFalo) 0 "/Game/Asset_Cucina/M_Master_Lampada_Inst1.M_Master_Lampada_Inst1")
            (Variables|Default|SetActivateLight? true)
            (Audio|PlaySoundatLocation "/Game/DefinitiveSounds/Camino/Campfire_01.Campfire_01" "0, 0, 0" "0, 0, 0" 1.0 1.0 0.0 "/Game/SoundSystem/SoundAttenuator/MainSoundAttenuator.MainSoundAttenuator" 0 0 0)))))
    (:CastFailed
      (bind _asbp_pg3 (Utilities|Casting|CastToBP_PG3 OtherActor))
      (if (Components|Activation|IsActive (Variables|/Game/PG3/BP_PG3.BP_PG3_C|GetRuneModeNiagara _asbp_pg3))
        (goto _label)))))

(event EventTick
  (params (DeltaSeconds :type Float%20%28single-precision%29))
  ;[1 1 1] Event tick
  (if (Variables|Default|GetActivateLight?)
    (bind _lightintensity (Timeline|LightUpTimeline Play)
      (:Update
        (Rendering|Components|Light|SetIntensity (Variables|/Script/Engine.Light|GetLightComponent (Variables|PointLightSettings|GetPointLight)) _lightintensity)))))

(event EventBeginPlay
  ;[1 1 1] Initialize
  (bind _pg3 (CallFunction|GetPlayer3))
  (Variables|Default|SetPG3 _pg3)
  (bind _pg1 (CallFunction|GetPlayer1))
  (Variables|Default|SetPG1 _pg1))

(fn ConstructionScript)