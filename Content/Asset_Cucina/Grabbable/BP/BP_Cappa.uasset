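; Kitchen hood (cappa) Blueprint that detects hits by grabbable objects or by the player while holding one, currently only printing a debug "hit".
; It caches Player 1 on BeginPlay, and its sphere overlap checks for a BP_InteractiveGrabbablesParent actor, otherwise whether either of Player 1's hands holds one.
; Each path fires once through its own DoOnce.
; Despite the helper's speed-named local variable, no speed is checked.
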(event OnComponentBeginOverlap(Sphere)
  (params (OverlappedComponent :type Primitive%20Component%20Object%20Reference) (OtherActor :type Actor%20Object%20Reference) (OtherComp :type Primitive%20Component%20Object%20Reference) (OtherBodyIndex :type Integer) (bFromSweep :type Boolean) (SweepResult :type Hit%20Result%20Structure%20%28by%20ref%29))
  ;[1 1 1] player is hitting cappa with object in hand
  (Utilities|Casting|CastToBP_InteractiveGrabbablesParent OtherActor
    (:then
      (Utilities|FlowControl|DoOnce false
        (:Completed
          (Development|PrintString "hit"))))
    (:CastFailed
      (bind _isplayerhittingcappawithobject_ (CallFunction|IsPlayerHittingCappawithObject?))
      (if _isplayerhittingcappawithobject_
        (Utilities|FlowControl|DoOnce false
          (:Completed
            (Development|PrintString "hit")))))))

(event EventBeginPlay
  ;[1 1 1] Initialize
  (bind _pg1 (CallFunction|GetPlayer1))
  (Variables|Default|SetPG1 _pg1))

(fn ConstructionScript)

(fn IsPlayerHittingCappawithObject?
  (bind _pg1 (Variables|Default|GetPG1))
  (bind _heldcomponentleft (Variables|/Game/Characters/VRPawn.VRPawn_C|GetHeldComponentLeft _pg1))
  (bind _heldcomponentright (Variables|/Game/Characters/VRPawn.VRPawn_C|GetHeldComponentRight _pg1))
  (Utilities|IsValid _heldcomponentleft
    (:Is%20Valid
      (Utilities|Casting|CastToBP_InteractiveGrabbablesParent (Components|GetOwner _heldcomponentleft)
        (:then
          (LocalVariables|SetIsPlayerHittingCappaWithEnoughSpeed?LocalVar true))
        (:CastFailed
          (Utilities|IsValid _heldcomponentright :!label _label
            (:Is%20Valid
              (Utilities|Casting|CastToBP_InteractiveGrabbablesParent (Components|GetOwner _heldcomponentright)
                (:then
                  (LocalVariables|SetIsPlayerHittingCappaWithEnoughSpeed?LocalVar true))
                (:CastFailed
                  (LocalVariables|SetIsPlayerHittingCappaWithEnoughSpeed?LocalVar false :!label _label_2))))
            (:Is%20Not%20Valid
              (goto _label_2))))))
    (:Is%20Not%20Valid
      (goto _label)))
  (return (LocalVariables|GetIsPlayerHittingCappaWithEnoughSpeed?LocalVar)))