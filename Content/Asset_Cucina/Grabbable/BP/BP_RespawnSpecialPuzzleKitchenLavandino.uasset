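; Trigger volume, apparently for the kitchen sink puzzle, that respawns special puzzle items entering its box.
; It caches the Game Manager on BeginPlay and, on box overlap, passes matching actors to the manager's RespawnGrabbables.
; The puzzle key (BPG_ChiavePuzzle) respawns unconditionally, while the sink plunger (BPG_SturaLavandino) respawns only if its GrabComponent reports it is not held.
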(event OnComponentBeginOverlap(Box)
  (params (OverlappedComponent :type Primitive%20Component%20Object%20Reference) (OtherActor :type Actor%20Object%20Reference) (OtherComp :type Primitive%20Component%20Object%20Reference) (OtherBodyIndex :type Integer) (bFromSweep :type Boolean) (SweepResult :type Hit%20Result%20Structure%20%28by%20ref%29))
  ;[1 1 1] Collision with special objects kitchen
  (bind _asbpg_chiave_puzzle (Utilities|Casting|CastToBPG_ChiavePuzzle OtherActor)
    (:then
      (Default|RespawnGrabbables (Variables|Default|GetGame%20Manager) _asbpg_chiave_puzzle))
    (:CastFailed
      (bind _asbpg_stura_lavandino (Utilities|Casting|CastToBPG_SturaLavandino OtherActor))
      (if (not (Variables|/Game/VRTemplate/Blueprints/GrabComponent.GrabComponent_C|GetbIsHeld (Variables|/Game/Blueprint_Grabbable/BP_InteractiveGrabbablesParent.BP_InteractiveGrabbablesParent_C|GetGrabComponent _asbpg_stura_lavandino)))
        (Default|RespawnGrabbables (Variables|Default|GetGame%20Manager) _asbpg_stura_lavandino)))))

(event EventBeginPlay
  ;[1 1 1] Initialize
  (bind _gamemanager (CallFunction|GetGameManager))
  (Variables|Default|SetGame%20Manager _gamemanager))

(fn ConstructionScript)