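; Spiderweb obstacle in the kitchen that burns away when a player in rune mode touches it.
; Box overlap accepts Player 1 with rune hand particles, or Player 3 with active rune Niagara plus a valid tutorial (whose check it clears) or toilet seat reference.
; Burning fires once, enables key puzzle collision and plays a delayed flame sound.
; A Tick-started timeline drives the material fade, then makes the toilet seat grabbable and destroys the web.
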(event OnComponentBeginOverlap(Box)
  (params (OverlappedComponent :type Primitive%20Component%20Object%20Reference) (OtherActor :type Actor%20Object%20Reference) (OtherComp :type Primitive%20Component%20Object%20Reference) (OtherBodyIndex :type Integer) (bFromSweep :type Boolean) (SweepResult :type Hit%20Result%20Structure%20%28by%20ref%29))
  (bind _pg1 (Variables|Default|GetPG1))
  (bind _cucinatutorial2 (Variables|Default|GetCucinaTutorial2))
  (bind _pg3 (Variables|Default|GetPG3))
  ;[1 1 1] Player collision
  (if (== OtherActor _pg1)
    (if (and (Variables|/Game/VRTemplate/Blueprints/VRPawn.VRPawn_C|GetIsRuneModeOn? _pg1) (or (Variables|/Game/VRTemplate/Blueprints/VRPawn.VRPawn_C|GetIsRuneModeOnParticlesOnRight? _pg1) (Variables|/Game/VRTemplate/Blueprints/VRPawn.VRPawn_C|GetIsRuneModeOnParticlesOnLeft? _pg1)))
      (Utilities|FlowControl|DoOnce false :!label _label
        (:Completed
          (CallFunction|StartBurning)))
      (else
        (if (and (== OtherActor _pg3) (Components|Activation|IsActive (Variables|/Game/PG3/BP_PG3.BP_PG3_C|GetRuneModeNiagara _pg3))) :!label _label_2
          (Utilities|IsValid _cucinatutorial2
            (:Is%20Valid
              (Variables|/Game/Asset_Cucina/BP/BP_CucinaTutorial2.BP_CucinaTutorial2_C|SetCanCheckTutorial2? _cucinatutorial2 false)
              (Variables|/Game/VRTemplate/Blueprints/VRPawn.VRPawn_C|SetIsRuneModeTutorialPassage? (Variables|Default|GetPG1) false)
              (goto _label))
            (:Is%20Not%20Valid
              (Utilities|IsValid (Variables|Cesso|GetBpTavolettaCesso)
                (:Is%20Valid
                  (goto _label))))))))
    (else
      (goto _label_2))))

(event Custom|StartBurning
  ;[1 1 1] Start burning
  (bind _returnvalue (Actor|GetActorOfClass "/Game/Asset_Cucina/Grabbable/BP/BPG_ChiavePuzzle.BPG_ChiavePuzzle_C"))
  (Utilities|IsValid _returnvalue
    (:Is%20Valid
      (Default|SetCollisiononKey _returnvalue))
    (:Is%20Not%20Valid
      _))
  (Variables|Default|SetStartFadeEffect true)
  (Utilities|FlowControl|Delay 0.5)
  (Audio|PlaySoundatLocation "/Game/DefinitiveSounds/RagnatelaBrucia/Flamethrower_Burst_01.Flamethrower_Burst_01" "0, 0, 0" "0, 0, 0" 1.0 1.0 0.0 "/Game/SoundSystem/SoundAttenuator/MainSoundAttenuator.MainSoundAttenuator" 0 0 0))

(event EventBeginPlay
  ;[1 1 1] Initialize
  (bind _pg1 (CallFunction|GetPlayer1))
  (Variables|Default|SetPG1 _pg1)
  (bind _pg3 (CallFunction|GetPlayer3))
  (Variables|Default|SetPG3 _pg3)
  (Rendering|Material|CreateDynamicMaterialInstance (Variables|Default|GetRagnatela) 0 (Variables|Default|GetSource%20Material) "None" :!class /Script/Engine.PrimitiveComponent))

(event EventTick
  (params (DeltaSeconds :type Float%20%28single-precision%29))
  (bind _bptavolettacesso (Variables|Cesso|GetBpTavolettaCesso))
  ;[1 1 1] Event tick
  (if (Variables|Default|GetStartFadeEffect)
    (bind _timefadeeffect (Timeline|FadeEffectRagnatela Play)
      (:Update
        (Rendering|Material|SetScalarParameterValueonMaterials (Variables|Default|GetRagnatela) "Fade_effect" _timefadeeffect))
      (:Finished
        (Utilities|IsValid _bptavolettacesso
          (:Is%20Valid
            (Default|CanbeGrabbed _bptavolettacesso))
          (:Is%20Not%20Valid
            _))
        (Actor|DestroyActor)))))

(fn ConstructionScript)