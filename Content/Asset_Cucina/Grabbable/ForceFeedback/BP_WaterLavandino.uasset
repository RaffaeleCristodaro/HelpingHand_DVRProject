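; Clogged sink water that drains in steps as a grabbed BPI_Unclogger actor repeatedly enters and leaves its trigger box.
; OnConstruction divides the start-to-end depth into stage heights, shown by instanced position markers.
; Each entry plays a sound and advances the count; each exit animates plane and box down one stage, with paired DoOnce gates enforcing alternation.
; The final entry disables collision, hides the water and deactivates Niagara.
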(event OnComponentBeginOverlap(Box)
  (params (OverlappedComponent :type Primitive%20Component%20Object%20Reference) (OtherActor :type Actor%20Object%20Reference) (OtherComp :type Primitive%20Component%20Object%20Reference) (OtherBodyIndex :type Integer) (bFromSweep :type Boolean) (SweepResult :type Hit%20Result%20Structure%20%28by%20ref%29))
  ;[0 0.5165 1 1 50] Overlaps
  ;;[1 1 1] Bog Begin Overlap
  (bind _isgrabbed_ (Class|BPIUnclogger|GetIsGrabbed(Message) OtherActor))
  (if (Math|Boolean|ANDBoolean _isgrabbed_ (Utilities|DoesObjectImplementInterface OtherActor "/Game/Managers/BlueprintInterfaces/BPI_Unclogger.BPI_Unclogger_C") (<= (+ (Variables|Default|GetCurrentNumberOfContactsForMakingWaterDisapear) 1) (Variables|Settings|GetUnclogIterations)))
    (Utilities|FlowControl|DoOnce false
      (:Completed
        (Audio|PlaySoundatLocation (Variables|Settings|GetSound) (Transformation|GetWorldLocation (Variables|Default|GetDefaultSceneRoot)) "0, 0, 0" 3.0 1.0 0.0 0 0 0 0)
        (Math|Integer|IncrementInt (Variables|Default|GetCurrentNumberOfContactsForMakingWaterDisapear)
          (:%20%20
            (CallFunction|ResetEndOverlap)
            (if (== (Variables|Default|GetCurrentNumberOfContactsForMakingWaterDisapear) (Variables|Settings|GetUnclogIterations))
              (Collision|SetCollisionEnabled (Variables|Default|GetBox) "NoCollision")
              (Rendering|SetVisibility (Variables|Default|GetCube) false false)
              (Components|Activation|Deactivate (Variables|Default|GetNiagara)))))))))

(event OnComponentEndOverlap(Box)
  (params (OverlappedComponent :type Primitive%20Component%20Object%20Reference) (OtherActor :type Actor%20Object%20Reference) (OtherComp :type Primitive%20Component%20Object%20Reference) (OtherBodyIndex :type Integer))
  (bind _cube (Variables|Default|GetCube))
  (bind _boxcolliderlocation (Variables|Settings|GetBoxColliderLocation))
  (bind _relativelocation (Variables|/Script/Engine.SceneComponent|GetRelativeLocation _cube))
  ;[0 0.5165 1 1 50] Overlaps
  ;;[1 1 1] Box End Overlap
  (bind _isgrabbed_ (Class|BPIUnclogger|GetIsGrabbed(Message) OtherActor))
  (if (and _isgrabbed_ (Utilities|DoesObjectImplementInterface OtherActor "/Game/Managers/BlueprintInterfaces/BPI_Unclogger.BPI_Unclogger_C"))
    (Utilities|FlowControl|DoOnce false
      (:Completed
        (Components|Timeline|SetPlayRate (Variables|Default|GetWaterAnim) 1.0)
        (bind _anim (Timeline|WaterAnim PlayFromStart)
          (:Update
            (Transformation|SetRelativeLocation (Variables|Default|GetCube) (Math|Vector|Lerp(Vector) (Math|Vector|MakeVector (.x _relativelocation) (.y _relativelocation) (Utilities|Array|Get(acopy) (Variables|Default|GetStages) (- (Variables|Default|GetCurrentNumberOfContactsForMakingWaterDisapear) 1))) (Math|Vector|MakeVector (.x _relativelocation) (.y _relativelocation) (Utilities|Array|Get(acopy) (Variables|Default|GetStages) (Variables|Default|GetCurrentNumberOfContactsForMakingWaterDisapear))) _anim) false false)
            (Transformation|SetRelativeLocation (Variables|Default|GetBox) (+ (Variables|/Script/Engine.SceneComponent|GetRelativeLocation (Variables|Default|GetCube)) (Math|Vector|MakeVector (.x _boxcolliderlocation) (.y _boxcolliderlocation) (+ (* (.z (Components|Box|GetScaledBoxExtent (Variables|Default|GetBox))) -1.0) (* (Variables|Settings|GetBoxColliderOffsetFromPlane) -1.0) 0.0))) false false))
          (:Finished
            (CallFunction|ResetBeginOverlap)))))))

(event Custom|ResetBeginOverlap
  ;[0 0.5165 1 1 50] Overlaps
  ;;[1 1 1] Bog Begin Overlap
  (Utilities|FlowControl|DoOnce false) ; enters at Reset
)

(event Custom|ResetEndOverlap
  (bind _cube (Variables|Default|GetCube))
  (bind _boxcolliderlocation (Variables|Settings|GetBoxColliderLocation))
  (bind _relativelocation (Variables|/Script/Engine.SceneComponent|GetRelativeLocation _cube))
  ;[0 0.5165 1 1 50] Overlaps
  ;;[1 1 1] Box End Overlap
  (Utilities|FlowControl|DoOnce false) ; enters at Reset
)

(event EventBeginPlay
  ;[1 0.06146 0.06146 1 50] Begin Play
  (CallFunction|OnConstruction))

(fn ConstructionScript
  (CallFunction|OnConstruction))

(fn OnConstruction
  (bind _cube (Variables|Default|GetCube))
  (bind _boxcolliderlocation (Variables|Settings|GetBoxColliderLocation))
  (bind _relativelocation (Variables|/Script/Engine.SceneComponent|GetRelativeLocation _cube))
  (Transformation|SetRelativeLocation (Variables|Default|GetStartPlaneLocation) (Variables|Settings|GetStartOffset) false false)
  (Transformation|SetRelativeLocation (Variables|Default|GetEndPlaneLocation) (Variables|Settings|GetEndOffset) false false)
  (Variables|Default|SetGapDistanceBetweenUnclogs (/ (+ (Math|Float|Absolute(Float) (.z (Variables|Settings|GetStartOffset))) (Math|Float|Absolute(Float) (.z (Variables|Settings|GetEndOffset)))) (Variables|Settings|GetUnclogIterations)))
  (Components|Box|SetBoxExtent (Variables|Default|GetBox) (Variables|Settings|GetBoxColliderExtents) true)
  (Transformation|SetRelativeLocation (Variables|Default|GetCube) (Math|Vector|MakeVector (.x _relativelocation) (.y _relativelocation) (.z (Variables|Settings|GetStartOffset))) false false)
  (Transformation|SetRelativeLocation (Variables|Default|GetPositions) (Variables|Settings|GetStartOffset) false false)
  (Transformation|SetRelativeLocation (Variables|Default|GetBox) (+ (Variables|Settings|GetStartOffset) (Math|Vector|MakeVector (.x _boxcolliderlocation) (.y _boxcolliderlocation) (+ (* (.z (Components|Box|GetScaledBoxExtent (Variables|Default|GetBox))) -1.0) (* (Variables|Settings|GetBoxColliderOffsetFromPlane) -1.0) 0.0))) false false)
  (Components|InstancedStaticMesh|ClearInstances (Variables|Default|GetPositions))
  (Utilities|Array|Clear (Variables|Default|GetStages))
  (for _index (range 0 (Variables|Settings|GetUnclogIterations))
    (Utilities|Array|Add (Variables|Default|GetStages) (* _index (Variables|Default|GetGapDistanceBetweenUnclogs) -1.0))
    (Components|InstancedStaticMesh|AddInstance (Variables|Default|GetPositions) (Math|Transform|MakeTransform (Math|Vector|MakeVector 0.0 0.0 (* _index (Variables|Default|GetGapDistanceBetweenUnclogs) -1.0)) "0, 0, 0" "1.000000,1.000000,1.000000") false)))