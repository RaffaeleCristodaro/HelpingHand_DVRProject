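; VR forced-teleport trigger that moves Player 1 to a set location and rotation when a BP_PG3 actor overlaps its box.
; The destination subtracts the yaw-rotated HMD camera offset to place the pawn correctly, with an IgnoreHeight option for Z.
; After firing, it disables itself and re-arms every other BP_ForcedTeleport in the level through the CanForceTeleport flag.
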(event OnComponentBeginOverlap(Box)
  (params (OverlappedComponent :type Primitive%20Component%20Object%20Reference) (OtherActor :type Actor%20Object%20Reference) (OtherComp :type Primitive%20Component%20Object%20Reference) (OtherBodyIndex :type Integer) (bFromSweep :type Boolean) (SweepResult :type Hit%20Result%20Structure%20%28by%20ref%29))
  (bind _returnvalue (Transformation|GetActorRotation))
  (bind _returnvalue_2 (Transformation|GetActorRotation))
  (bind _setplayerlocation (Variables|TeleportRef|GetSetPlayerLocation))
  (bind _pg1 (Variables|Default|GetPG1))
  (bind _pg1_2 (Variables|Default|GetPG1))
  (bind _pg1_3 (Variables|Default|GetPG1))
  (bind _setplayerlocation_2 (Variables|TeleportRef|GetSetPlayerLocation))
  (bind _returnvalue_3 (Transformation|GetActorLocation _pg1_2))
  (bind _camera (Variables|/Game/VRTemplate/Blueprints/VRPawn.VRPawn_C|GetCamera _pg1))
  (bind _camera_2 (Variables|/Game/VRTemplate/Blueprints/VRPawn.VRPawn_C|GetCamera _pg1_3))
  (bind _relativelocation (Variables|/Script/Engine.SceneComponent|GetRelativeLocation _camera))
  (bind _relativelocation_2 (Variables|/Script/Engine.SceneComponent|GetRelativeLocation _camera_2))
  (bind (_x _y) (Math|Vector|BreakVector _relativelocation_2))
  (bind (_x_2 _y_2) (Math|Vector|BreakVector _relativelocation))
  (bind _returnvalue_4 (Math|Vector|MakeVector _x _y 0.0))
  (bind _returnvalue_5 (Math|Vector|MakeVector _x_2 _y_2 (.z _returnvalue_3)))
  (bind _returnvalue_6 (Math|Vector|RotateVector _returnvalue_4 (Math|Rotator|MakeRotator 0.0 0.0 (.yaw _returnvalue))))
  (bind _returnvalue_7 (Math|Vector|RotateVector _returnvalue_5 (Math|Rotator|MakeRotator 0.0 0.0 (.yaw _returnvalue_2))))
  (bind _returnvalue_8 (- _setplayerlocation _returnvalue_6))
  (bind _returnvalue_9 (- _setplayerlocation_2 _returnvalue_7))
  ;[1 1 1] Forced Teleport
  (if (Variables|TeleportRef|GetMustActivateTeleportOnlyOnce)
    (Utilities|FlowControl|DoOnce false
      (:Completed
        _)))
  (if (Variables|Default|GetCanForceTeleport?)
    (Utilities|Casting|CastToBP_PG3 OtherActor)
    (if (Variables|TeleportRef|GetIgnoreHeight?)
      (Transformation|Teleport (Variables|Default|GetPG1) (Math|Vector|MakeVector (.x _returnvalue_9) (.y _returnvalue_9) 0.0) (Math|Rotator|MakeRotator 0.0 0.0 (.yaw _returnvalue_2)))
      (Transformation|SetActorRotation (Variables|Default|GetPG1) (Variables|TeleportRef|GetSetPlayerRotation))
      (CallFunction|ReactivateOtherForcedTeleports self)
      (else
        (Transformation|Teleport (Variables|Default|GetPG1) (Math|Vector|MakeVector (.x _returnvalue_8) (.y _returnvalue_8) (.z _returnvalue_8)) (Math|Rotator|MakeRotator 0.0 0.0 (.yaw _returnvalue)))
        (Transformation|SetActorRotation (Variables|Default|GetPG1) (Variables|TeleportRef|GetSetPlayerRotation))
        (CallFunction|ReactivateOtherForcedTeleports self)))))

(event EventBeginPlay
  ;[1 1 1] Initialize
  (bind _pg1 (CallFunction|GetPlayer1))
  (Variables|Default|SetPG1 _pg1))

(fn ConstructionScript
  (|CallParentFunction))

(fn ReactivateOtherForcedTeleports
  (params (ThisTeleport :type BP%20Forced%20Teleport%20Object%20Reference))
  (bind _outactors (Actor|GetAllActorsOfClass "BP_ForcedTeleport_C"))
  (for _array_element _outactors
    (Variables|BP_ForcedTeleport_C|SetCanForceTeleport? _array_element true))
  (Variables|BP_ForcedTeleport_C|SetCanForceTeleport? ThisTeleport false)
  (return))