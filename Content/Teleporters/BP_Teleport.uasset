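; BP_Teleport is a teleport point actor that offers itself to the player as a teleport when nearby and on screen.
; On BeginPlay it caches the player and all teleports.
; Each Tick it checks player distance and whether its projected screen position lies within the viewport, then flags itself usable and registers as the teleport the player is looking at.
; A check to hide it at close range exists but is unconnected.
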(event EventTick
  (params (DeltaSeconds :type Float%20%28single-precision%29))
  (bind _returnvalue (Transformation|GetActorLocation))
  (bind _returnvalue_2 (Viewport|GetViewportSize))
  (bind _returnvalue_3 (Game|GetPlayerController 0))
  (bind _screenlocation (Class|PlayerController|ProjectWorldLocationtoScreen _returnvalue_3 _returnvalue false))
  ;[1 1 1] OnScreen
  (bind _canbeactivated_ (CallFunction|CheckifPlayerIsinRangetoActivateTeleport (Variables|Teleport|GetPlayer%20Distance%20to%20Activate%20Teleport)))
  (CallFunction|StartingTeleport (Math|Boolean|ANDBoolean _canbeactivated_ (> (.x _screenlocation) 0.0) (> (.y _screenlocation) 0.0) (< (.x _screenlocation) (.x _returnvalue_2)) (< (.y _screenlocation) (.y _returnvalue_2)))))

(event EventBeginPlay
  ;[1 1 1] Initialize
  (bind _pg1 (CallFunction|GetPlayer1))
  (Variables|playerRef|SetPG1 _pg1)
  (bind _teleports (CallFunction|GetAllTeleports))
  (Variables|Teleport|SetTeleports _teleports))

(fn ConstructionScript)

(fn StartingTeleport
  (params (Condition :type Boolean))
  (if Condition
    (Variables|Teleport|SetCanBeUsedAsTeleport? true)
    (Variables|/Game/VRTemplate/Blueprints/VRPawn.VRPawn_C|SetTeleportPlayerIsLookingAt (Variables|playerRef|GetPG1) self)
    (else
      (Variables|Teleport|SetCanBeUsedAsTeleport? false))))

(fn CheckifPlayerIsinRangetoActivateTeleport
  (params (PlayerDistanceToActivateTeleport :type Float%20%28double-precision%29))
  (if (< (Math|Vector|VectorLength (- (Transformation|GetActorLocation (Variables|playerRef|GetPG1)) (Transformation|GetActorLocation))) PlayerDistanceToActivateTeleport)
    (LocalVariables|SetTeleportIsInRange? true)
    (else
      (LocalVariables|SetTeleportIsInRange? false)))
  (return (LocalVariables|GetTeleportIsInRange?)))

(fn CheckifPlayerIsinRangetoShutDownTeleport
  (params (PlayerInRangeToShutDownTeleport :type Float%20%28double-precision%29))
  (if (< (Math|Vector|VectorLength (- (Transformation|GetActorLocation (Variables|playerRef|GetPG1)) (Transformation|GetActorLocation))) PlayerInRangeToShutDownTeleport)
    (Variables|Teleport|SetCanBeSeen? false)
    (else
      (Variables|Teleport|SetCanBeSeen? true)))
  (return))