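; Teleport spawner that reveals a teleporter and moves it into place when PG3 enters its trigger box.
; The first overlap while CanTeleportSpawner is set starts a Tick-driven sequence.
; It destroys the placeholder mesh once, calls GameManager's SpawnTeleport at the start transform and activates the teleporter's Niagara effect.
; Constant-speed interpolation then moves and rotates the teleporter toward its final transform, stopping once the location matches.
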(event OnComponentBeginOverlap(Box)
  (params (OverlappedComponent :type Primitive%20Component%20Object%20Reference) (OtherActor :type Actor%20Object%20Reference) (OtherComp :type Primitive%20Component%20Object%20Reference) (OtherBodyIndex :type Integer) (bFromSweep :type Boolean) (SweepResult :type Hit%20Result%20Structure%20%28by%20ref%29))
  ;[1 1 1] Collsion with PG3
  (if (== OtherActor (Variables|Default|GetPG3))
    (if (Variables|Default|GetCanTeleportSpawner?)
      (Utilities|FlowControl|DoOnce false
        (:Completed
          (Variables|Teleport|SetCanSpawnTeleport? true))))))

(event EventBeginPlay
  ;[1 1 1] Initialize
  (bind _gamemanager (CallFunction|GetGameManager))
  (Variables|Default|SetGame%20Manager _gamemanager)
  (bind _pg3 (CallFunction|GetPlayer3))
  (Variables|Default|SetPG3 _pg3))

(event EventTick
  (params (DeltaSeconds :type Float%20%28single-precision%29))
  (bind _staticmesh (Variables|Default|GetStaticMesh))
  (bind _teleport (Variables|Teleport|GetTeleport))
  (bind _teleport_2 (Variables|Teleport|GetTeleport))
  (bind _teleport_3 (Variables|Teleport|GetTeleport))
  ;[1 1 1] Event tick
  (if (Variables|Teleport|GetCanSpawnTeleport?)
    (Utilities|FlowControl|Sequence
      (:then_0
        (Utilities|FlowControl|DoOnce false
          (:Completed
            (Utilities|IsValid _staticmesh
              (:Is%20Valid
                (Components|DestroyComponent _staticmesh))
              (:Is%20Not%20Valid
                _))
            (Default|SpawnTeleport (Variables|Default|GetGame%20Manager) (Variables|Teleport|GetTeleportStartLocation) (Variables|Teleport|GetTeleportStartRotation) _teleport_3)
            (Components|Activation|Activate (Variables|/Game/Teleporters/BP_Teleport.BP_Teleport_C|GetNiagara _teleport_3) false))))
      (:then_1
        (Transformation|SetActorLocation _teleport_2 (Math|Interpolation|VInterptoConstant (Transformation|GetActorLocation _teleport_2) (Variables|Teleport|GetFinalTeleportLocation) (Variables|Default|GetDelta%20Time) (Variables|Default|GetInterpSpeedLoc)) false false)
        (Transformation|SetActorRotation _teleport (Class|KismetMathLibrary|RInterptoConstant (Transformation|GetActorRotation _teleport) (Variables|Teleport|GetFinalTeleportRotation) (Variables|Default|GetDelta%20Time) (Variables|Default|GetInterpSpeedRot)))
        (if (Utilities|Operators|EqualEqual (Transformation|GetActorLocation _teleport) (Variables|Teleport|GetFinalTeleportLocation) 0.1)
          (Variables|Teleport|SetCanSpawnTeleport? false))))))

(fn ConstructionScript)