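; Records VR hand gestures for the Fire, Strenght and Super runes into the Save_HelpingHand save game.
; While the right Touch B button is held, Tick stores frame-to-frame offsets of the player's right-hand sphere, printing each and spawning a debug sphere.
; Release or reaching MaxPoints saves the offsets and preset gesture string to the slot picked by RuneToSave.
; The D key wipes all three saved gestures.
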(event Custom|StopRecording
  ;[1 1 1] Stop recording
  (if (Variables|gestures|GetCanRecord?)
    (Variables|gestures|SetCanStartRecording? false)
    (bind _returnvalue (SaveGame|DoesSaveGameExist "Save_HelpingHand"))
    (if _returnvalue
      (bind _returnvalue_2 (SaveGame|LoadGamefromSlot "Save_HelpingHand"))
      (bind _assg_helping_hand (Utilities|Casting|CastToSG_HelpingHand _returnvalue_2))
      (switch int (Variables|gestures|GetRuneToSave?)
        (:0
          (Variables|/Game/LoadingAndSaving/SG_HelpingHand.SG_HelpingHand_C|SetGestureFire _assg_helping_hand (Variables|gestures|GetGestureFireToRecord))
          (Variables|/Game/LoadingAndSaving/SG_HelpingHand.SG_HelpingHand_C|SetGestureLocationFireRune _assg_helping_hand (Variables|gestures|GetHandGestureLocation))
          (SaveGame|SaveGametoSlot _assg_helping_hand "Save_HelpingHand"))
        (:1
          (Variables|/Game/LoadingAndSaving/SG_HelpingHand.SG_HelpingHand_C|SetGestureStrenght _assg_helping_hand (Variables|gestures|GetGestureStrenghtToRecord))
          (Variables|/Game/LoadingAndSaving/SG_HelpingHand.SG_HelpingHand_C|SetGestureLocationStrenghtRune _assg_helping_hand (Variables|gestures|GetHandGestureLocation))
          (SaveGame|SaveGametoSlot _assg_helping_hand "Save_HelpingHand"))
        (:2
          (Variables|/Game/LoadingAndSaving/SG_HelpingHand.SG_HelpingHand_C|SetGestureSuper _assg_helping_hand (Variables|gestures|GetGestureSuperToRecord))
          (Variables|/Game/LoadingAndSaving/SG_HelpingHand.SG_HelpingHand_C|SetGestureLocationSuperRune _assg_helping_hand (Variables|gestures|GetHandGestureLocation))
          (SaveGame|SaveGametoSlot _assg_helping_hand "Save_HelpingHand"))))))

(event Custom|StartRecording
  ;[1 1 1] Record gesture
  (if (Variables|gestures|GetCanRecord?)
    (bind _returnvalue (SaveGame|DoesSaveGameExist "Save_HelpingHand"))
    (if _returnvalue
      (Variables|gestures|SetCanStartRecording? true)
      (Variables|gestures|SetPreviousHandGestureLocation (Transformation|GetWorldLocation (Variables|/Game/Characters/VRPawn.VRPawn_C|GetSphereRight (Variables|Default|GetPG1)))))))

(event EventBeginPlay
  ;[0 1 0.06763] Begin Play
  (bind _gamemanager (CallFunction|GetGameManager))
  (bind _output_get (Variables|Default|SetGame%20Manager _gamemanager))
  (Default|LoadGame _output_get)
  (bind _pg1 (CallFunction|GetPlayer1))
  (Variables|Default|SetPG1 _pg1))

(event EventTick
  (params (DeltaSeconds :type Float%20%28single-precision%29))
  ;[1 1 1] Event tick
  (if (and (Variables|gestures|GetCanStartRecording?) (Variables|gestures|GetCanRecord?))
    (if (< (Utilities|Array|Length (Variables|gestures|GetHandGestureLocation)) (Variables|gestures|GetMaxPoints))
      (Development|PrintString (Utilities|String|Append "----------------------------" (Utilities|String|ToString(Vector) (- (Variables|/Script/Engine.SceneComponent|GetRelativeLocation (Variables|/Game/Characters/VRPawn.VRPawn_C|GetSphereRight (Variables|Default|GetPG1))) (Variables|gestures|GetPreviousHandGestureLocation)))) true true "(R=0.000000,G=0.660000,B=1.000000,A=1.000000)" 0.008)
      (Utilities|Array|Add (Variables|gestures|GetHandGestureLocation) (- (Variables|/Script/Engine.SceneComponent|GetRelativeLocation (Variables|/Game/Characters/VRPawn.VRPawn_C|GetSphereRight (Variables|Default|GetPG1))) (Variables|gestures|GetPreviousHandGestureLocation)))
      (Game|SpawnActorfromClass "/Game/BP_SphereTest.BP_SphereTest_C" (Math|Transform|MakeTransform (- (Variables|/Script/Engine.SceneComponent|GetRelativeLocation (Variables|/Game/Characters/VRPawn.VRPawn_C|GetSphereRight (Variables|Default|GetPG1))) (Variables|gestures|GetPreviousHandGestureLocation)) "0, 0, 0" "1.000000,1.000000,1.000000") "Undefined" 0 0)
      (Variables|gestures|SetPreviousHandGestureLocation (Variables|/Script/Engine.SceneComponent|GetRelativeLocation (Variables|/Game/Characters/VRPawn.VRPawn_C|GetSphereRight (Variables|Default|GetPG1))))
      (else
        (CallFunction|StopRecording)))))

(event Input|ActionEvents|InputActionRuneModeBPress-OculusTouch(R)BPress
  (params (Key :type Key%20Structure :default "None"))
  ;[1 1 1] Input
  (:Pressed
    (CallFunction|StartRecording))
  (:Released
    (CallFunction|StopRecording)))

(event Input|KeyboardEvents|D
  (params (Key :type Key%20Structure :default "None"))
  (bind _handgesturelocationempty (Variables|gestures|GetHandGestureLocationEmpty))
  ;[1 1 1] Clear gesture
  (:Pressed
    (bind _returnvalue (SaveGame|DoesSaveGameExist "Save_HelpingHand"))
    (if _returnvalue
      (bind _returnvalue_2 (SaveGame|LoadGamefromSlot "Save_HelpingHand"))
      (bind _assg_helping_hand (Utilities|Casting|CastToSG_HelpingHand _returnvalue_2))
      (Variables|/Game/LoadingAndSaving/SG_HelpingHand.SG_HelpingHand_C|SetGestureFire _assg_helping_hand "")
      (Variables|/Game/LoadingAndSaving/SG_HelpingHand.SG_HelpingHand_C|SetGestureStrenght _assg_helping_hand "")
      (Variables|/Game/LoadingAndSaving/SG_HelpingHand.SG_HelpingHand_C|SetGestureSuper _assg_helping_hand "")
      (Variables|/Game/LoadingAndSaving/SG_HelpingHand.SG_HelpingHand_C|SetGestureLocationFireRune _assg_helping_hand _handgesturelocationempty)
      (Variables|/Game/LoadingAndSaving/SG_HelpingHand.SG_HelpingHand_C|SetGestureLocationStrenghtRune _assg_helping_hand _handgesturelocationempty)
      (Variables|/Game/LoadingAndSaving/SG_HelpingHand.SG_HelpingHand_C|SetGestureLocationSuperRune _assg_helping_hand _handgesturelocationempty)
      (SaveGame|SaveGametoSlot _assg_helping_hand "Save_HelpingHand"))))

(fn ConstructionScript)