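; VR toilet in the bathroom with a seat the player raises and lowers by hand.
; While GrabComponent is held, Tick maps the holding hand's world height to clamped seat roll, with IsYFridgeNegative flipping the sign.
; Past an angle threshold, it enables the spider web's box collision, apparently so it can burn.
; A distance check releases the grab unless the player's last toilet hit is valid; only the left hand checks height.
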(event OnGrabbed(GrabComponent)
  ;[1 1 1] On Grabbed
  (Variables|CessoRef|SetCanFollowPlayerHand? true))

(event OnDropped(GrabComponent)
  ;[1 1 1] On Grabbed
  (Variables|CessoRef|SetCanFollowPlayerHand? false))

(event Custom|CheckHandleDistanceFromLever
  (bind _pg1 (Variables|Default|GetPG1))
  (bind _wc_sm_tavoletta (Variables|Default|Getwc_SM_Tavoletta))
  (bind _wc_sm_tavoletta_2 (Variables|Default|Getwc_SM_Tavoletta))
  (bind _pg1_2 (Variables|Default|GetPG1))
  (bind _returnvalue (Transformation|GetWorldLocation _wc_sm_tavoletta_2))
  (bind _returnvalue_2 (Transformation|GetWorldLocation _wc_sm_tavoletta))
  (bind _lefthand (Variables|/Game/Characters/VRPawn.VRPawn_C|GetLeftHand _pg1_2))
  (bind _righthand (Variables|/Game/Characters/VRPawn.VRPawn_C|GetRightHand _pg1))
  (bind _returnvalue_3 (Transformation|GetWorldLocation _lefthand))
  (bind _returnvalue_4 (Transformation|GetWorldLocation _righthand))
  ;[1 1 1] Release hand from lever if too far
  (if (!= (Variables|/Game/Characters/VRPawn.VRPawn_C|GetHeldComponentLeft _pg1_2) 0)
    (if (Math|Boolean|ORBoolean (>= (Math|Float|Absolute(Float) (- (.x _returnvalue_3) (.x _returnvalue))) (Variables|CessoRef|GetMaxDistancefromFridgeToUseLeverX)) (>= (Math|Float|Absolute(Float) (- (.y _returnvalue_3) (.y _returnvalue))) (Variables|CessoRef|GetMaxDistancefromFridgeToUseLeverY)) (>= (Math|Float|Absolute(Float) (- (.z _returnvalue_3) (.z _returnvalue))) (Variables|CessoRef|GetMaxDistancefromFridgeToUseLeverZ)))
      (Utilities|IsValid (Variables|/Game/Characters/VRPawn.VRPawn_C|GetLastCessoHitLeft (Variables|Default|GetPG1))
        (:Is%20Not%20Valid
          (Default|TryRelease (Variables|Default|GetGrabComponent))
          (Variables|CessoRef|SetCanFollowPlayerHand? false))))
    (elif (!= (Variables|/Game/Characters/VRPawn.VRPawn_C|GetHeldComponentRight _pg1) 0)
      (if (or (>= (Math|Float|Absolute(Float) (- (.x _returnvalue_4) (.x _returnvalue_2))) (Variables|CessoRef|GetMaxDistancefromFridgeToUseLeverX)) (>= (Math|Float|Absolute(Float) (- (.y _returnvalue_4) (.y _returnvalue_2))) (Variables|CessoRef|GetMaxDistancefromFridgeToUseLeverX)))
        (Utilities|IsValid (Variables|/Game/Characters/VRPawn.VRPawn_C|GetLastCessoHitRight (Variables|Default|GetPG1))
          (:Is%20Not%20Valid
            (Default|TryRelease (Variables|Default|GetGrabComponent))
            (Variables|CessoRef|SetCanFollowPlayerHand? false)))))))

(event EventBeginPlay
  ;[1 1 1] Initialize
  (bind _pg1 (CallFunction|GetPlayer1))
  (Variables|Default|SetPG1 _pg1))

(event EventTick
  (params (DeltaSeconds :type Float%20%28single-precision%29))
  (bind _maxangle (Variables|CessoRef|GetMaxAngle))
  (bind _pg1 (Variables|Default|GetPG1))
  (bind _maxangle_2 (Variables|CessoRef|GetMaxAngle))
  (bind _grabtreeshold (Variables|CessoRef|GetGrabTreeshold))
  (bind _wc_sm_tavoletta (Variables|Default|Getwc_SM_Tavoletta))
  (bind _minangle (Variables|CessoRef|GetMinAngle))
  (bind _maxangle_3 (Variables|CessoRef|GetMaxAngle))
  (bind _minangle_2 (Variables|CessoRef|GetMinAngle))
  (bind _grabtreeshold_2 (Variables|CessoRef|GetGrabTreeshold))
  (bind _pg1_2 (Variables|Default|GetPG1))
  (bind _wc_sm_tavoletta_2 (Variables|Default|Getwc_SM_Tavoletta))
  (bind _maxangle_4 (Variables|CessoRef|GetMaxAngle))
  (bind _minangle_3 (Variables|CessoRef|GetMinAngle))
  (bind _minangle_4 (Variables|CessoRef|GetMinAngle))
  (bind _pg1_3 (Variables|Default|GetPG1))
  (bind _grabtreeshold_3 (Variables|CessoRef|GetGrabTreeshold))
  (bind _wc_sm_tavoletta_3 (Variables|Default|Getwc_SM_Tavoletta))
  (bind _wc_sm_tavoletta_4 (Variables|Default|Getwc_SM_Tavoletta))
  (bind _grabtreeshold_4 (Variables|CessoRef|GetGrabTreeshold))
  (bind _pg1_4 (Variables|Default|GetPG1))
  (bind _returnvalue (Transformation|GetWorldRotation _wc_sm_tavoletta_3))
  (bind _returnvalue_2 (Transformation|GetWorldRotation _wc_sm_tavoletta_4))
  (bind _returnvalue_3 (Transformation|GetWorldRotation _wc_sm_tavoletta_2))
  (bind _returnvalue_4 (Transformation|GetWorldRotation _wc_sm_tavoletta))
  (bind _sphereright (Variables|/Game/Characters/VRPawn.VRPawn_C|GetSphereRight _pg1_4))
  (bind _sphereleft (Variables|/Game/Characters/VRPawn.VRPawn_C|GetSphereLeft _pg1))
  (bind _sphereleft_2 (Variables|/Game/Characters/VRPawn.VRPawn_C|GetSphereLeft _pg1_2))
  (bind _sphereright_2 (Variables|/Game/Characters/VRPawn.VRPawn_C|GetSphereRight _pg1_3))
  (bind _returnvalue_5 (Transformation|GetWorldLocation _sphereright_2))
  (bind _returnvalue_6 (Transformation|GetWorldLocation _sphereright))
  (bind _returnvalue_7 (Transformation|GetWorldLocation _sphereleft))
  (bind _returnvalue_8 (Transformation|GetWorldLocation _sphereleft_2))
  (bind _returnvalue_9 (Math|Float|Absolute(Float) (.z _returnvalue_5)))
  (bind _returnvalue_10 (Math|Float|Absolute(Float) (.z _returnvalue_8)))
  (bind _returnvalue_11 (Math|Float|Absolute(Float) (.z _returnvalue_6)))
  (bind _returnvalue_12 (Math|Float|Absolute(Float) (.z _returnvalue_7)))
  (bind _returnvalue_13 (- _returnvalue_11 _grabtreeshold_4))
  (bind _returnvalue_14 (- _returnvalue_9 _grabtreeshold_3))
  (bind _returnvalue_15 (- _returnvalue_12 _grabtreeshold))
  (bind _returnvalue_16 (- _returnvalue_10 _grabtreeshold_2))
  (bind _returnvalue_17 (Math|Float|Clamp(Float) _returnvalue_13 _minangle_2 _maxangle_4))
  (bind _returnvalue_18 (Math|Float|Clamp(Float) _returnvalue_15 _minangle_4 _maxangle))
  (bind _returnvalue_19 (* _returnvalue_16 -1.0))
  (bind _returnvalue_20 (* _returnvalue_14 -1.0))
  (bind _returnvalue_21 (Math|Float|Clamp(Float) _returnvalue_19 _minangle _maxangle_3))
  (bind _returnvalue_22 (Math|Float|Clamp(Float) _returnvalue_20 _minangle_3 _maxangle_2))
  (bind _returnvalue_23 (* _returnvalue_17 -1.0))
  (bind _returnvalue_24 (* _returnvalue_18 -1.0))
  ;[1 1 1] Event tick
  (if (Variables|CessoRef|GetCanFollowPlayerHand?)
    (CallFunction|CheckHandleDistancefromLever)
    (if (Variables|CessoRef|GetIsYFridgeNegative?)
      (if (!= (Variables|/Game/Characters/VRPawn.VRPawn_C|GetHeldComponentLeft (Variables|Default|GetPG1)) 0)
        (if (Variables|Default|GetTesting?)
          (Development|PrintString (Utilities|String|ToString(Float) _returnvalue_15)))
        (Transformation|SetWorldRotation (Variables|Default|Getwc_SM_Tavoletta) (Math|Rotator|MakeRotator _returnvalue_24 (.pitch _returnvalue_2) (.yaw _returnvalue_2)) false false)
        (if (>= (* _returnvalue_24 -1.0) (Variables|InteractRef|GetZRotationForBurnableSpiderWeb))
          (Collision|SetCollisionEnabled (Variables|/Game/Asset_Cucina/Grabbable/BP/BP_Ragnatela.BP_Ragnatela_C|GetBox (Variables|InteractRef|GetRagnatela)) "QueryAndPhysics")
          (else
            (Collision|SetCollisionEnabled (Variables|/Game/Asset_Cucina/Grabbable/BP/BP_Ragnatela.BP_Ragnatela_C|GetBox (Variables|InteractRef|GetRagnatela)) "NoCollision")))
        (elif (!= (Variables|/Game/Characters/VRPawn.VRPawn_C|GetHeldComponentRight (Variables|Default|GetPG1)) 0)
          (if (Variables|Default|GetTesting?)
            (Development|PrintString (Utilities|String|ToString(Float) _returnvalue_13)))
          (Transformation|SetWorldRotation (Variables|Default|Getwc_SM_Tavoletta) (Math|Rotator|MakeRotator _returnvalue_23 (.pitch _returnvalue) (.yaw _returnvalue)) false false)
          (if (>= (* _returnvalue_23 -1.0) (Variables|InteractRef|GetZRotationForBurnableSpiderWeb))
            (Collision|SetCollisionEnabled (Variables|/Game/Asset_Cucina/Grabbable/BP/BP_Ragnatela.BP_Ragnatela_C|GetBox (Variables|InteractRef|GetRagnatela)) "QueryAndPhysics")
            (else
              (Collision|SetCollisionEnabled (Variables|/Game/Asset_Cucina/Grabbable/BP/BP_Ragnatela.BP_Ragnatela_C|GetBox (Variables|InteractRef|GetRagnatela)) "NoCollision")))))
      (elif (!= (Variables|/Game/Characters/VRPawn.VRPawn_C|GetHeldComponentLeft (Variables|Default|GetPG1)) 0)
        (if (Variables|Default|GetTesting?)
          (Development|PrintString (Utilities|String|ToString(Float) _returnvalue_16)))
        (Transformation|SetWorldRotation (Variables|Default|Getwc_SM_Tavoletta) (Math|Rotator|MakeRotator _returnvalue_21 (.pitch _returnvalue_4) (.yaw _returnvalue_4)) false false)
        (if (>= _returnvalue_21 (Variables|InteractRef|GetZRotationForBurnableSpiderWeb))
          (Collision|SetCollisionEnabled (Variables|/Game/Asset_Cucina/Grabbable/BP/BP_Ragnatela.BP_Ragnatela_C|GetBox (Variables|InteractRef|GetRagnatela)) "QueryAndPhysics")
          (else
            (Collision|SetCollisionEnabled (Variables|/Game/Asset_Cucina/Grabbable/BP/BP_Ragnatela.BP_Ragnatela_C|GetBox (Variables|InteractRef|GetRagnatela)) "NoCollision")))
        (elif (!= (Variables|/Game/Characters/VRPawn.VRPawn_C|GetHeldComponentRight (Variables|Default|GetPG1)) 0)
          (if (Variables|Default|GetTesting?)
            (Development|PrintString (Utilities|String|ToString(Float) _returnvalue_14)))
          (Transformation|SetWorldRotation (Variables|Default|Getwc_SM_Tavoletta) (Math|Rotator|MakeRotator _returnvalue_22 (.pitch _returnvalue_3) (.yaw _returnvalue_3)) false false)
          (if (>= _returnvalue_22 (Variables|InteractRef|GetZRotationForBurnableSpiderWeb))
            (Collision|SetCollisionEnabled (Variables|/Game/Asset_Cucina/Grabbable/BP/BP_Ragnatela.BP_Ragnatela_C|GetBox (Variables|InteractRef|GetRagnatela)) "QueryAndPhysics")
            (else
              (Collision|SetCollisionEnabled (Variables|/Game/Asset_Cucina/Grabbable/BP/BP_Ragnatela.BP_Ragnatela_C|GetBox (Variables|InteractRef|GetRagnatela)) "NoCollision"))))))))

(fn ConstructionScript)