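; BP_Vasca is a bathroom tub actor that switches the collision type of floatable objects entering or leaving its box volume.
; Box overlap events compare the other actor against the ActorsThatCanFloat list.
; A match has its StaticMesh collision object type set to WorldDynamic on entry and back to PhysicsBody on exit.
; The Blueprint itself applies no buoyancy forces.
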(event OnComponentBeginOverlap(Box)
  (params (OverlappedComponent :type Primitive%20Component%20Object%20Reference) (OtherActor :type Actor%20Object%20Reference) (OtherComp :type Primitive%20Component%20Object%20Reference) (OtherBodyIndex :type Integer) (bFromSweep :type Boolean) (SweepResult :type Hit%20Result%20Structure%20%28by%20ref%29))
  ;[1 1 1] CheckCollision
  (for _array_element (Variables|Default|GetActorsThatCanFloat)
    (if (== _array_element OtherActor)
      (Collision|SetCollisionObjectType (Variables|/Game/Blueprint_Grabbable/BP_InteractiveGrabbablesParent.BP_InteractiveGrabbablesParent_C|GetStaticMesh _array_element) "ECC_WorldDynamic"))))

(event OnComponentEndOverlap(Box)
  (params (OverlappedComponent :type Primitive%20Component%20Object%20Reference) (OtherActor :type Actor%20Object%20Reference) (OtherComp :type Primitive%20Component%20Object%20Reference) (OtherBodyIndex :type Integer))
  ;[1 1 1] CheckCollision
  (for _array_element (Variables|Default|GetActorsThatCanFloat)
    (if (== _array_element OtherActor)
      (Collision|SetCollisionObjectType (Variables|/Game/Blueprint_Grabbable/BP_InteractiveGrabbablesParent.BP_InteractiveGrabbablesParent_C|GetStaticMesh _array_element) "ECC_PhysicsBody"))))

(fn ConstructionScript)