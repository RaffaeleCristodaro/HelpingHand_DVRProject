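; BP_AsseDaRompere is a breakable wooden plank in the bathroom assets, made of left and right plank meshes and a trigger box.
; When the VRPawn overlaps the box, a one-time gate turns on physics for both halves so the plank comes apart.
; The whole actor destroys itself after a short delay.
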(event OnComponentBeginOverlap(Box)
  (params (OverlappedComponent :type Primitive%20Component%20Object%20Reference) (OtherActor :type Actor%20Object%20Reference) (OtherComp :type Primitive%20Component%20Object%20Reference) (OtherBodyIndex :type Integer) (bFromSweep :type Boolean) (SweepResult :type Hit%20Result%20Structure%20%28by%20ref%29))
  ;[1 1 1] Collision with PG1
  (Utilities|Casting|CastToVRPawn OtherActor)
  (if true
    (Utilities|FlowControl|DoOnce false
      (:Completed
        (Physics|SetSimulatePhysics (Variables|Default|GetSM_AsseLegnoLeft) true)
        (Physics|SetSimulatePhysics (Variables|Default|GetSM_AsseLegnoRigth) true)
        (Utilities|IsValid (Variables|Default|GetSM_AsseLegnoLeft)
          (:Is%20Valid
            (Utilities|FlowControl|Delay 5.0)
            (Actor|DestroyActor)))))))

(fn ConstructionScript)