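; BP_Mirror is a broken bathroom mirror that is rebuilt from glass shards the player carries with telekinesis.
; Its shard-release logic releases the player's right-hand grab, clears the shard from both hands' hit lists, reveals the slot matching its GlassIndex and destroys it.
; RestoreGlass counts placed shards and, once the total is reached, hides the broken mirror and slot pieces and shows the intact mirror.
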(event Custom|RestoreGlass
  (bind _currentnumberofglass (Variables|Default|GetCurrentNumberOfGlass))
  ;[1 1 1] Ricomponi specchio
  (Math|Integer|IncrementInt _currentnumberofglass
    (:%20%20
      (if (>= _currentnumberofglass (Variables|Default|GetTotNumberOfGlass))
        (Development|SetHiddeninGame (Variables|Default|GetSpecchioIntero) false false)
        (Development|SetHiddeninGame (Variables|Default|GetSpecchioRotto) true false)
        (Development|SetHiddeninGame (Variables|Default|GetGlassShard1) true false)
        (Development|SetHiddeninGame (Variables|Default|GetGlassShard2) true false)
        (Development|SetHiddeninGame (Variables|Default|GetGlassShard3) true false)))))

(event Custom|DetachGlassShard
  (params (GlassShard :type BPG%20Glass%20Shard%20Object%20Reference))
  ;[1 1 1] Detach glass shard
)

(event EventBeginPlay
  ;[1 1 1] Initialize
  (bind _pg1 (CallFunction|GetPlayer1))
  (Variables|Default|SetPG1 _pg1))

(fn ConstructionScript)

(fn CheckGlassShard
  (params (GlassIndex :type Integer))
  (switch int GlassIndex
    (:Default
      (Development|SetHiddeninGame (Variables|Default|GetGlassShard1) false false :!label _label))
    (:0
      (goto _label))
    (:1
      (Development|SetHiddeninGame (Variables|Default|GetGlassShard2) false false))
    (:2
      (Development|SetHiddeninGame (Variables|Default|GetGlassShard3) false false)))
  (return))