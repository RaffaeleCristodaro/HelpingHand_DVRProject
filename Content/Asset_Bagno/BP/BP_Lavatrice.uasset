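; Interactive VR washing machine with a pressable button, spinning drum and grabbable door.
; On Tick, player overlap slides the button, and a DoOnce plus FlipFlop alternates on and off once per press.
; On plays the sound, spins the drum, resets the door and disables its collision; off stops the sound and restores collision.
; While off, a grabbed door's clamped yaw follows the hand's world Y, auto-releasing when the hand strays too far.
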(event OnDropped(GrabComponent)
  ;[1 1 1] OnGrab
  (Variables|Lavatrice|SetCanFollowPlayerHand? false))

(event OnGrabbed(GrabComponent)
  ;[1 1 1] OnGrab
  (if (not (Variables|Lavatrice|GetIsLavatriceOn?))
    (Variables|Lavatrice|SetCanFollowPlayerHand? true)))

(event Custom|CheckHandleDistanceFromLever
  (bind _pg1 (Variables|Default|GetPG1))
  (bind _lavatrice_sm_sportello_lavatrice (Variables|Default|GetLavatrice_SM_Sportello_Lavatrice))
  (bind _lavatrice_sm_sportello_lavatrice_2 (Variables|Default|GetLavatrice_SM_Sportello_Lavatrice))
  (bind _returnvalue (Transformation|GetWorldLocation _lavatrice_sm_sportello_lavatrice_2))
  (bind _returnvalue_2 (Transformation|GetWorldLocation _lavatrice_sm_sportello_lavatrice))
  (bind _lefthand (Variables|/Game/VRTemplate/Blueprints/VRPawn.VRPawn_C|GetLeftHand _pg1))
  (bind _righthand (Variables|/Game/VRTemplate/Blueprints/VRPawn.VRPawn_C|GetRightHand _pg1))
  (bind _returnvalue_3 (Transformation|GetWorldLocation _lefthand))
  (bind _returnvalue_4 (Transformation|GetWorldLocation _righthand))
  ;[1 1 1] Release hand from lever if too far
  (if (!= (Variables|/Game/VRTemplate/Blueprints/VRPawn.VRPawn_C|GetHeldComponentLeft _pg1) 0)
    (if (Math|Boolean|ORBoolean (>= (Math|Float|Absolute(Float) (- (.x _returnvalue_3) (.x _returnvalue))) (Variables|Lavatrice|GetMaxDistancefromFridgeToUseLeverX)) (>= (Math|Float|Absolute(Float) (- (.y _returnvalue_3) (.y _returnvalue))) (Variables|Lavatrice|GetMaxDistancefromFridgeToUseLeverY)) (>= (Math|Float|Absolute(Float) (- (.z _returnvalue_3) (.z _returnvalue))) (Variables|Lavatrice|GetMaxDistancefromFridgeToUseLeverZ)))
      (Default|TryRelease (Variables|Default|GetGrabComponent) (Variables|/Game/VRTemplate/Blueprints/VRPawn.VRPawn_C|GetMotionControllerLeft (Variables|Default|GetPG1)))
      (Variables|Lavatrice|SetCanFollowPlayerHand? false))
    (elif (!= (Variables|/Game/VRTemplate/Blueprints/VRPawn.VRPawn_C|GetHeldComponentRight _pg1) 0)
      (if (or (>= (Math|Float|Absolute(Float) (- (.x _returnvalue_4) (.x _returnvalue_2))) (Variables|Lavatrice|GetMaxDistancefromFridgeToUseLeverX)) (>= (Math|Float|Absolute(Float) (- (.y _returnvalue_4) (.y _returnvalue_2))) (Variables|Lavatrice|GetMaxDistancefromFridgeToUseLeverX)))
        (Default|TryRelease (Variables|Default|GetGrabComponent) (Variables|/Game/VRTemplate/Blueprints/VRPawn.VRPawn_C|GetMotionControllerRight (Variables|Default|GetPG1)))
        (Variables|Lavatrice|SetCanFollowPlayerHand? false)))))

(event EventBeginPlay
  (bind _lavatrice_sm_sportello_lavatrice (Variables|Default|GetLavatrice_SM_Sportello_Lavatrice))
  ;[1 1 1] Initialize
  (bind _pg1 (CallFunction|GetPlayer1))
  (Variables|Default|SetPG1 _pg1)
  (Collision|SetCollisionEnabled _lavatrice_sm_sportello_lavatrice "NoCollision")
  (Variables|Lavatrice|SetInitialRotation (Transformation|GetWorldRotation _lavatrice_sm_sportello_lavatrice)))

(event EventTick
  (params (DeltaSeconds :type Float%20%28single-precision%29))
  (bind _pg1 (Variables|Default|GetPG1))
  (bind _minoffsetbuttons (Variables|Button|GetMinOffsetButtons))
  (bind _maxoffsetbuttons (Variables|Button|GetMaxOffsetButtons))
  (bind _minoffsetbuttons_2 (Variables|Button|GetMinOffsetButtons))
  (bind _maxoffsetbuttons_2 (Variables|Button|GetMaxOffsetButtons))
  (bind _grabtreeshold (Variables|Lavatrice|GetGrabTreeshold))
  (bind _speedrotationlavatriceinterna (Variables|Lavatrice|GetSpeedRotationLavatriceInterna))
  (bind _grabtreeshold_2 (Variables|Lavatrice|GetGrabTreeshold))
  (bind _pg1_2 (Variables|Default|GetPG1))
  (bind _lavatrice_pulsante_sm_pulsante (Variables|Default|GetLavatrice_Pulsante_SM_Pulsante))
  (bind _lavatrice_pulsante_sm_pulsante_2 (Variables|Default|GetLavatrice_Pulsante_SM_Pulsante))
  (bind _lavatrice_sm_cestello (Variables|Default|GetLavatrice_SM_Cestello))
  (bind _soundbuttonclick (Variables|Button|GetSoundButtonClick))
  (bind _lavatrice_sm_sportello_lavatrice (Variables|Default|GetLavatrice_SM_Sportello_Lavatrice))
  (bind _lavatrice_sm_sportello_lavatrice_2 (Variables|Default|GetLavatrice_SM_Sportello_Lavatrice))
  (bind _lavatrice_sm_sportello_lavatrice_3 (Variables|Default|GetLavatrice_SM_Sportello_Lavatrice))
  (bind _lavatrice_sm_sportello_lavatrice_4 (Variables|Default|GetLavatrice_SM_Sportello_Lavatrice))
  (bind _pg1_3 (Variables|Default|GetPG1))
  (bind _grabtreeshold_3 (Variables|Lavatrice|GetGrabTreeshold))
  (bind _grabtreeshold_4 (Variables|Lavatrice|GetGrabTreeshold))
  (bind _pg1_4 (Variables|Default|GetPG1))
  (bind _returnvalue (Transformation|GetWorldRotation _lavatrice_sm_sportello_lavatrice_3))
  (bind _returnvalue_2 (Transformation|GetRelativeTransform _lavatrice_pulsante_sm_pulsante))
  (bind _returnvalue_3 (Transformation|GetWorldRotation _lavatrice_sm_sportello_lavatrice_2))
  (bind _returnvalue_4 (Transformation|GetWorldRotation _lavatrice_sm_sportello_lavatrice))
  (bind _returnvalue_5 (Transformation|GetWorldRotation _lavatrice_sm_sportello_lavatrice_4))
  (bind _returnvalue_6 (Transformation|GetRelativeTransform _lavatrice_pulsante_sm_pulsante_2))
  (bind _sphereleft (Variables|/Game/VRTemplate/Blueprints/VRPawn.VRPawn_C|GetSphereLeft _pg1))
  (bind _sphereright (Variables|/Game/VRTemplate/Blueprints/VRPawn.VRPawn_C|GetSphereRight _pg1_4))
  (bind _sphereleft_2 (Variables|/Game/VRTemplate/Blueprints/VRPawn.VRPawn_C|GetSphereLeft _pg1_2))
  (bind _sphereright_2 (Variables|/Game/VRTemplate/Blueprints/VRPawn.VRPawn_C|GetSphereRight _pg1_3))
  (bind _relativerotation (Variables|/Script/Engine.SceneComponent|GetRelativeRotation _lavatrice_sm_cestello))
  (bind _returnvalue_7 (Transformation|GetWorldLocation _sphereright_2))
  (bind _returnvalue_8 (Transformation|GetWorldLocation _sphereright))
  (bind _returnvalue_9 (Transformation|GetWorldLocation _sphereleft))
  (bind _returnvalue_10 (Transformation|GetWorldLocation _sphereleft_2))
  (bind _returnvalue_11 (+ (.pitch _relativerotation) _speedrotationlavatriceinterna))
  (bind _returnvalue_12 (- (.location _returnvalue_2) "0.000000,3.000000,0.000000"))
  (bind _returnvalue_13 (+ (.location _returnvalue_6) "0.000000,3.000000,0.000000"))
  (bind _returnvalue_14 (Math|Float|Absolute(Float) (.y _returnvalue_7)))
  (bind _returnvalue_15 (Math|Float|Clamp(Float) (.y _returnvalue_12) _minoffsetbuttons_2 _maxoffsetbuttons_2))
  (bind _returnvalue_16 (Math|Float|Clamp(Float) (.y _returnvalue_13) _minoffsetbuttons _maxoffsetbuttons))
  (bind _returnvalue_17 (Math|Float|Absolute(Float) (.y _returnvalue_8)))
  (bind _returnvalue_18 (Math|Float|Absolute(Float) (.y _returnvalue_9)))
  (bind _returnvalue_19 (Math|Float|Absolute(Float) (.y _returnvalue_10)))
  (bind _returnvalue_20 (- _returnvalue_17 _grabtreeshold_4))
  (bind _returnvalue_21 (- _returnvalue_14 _grabtreeshold_3))
  (bind _returnvalue_22 (- _returnvalue_18 _grabtreeshold))
  (bind _returnvalue_23 (- _returnvalue_19 _grabtreeshold_2))
  ;[1 1 1] Event tick
  (Utilities|FlowControl|Sequence
    (:then_0
      (if (Collision|IsOverlappingActor (Variables|Default|GetLavatrice_Pulsante_SM_Pulsante_Collsion) (Variables|Default|GetPG1) :!class /Script/Engine.PrimitiveComponent)
        (Components|MoveComponentTo _lavatrice_pulsante_sm_pulsante (Math|Vector|MakeVector (.x _returnvalue_12) _returnvalue_15 (.z _returnvalue_12)) (.rotation _returnvalue_2) false true (Variables|Button|GetOver%20Time) false)
        (if (<= _returnvalue_15 (/ (+ (Variables|Button|GetMinOffsetButtons) (Variables|Button|GetMaxOffsetButtons)) (Variables|Button|GetTriggerTime)))
          (Utilities|FlowControl|DoOnce false :!label _label
            (:Completed
              (Utilities|IsValid _soundbuttonclick
                (:Is%20Valid
                  (Audio|PlaySound2D _soundbuttonclick 1.0 1.0 0.0 0 0))
                (:Is%20Not%20Valid
                  _))
              (Utilities|FlowControl|FlipFlop
                (:A
                  (Variables|Lavatrice|SetIsLavatriceOn? false)
                  (Collision|SetCollisionEnabled (Variables|Default|GetLavatrice_SM_Sportello_Lavatrice) "QueryAndPhysics")
                  (Utilities|IsValid (Variables|Default|GetSoundLavatriceOn)
                    (:Is%20Valid
                      (Audio|Components|Audio|Stop (Variables|Default|GetSoundLavatriceOn)))))
                (:B
                  (Variables|Lavatrice|SetIsLavatriceOn? true)
                  (Collision|SetCollisionEnabled (Variables|Default|GetLavatrice_SM_Sportello_Lavatrice) "NoCollision")
                  (Variables|Lavatrice|SetCanFollowPlayerHand? false)
                  (bind _returnvalue_24 (Audio|SpawnSound2D (Variables|Lavatrice|GetSoundLavatrice) 1.0 1.0 0.0 0))
                  (Variables|Default|SetSoundLavatriceOn _returnvalue_24)
                  (Transformation|SetWorldRotation (Variables|Default|GetLavatrice_SM_Sportello_Lavatrice) (Variables|Lavatrice|GetInitialRotation) false false))))))
        (else
          (Components|MoveComponentTo _lavatrice_pulsante_sm_pulsante_2 (Math|Vector|MakeVector (.x _returnvalue_13) _returnvalue_16 (.z _returnvalue_13)) (.rotation _returnvalue_6) false true (Variables|Button|GetOver%20Time) false)
          (if (>= _returnvalue_16 (Variables|Button|GetMaxOffsetButtons))
            (goto _label Reset)))))
    (:then_1
      (if (Variables|Lavatrice|GetIsLavatriceOn?)
        (Transformation|SetRelativeRotation _lavatrice_sm_cestello (Math|Rotator|MakeRotator (.roll _relativerotation) _returnvalue_11 (.yaw _relativerotation)) false false)
        (if (>= _returnvalue_11 9e+01)
          (Transformation|SetRelativeRotation _lavatrice_sm_cestello (Math|Rotator|MakeRotator (.roll _relativerotation) 0.0 (.yaw _relativerotation)) false false))))
    (:then_2
      (if (Variables|Lavatrice|GetCanFollowPlayerHand?)
        (CallFunction|CheckHandleDistancefromLever)
        (if (Variables|Lavatrice|GetIsYFridgeNegative?)
          (if (!= (Variables|/Game/VRTemplate/Blueprints/VRPawn.VRPawn_C|GetHeldComponentLeft (Variables|Default|GetPG1)) 0)
            (if (Variables|Default|GetTesting?)
              (Development|PrintString (Utilities|String|ToString(Float) _returnvalue_22)))
            (Transformation|SetWorldRotation (Variables|Default|GetLavatrice_SM_Sportello_Lavatrice) (Math|Rotator|MakeRotator (.roll _returnvalue_3) (.pitch _returnvalue_3) (Math|Float|Clamp(Float) _returnvalue_22 (Variables|Lavatrice|GetMinAngle) (Variables|Lavatrice|GetMaxAngle))) false false)
            (elif (!= (Variables|/Game/VRTemplate/Blueprints/VRPawn.VRPawn_C|GetHeldComponentRight (Variables|Default|GetPG1)) 0)
              (if (Variables|Default|GetTesting?)
                (Development|PrintString (Utilities|String|ToString(Float) _returnvalue_20)))
              (Transformation|SetWorldRotation (Variables|Default|GetLavatrice_SM_Sportello_Lavatrice) (Math|Rotator|MakeRotator (.roll _returnvalue) (.pitch _returnvalue) (Math|Float|Clamp(Float) _returnvalue_20 (Variables|Lavatrice|GetMinAngle) (Variables|Lavatrice|GetMaxAngle))) false false)))
          (elif (!= (Variables|/Game/VRTemplate/Blueprints/VRPawn.VRPawn_C|GetHeldComponentLeft (Variables|Default|GetPG1)) 0)
            (if (Variables|Default|GetTesting?)
              (Development|PrintString (Utilities|String|ToString(Float) _returnvalue_23)))
            (Transformation|SetWorldRotation (Variables|Default|GetLavatrice_SM_Sportello_Lavatrice) (Math|Rotator|MakeRotator (.roll _returnvalue_5) (.pitch _returnvalue_5) (* (Math|Float|Clamp(Float) _returnvalue_23 (Variables|Lavatrice|GetMinAngle) (Variables|Lavatrice|GetMaxAngle)) -1.0)) false false)
            (elif (!= (Variables|/Game/VRTemplate/Blueprints/VRPawn.VRPawn_C|GetHeldComponentRight (Variables|Default|GetPG1)) 0)
              (if (Variables|Default|GetTesting?)
                (Development|PrintString (Utilities|String|ToString(Float) _returnvalue_21)))
              (Transformation|SetWorldRotation (Variables|Default|GetLavatrice_SM_Sportello_Lavatrice) (Math|Rotator|MakeRotator (.roll _returnvalue_4) (.pitch _returnvalue_4) (* (Math|Float|Clamp(Float) _returnvalue_21 (Variables|Lavatrice|GetMinAngle) (Variables|Lavatrice|GetMaxAngle)) -1.0)) false false))))))))

(fn ConstructionScript)