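; VR interactable fridge whose door (PortaFrigo) swings with the player's grabbing hand while unlocked.
; Grab and release events toggle following, and Tick sets door yaw from the hand sphere's absolute world Y minus a threshold, clamped and sign-flipped by IsYFridgeNegative.
; A distance check force-releases the hand when too far, testing X/Y/Z for the left but only X/Y for the right, both against the X limit.
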(event Custom|CheckHandleDistanceFromLever
  (bind _scene (Variables|Default|GetScene))
  (bind _scene_2 (Variables|Default|GetScene))
  (bind _pg1 (Variables|Default|GetPG1))
  (bind _returnvalue (Transformation|GetWorldLocation _scene_2))
  (bind _returnvalue_2 (Transformation|GetWorldLocation _scene))
  (bind _lefthand (Variables|/Game/VRTemplate/Blueprints/VRPawn.VRPawn_C|GetLeftHand _pg1))
  (bind _righthand (Variables|/Game/VRTemplate/Blueprints/VRPawn.VRPawn_C|GetRightHand _pg1))
  (bind _returnvalue_3 (Transformation|GetWorldLocation _lefthand))
  (bind _returnvalue_4 (Transformation|GetWorldLocation _righthand))
  ;[1 1 1] Release hand from lever if too far
  (if (!= (Variables|/Game/VRTemplate/Blueprints/VRPawn.VRPawn_C|GetHeldComponentLeft _pg1) 0)
    (if (Math|Boolean|ORBoolean (>= (Math|Float|Absolute(Float) (- (.x _returnvalue_3) (.x _returnvalue))) (Variables|FridgeRef|GetMaxDistancefromFridgeToUseLeverX)) (>= (Math|Float|Absolute(Float) (- (.y _returnvalue_3) (.y _returnvalue))) (Variables|FridgeRef|GetMaxDistancefromFridgeToUseLeverY)) (>= (Math|Float|Absolute(Float) (- (.z _returnvalue_3) (.z _returnvalue))) (Variables|FridgeRef|GetMaxDistancefromFridgeToUseLeverZ)))
      (Default|TryRelease (Variables|Default|GetGrabComponent) (Variables|/Game/VRTemplate/Blueprints/VRPawn.VRPawn_C|GetMotionControllerLeft (Variables|Default|GetPG1)))
      (CallFunction|ReleaseFridge))
    (elif (!= (Variables|/Game/VRTemplate/Blueprints/VRPawn.VRPawn_C|GetHeldComponentRight _pg1) 0)
      (if (or (>= (Math|Float|Absolute(Float) (- (.x _returnvalue_4) (.x _returnvalue_2))) (Variables|FridgeRef|GetMaxDistancefromFridgeToUseLeverX)) (>= (Math|Float|Absolute(Float) (- (.y _returnvalue_4) (.y _returnvalue_2))) (Variables|FridgeRef|GetMaxDistancefromFridgeToUseLeverX)))
        (Default|TryRelease (Variables|Default|GetGrabComponent) (Variables|/Game/VRTemplate/Blueprints/VRPawn.VRPawn_C|GetMotionControllerRight (Variables|Default|GetPG1)))
        (CallFunction|ReleaseFridge)))))

(event EventGrabFridge
  ;[1 1 1] Grab fridge
  (Variables|FridgeRef|SetCanFollowPlayerHand? true))

(event EventBeginPlay
  ;[1 1 1] Initialize
  (bind _pg1 (CallFunction|GetPlayer1))
  (Variables|Default|SetPG1 _pg1))

(event EventTick
  (params (DeltaSeconds :type Float%20%28single-precision%29))
  (bind _portafrigo (Variables|Default|GetPortaFrigo))
  (bind _portafrigo_2 (Variables|Default|GetPortaFrigo))
  (bind _portafrigo_3 (Variables|Default|GetPortaFrigo))
  (bind _portafrigo_4 (Variables|Default|GetPortaFrigo))
  (bind _returnvalue (Transformation|GetWorldRotation _portafrigo))
  (bind _returnvalue_2 (Transformation|GetWorldRotation _portafrigo_2))
  (bind _returnvalue_3 (Transformation|GetWorldRotation _portafrigo_4))
  (bind _returnvalue_4 (Transformation|GetWorldRotation _portafrigo_3))
  ;[1 1 1] Event tick
  (if (and (Variables|FridgeRef|GetCanFollowPlayerHand?) (Variables|FridgeRef|GetIsUnlocked?))
    (CallFunction|CheckHandleDistancefromLever)
    (if (Variables|FridgeRef|GetIsYFridgeNegative?)
      (if (!= (Variables|/Game/VRTemplate/Blueprints/VRPawn.VRPawn_C|GetHeldComponentLeft (Variables|Default|GetPG1)) 0)
        (Transformation|SetWorldRotation (Variables|Default|GetPortaFrigo) (Math|Rotator|MakeRotator (.roll _returnvalue_2) (.pitch _returnvalue_2) (Math|Float|Clamp(Float) (- (Math|Float|Absolute(Float) (.y (Transformation|GetWorldLocation (Variables|/Game/VRTemplate/Blueprints/VRPawn.VRPawn_C|GetSphereLeft (Variables|Default|GetPG1))))) (Variables|FridgeRef|GetGrabTreeshold)) (Variables|FridgeRef|GetMinAngle) (Variables|FridgeRef|GetMaxAngle))) false false)
        (elif (!= (Variables|/Game/VRTemplate/Blueprints/VRPawn.VRPawn_C|GetHeldComponentRight (Variables|Default|GetPG1)) 0)
          (Transformation|SetWorldRotation (Variables|Default|GetPortaFrigo) (Math|Rotator|MakeRotator (.roll _returnvalue) (.pitch _returnvalue) (Math|Float|Clamp(Float) (- (Math|Float|Absolute(Float) (.y (Transformation|GetWorldLocation (Variables|/Game/VRTemplate/Blueprints/VRPawn.VRPawn_C|GetSphereRight (Variables|Default|GetPG1))))) (Variables|FridgeRef|GetGrabTreeshold)) (Variables|FridgeRef|GetMinAngle) (Variables|FridgeRef|GetMaxAngle))) false false)))
      (elif (!= (Variables|/Game/VRTemplate/Blueprints/VRPawn.VRPawn_C|GetHeldComponentLeft (Variables|Default|GetPG1)) 0)
        (Transformation|SetWorldRotation (Variables|Default|GetPortaFrigo) (Math|Rotator|MakeRotator (.roll _returnvalue_4) (.pitch _returnvalue_4) (* (Math|Float|Clamp(Float) (- (Math|Float|Absolute(Float) (.y (Transformation|GetWorldLocation (Variables|/Game/VRTemplate/Blueprints/VRPawn.VRPawn_C|GetSphereLeft (Variables|Default|GetPG1))))) (Variables|FridgeRef|GetGrabTreeshold)) (Variables|FridgeRef|GetMinAngle) (Variables|FridgeRef|GetMaxAngle)) -1.0)) false false)
        (elif (!= (Variables|/Game/VRTemplate/Blueprints/VRPawn.VRPawn_C|GetHeldComponentRight (Variables|Default|GetPG1)) 0)
          (Transformation|SetWorldRotation (Variables|Default|GetPortaFrigo) (Math|Rotator|MakeRotator (.roll _returnvalue_3) (.pitch _returnvalue_3) (* (Math|Float|Clamp(Float) (- (Math|Float|Absolute(Float) (.y (Transformation|GetWorldLocation (Variables|/Game/VRTemplate/Blueprints/VRPawn.VRPawn_C|GetSphereRight (Variables|Default|GetPG1))))) (Variables|FridgeRef|GetGrabTreeshold)) (Variables|FridgeRef|GetMinAngle) (Variables|FridgeRef|GetMaxAngle)) -1.0)) false false))))))

(event EventReleaseFridge
  ;[1 1 1] Release fridge
  (Variables|FridgeRef|SetCanFollowPlayerHand? false))

(fn ConstructionScript)