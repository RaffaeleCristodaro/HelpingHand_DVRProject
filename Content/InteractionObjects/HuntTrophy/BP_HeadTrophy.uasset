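; BP_HeadTrophy is an interactive hunt trophy with a speak button that player 1 presses by overlapping it to trigger a voice clip.
; Each tick, an overlap check on CollisionSpeak slides ButtonSpeak in or out along local Y within clamped limits.
; A full press stops the existing Go_go_fight sound or spawns it in 2D if none is valid.
; A DoOnce limits this to one action per press, resetting shortly after full release.
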(event EventBeginPlay
  ;[1 1 1] Initialize
  (bind _pg1 (CallFunction|GetPlayer1))
  (Variables|Default|SetPG1 _pg1))

(event EventTick
  (params (DeltaSeconds :type Float%20%28single-precision%29))
  (bind _button_speak (Variables|Default|GetButton_Speak))
  (bind _button_speak_2 (Variables|Default|GetButton_Speak))
  (bind _maxoffsetbuttons (Variables|Default|GetMaxOffsetButtons))
  (bind _minoffsetbuttons (Variables|Default|GetMinOffsetButtons))
  (bind _minoffsetbuttons_2 (Variables|Default|GetMinOffsetButtons))
  (bind _maxoffsetbuttons_2 (Variables|Default|GetMaxOffsetButtons))
  (bind _returnvalue (Transformation|GetRelativeTransform _button_speak_2))
  (bind _returnvalue_2 (Transformation|GetRelativeTransform _button_speak))
  (bind _returnvalue_3 (- (.location _returnvalue) "0.000000,3.000000,0.000000"))
  (bind _returnvalue_4 (+ (.location _returnvalue_2) "0.000000,3.000000,0.000000"))
  (bind _returnvalue_5 (Math|Float|Clamp(Float) (.y _returnvalue_3) _minoffsetbuttons _maxoffsetbuttons))
  (bind _returnvalue_6 (Math|Float|Clamp(Float) (.y _returnvalue_4) _minoffsetbuttons_2 _maxoffsetbuttons_2))
  ;[1 1 1] Event tick
  (if (Collision|IsOverlappingActor (Variables|Default|GetCollision_Speak) (Variables|Default|GetPG1) :!class /Script/Engine.PrimitiveComponent)
    (Components|MoveComponentTo _button_speak_2 (Math|Vector|MakeVector (.x _returnvalue_3) _returnvalue_5 (.z _returnvalue_3)) (.rotation _returnvalue) false true (Variables|Default|GetOver%20Time) false)
    (if (<= _returnvalue_5 (Variables|Default|GetMinOffsetButtons))
      (Utilities|FlowControl|DoOnce false :!label _label
        (:Completed
          (Utilities|IsValid (Variables|Default|GetGoGoFightSound)
            (:Is%20Valid
              (Audio|Components|Audio|Stop (Variables|Default|GetGoGoFightSound)))
            (:Is%20Not%20Valid
              (bind _returnvalue_7 (Audio|SpawnSound2D "/Game/InteractionObjects/HuntTrophy/go_go_fight.go_go_fight" 1.0 1.0 0.0 0))
              (Variables|Default|SetGoGoFightSound _returnvalue_7))))))
    (else
      (Components|MoveComponentTo _button_speak (Math|Vector|MakeVector (.x _returnvalue_4) _returnvalue_6 (.z _returnvalue_4)) (.rotation _returnvalue_2) false true (Variables|Default|GetOver%20Time) false)
      (if (>= _returnvalue_6 (Variables|Default|GetMaxOffsetButtons))
        (Utilities|FlowControl|Delay 0.2)
        (goto _label Reset)))))

(fn ConstructionScript)