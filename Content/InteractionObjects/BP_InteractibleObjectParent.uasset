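; Parent Blueprint for interactible objects that provides a shared distance-based respawn for objects left far from the player.
; BeginPlay caches a reference to player 1.
; RespawnObject measures the distance from that player's camera to the actor and, at or beyond a given threshold, teleports the actor to a supplied original spawn position.
; The function is not called within this Blueprint.
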(event EventBeginPlay
  ;[1 1 1] Initialize
  (bind _pg1 (CallFunction|GetPlayer1))
  (Variables|Default|SetPG1 _pg1))

(fn ConstructionScript)

(fn RespawnObject
  (params (DistanceFromPlayerToRespawnThisObject :type Float%20%28double-precision%29) (ThisObjectOriginalSpawnPos :type Vector))
  (if (>= (Math|Vector|VectorLength (- (Transformation|GetWorldLocation (Variables|/Game/VRTemplate/Blueprints/VRPawn.VRPawn_C|GetCamera (Variables|Default|GetPG1))) (Transformation|GetActorLocation))) DistanceFromPlayerToRespawnThisObject)
    (Transformation|SetActorLocation ThisObjectOriginalSpawnPos false true)))