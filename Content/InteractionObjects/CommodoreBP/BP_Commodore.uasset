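; BP_Commodore is an interactive Commodore object with a button (Pulsante) that player 1 presses by overlapping its collision.
; Each tick, MoveComponentTo eases the button down during overlap and back up otherwise, clamped between min and max offsets.
; A DoOnce increments CurrentNumberOfClicks when the button sinks past a threshold derived from TriggerTime, and resets once the button returns to the top.
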(event EventBeginPlay
  ;[1 1 1] Initialize
  (bind _pg1 (CallFunction|GetPlayer1))
  (Variables|Default|SetPG1 _pg1))

(event EventTick
  (params (DeltaSeconds :type Float%20%28single-precision%29))
  (bind _pulsante (Variables|Default|GetPulsante))
  (bind _pulsante_2 (Variables|Default|GetPulsante))
  (bind _returnvalue (Transformation|GetRelativeTransform _pulsante_2))
  (bind _returnvalue_2 (Transformation|GetRelativeTransform _pulsante))
  (bind _returnvalue_3 (- (.location _returnvalue) "0.000000,0.000000,3.000000"))
  (bind _returnvalue_4 (+ (.location _returnvalue_2) "0.000000,0.000000,3.000000"))
  ;[1 1 1] Event tick
  (Utilities|FlowControl|Sequence
    (:then_0
      (if (Collision|IsOverlappingActor (Variables|Default|GetPulsanteCommodoreCollision) (Variables|Default|GetPG1) :!class /Script/Engine.PrimitiveComponent)
        (Components|MoveComponentTo _pulsante_2 (Math|Vector|MakeVector (.x _returnvalue_3) (.y _returnvalue_3) (Math|Float|Clamp(Float) (.z _returnvalue_3) (Variables|Default|GetMinOffsetButtons) (Variables|Default|GetMaxOffsetButtons))) (.rotation _returnvalue) false true (Variables|Default|GetOver%20Time) false)
        (if (<= (.z _returnvalue_3) (/ (+ (Variables|Default|GetMinOffsetButtons) (Variables|Default|GetMaxOffsetButtons)) (Variables|Default|GetTriggerTime)))
          (Utilities|FlowControl|DoOnce false :!label _label
            (:Completed
              (Math|Integer|IncrementInt (Variables|Default|GetCurrentNumberOfClicks)))))
        (else
          (Components|MoveComponentTo _pulsante (Math|Vector|MakeVector (.x _returnvalue_4) (.y _returnvalue_4) (Math|Float|Clamp(Float) (.z _returnvalue_4) (Variables|Default|GetMinOffsetButtons) (Variables|Default|GetMaxOffsetButtons))) (.rotation _returnvalue_2) false true (Variables|Default|GetOver%20Time) false)
          (if (>= (.z _returnvalue_4) (Variables|Default|GetMaxOffsetButtons))
            (goto _label Reset)))))))

(fn ConstructionScript)