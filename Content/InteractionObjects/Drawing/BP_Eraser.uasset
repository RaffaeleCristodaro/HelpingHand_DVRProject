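; BP_Eraser is an eraser interaction object that removes crayon drawings on a BP_canvas.
; Each tick it runs a sphere trace at its static mesh's location, sized by EraserRadius and drawn as a one-frame debug shape.
; When the hit actor is a canvas, it passes the hit location and EraserDistance to BPCrayon's DestroySpline.
; BeginPlay calls SetRespawnVariables to set up respawning.
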(event EventBeginPlay
  ;[1 1 1] Initialize
  (CallFunction|SetRespawnVariables))

(event EventTick
  (params (DeltaSeconds :type Float%20%28single-precision%29))
  (bind _staticmesh (Variables|Default|GetStaticMesh))
  (bind _returnvalue (Transformation|GetWorldLocation _staticmesh))
  ;[1 1 1] Event  tick
  (bind _outhit (Collision|SphereTraceByChannel _returnvalue _returnvalue (Variables|Default|GetEraserRadius) "TraceTypeQuery1" false 0 "ForOneFrame"))
  (Utilities|Casting|CastToBP_canvas (.HitActor (Collision|BreakHitResult _outhit)))
  (Default|DestroySpline (Variables|Default|GetBP_Crayon) (.Location (Collision|BreakHitResult _outhit)) (Variables|Default|GetEraser%20Distance)))

(fn ConstructionScript)