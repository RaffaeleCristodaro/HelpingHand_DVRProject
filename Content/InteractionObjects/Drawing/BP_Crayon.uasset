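; BP_Crayon is a crayon that draws paint strokes on a BP_canvas and lets them be erased.
; While its box overlaps the canvas, a gated Tick sphere-traces for it and adds a spline mesh whenever accumulated brush travel reaches a threshold.
; Segments chain from the previous end point, pinned to a fixed plane chosen by IsYOriented.
; DestroySpline removes segments whose stored impact locations lie within the eraser's radius.
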(event OnComponentBeginOverlap(Box)
  (params (OverlappedComponent :type Primitive%20Component%20Object%20Reference) (OtherActor :type Actor%20Object%20Reference) (OtherComp :type Primitive%20Component%20Object%20Reference) (OtherBodyIndex :type Integer) (bFromSweep :type Boolean) (SweepResult :type Hit%20Result%20Structure%20%28by%20ref%29))
  ;[1 1 1] Canvas collision
  (Utilities|Casting|CastToBP_canvas OtherActor)
  (CallFunction|OpenGate))

(event OnComponentEndOverlap(Box)
  (params (OverlappedComponent :type Primitive%20Component%20Object%20Reference) (OtherActor :type Actor%20Object%20Reference) (OtherComp :type Primitive%20Component%20Object%20Reference) (OtherBodyIndex :type Integer))
  ;[1 1 1] Canvas collision
  (Utilities|Casting|CastToBP_canvas OtherActor)
  (CallFunction|CloseGate)
  (Utilities|Array|Clear (Variables|DrawRef|GetDrawSpline)))

(event Custom|CloseGate
  (bind _brushstrikelocation (Variables|Default|GetBrushStrikeLocation))
  (bind _brushstrikelocation_2 (Variables|Default|GetBrushStrikeLocation))
  (bind _box (Variables|Default|GetBox))
  (bind _brushstrikelocation_3 (Variables|Default|GetBrushStrikeLocation))
  (bind _brushstrikelocation_4 (Variables|Default|GetBrushStrikeLocation))
  (bind _end_pos_y (Variables|Orientation|GetEnd%20Pos%20Y))
  (bind _end_pos_x (Variables|Orientation|GetEnd%20Pos%20X))
  (bind _brushstrikelocation_5 (Variables|Default|GetBrushStrikeLocation))
  (bind _returnvalue (Transformation|GetWorldLocation _brushstrikelocation_5))
  (bind _returnvalue_2 (Transformation|GetWorldLocation _brushstrikelocation))
  (bind _returnvalue_3 (Transformation|GetWorldLocation _brushstrikelocation_2))
  (bind _returnvalue_4 (Transformation|GetWorldLocation _brushstrikelocation_4))
  (bind _returnvalue_5 (Transformation|GetWorldLocation _brushstrikelocation_3))
  (bind _returnvalue_6 (Transformation|GetWorldLocation _box))
  ;[1 1 1] Event tick
  (Utilities|FlowControl|Gate true) ; enters at Close
)

(event Custom|OpenGate
  (bind _brushstrikelocation (Variables|Default|GetBrushStrikeLocation))
  (bind _brushstrikelocation_2 (Variables|Default|GetBrushStrikeLocation))
  (bind _box (Variables|Default|GetBox))
  (bind _brushstrikelocation_3 (Variables|Default|GetBrushStrikeLocation))
  (bind _brushstrikelocation_4 (Variables|Default|GetBrushStrikeLocation))
  (bind _end_pos_y (Variables|Orientation|GetEnd%20Pos%20Y))
  (bind _end_pos_x (Variables|Orientation|GetEnd%20Pos%20X))
  (bind _brushstrikelocation_5 (Variables|Default|GetBrushStrikeLocation))
  (bind _returnvalue (Transformation|GetWorldLocation _brushstrikelocation_5))
  (bind _returnvalue_2 (Transformation|GetWorldLocation _brushstrikelocation))
  (bind _returnvalue_3 (Transformation|GetWorldLocation _brushstrikelocation_2))
  (bind _returnvalue_4 (Transformation|GetWorldLocation _brushstrikelocation_4))
  (bind _returnvalue_5 (Transformation|GetWorldLocation _brushstrikelocation_3))
  (bind _returnvalue_6 (Transformation|GetWorldLocation _box))
  ;[1 1 1] Event tick
  (Utilities|FlowControl|Gate true) ; enters at Open
)

(event Custom|DestroySpline
  (params (BP_EraserLocation :type Vector) (EraserDistance :type Float%20%28double-precision%29))
  (bind _totaldrawnsplineimpactlocation (Variables|DrawRef|GetTotalDrawnSplineImpactLocation))
  (bind _totaldrawnspline (Variables|DrawRef|GetTotalDrawnSpline))
  ;[1 1 1] Destroy spline
  (for (_array_element _array_index) _totaldrawnspline
    (Utilities|IsValid _array_element
      (:Is%20Valid
        (if (<= (Math|Vector|VectorLength (- BP_EraserLocation (Utilities|Array|Get(acopy) _totaldrawnsplineimpactlocation _array_index))) EraserDistance)
          (Components|DestroyComponent _array_element)
          (Utilities|Array|RemoveItem _totaldrawnspline _array_element)
          (Utilities|Array|RemoveItem _totaldrawnsplineimpactlocation (Utilities|Array|Get(acopy) _totaldrawnsplineimpactlocation _array_index)))))))

(event EventBeginPlay
  ;[1 1 1] Initialize
  (CallFunction|SetRespawnVariables)
  (Rendering|Material|SetMaterial (Variables|Default|GetStaticMesh) 0 (Variables|MaterialCrayon|GetMaterialCrayon)))

(event EventTick
  (params (DeltaSeconds :type Float%20%28single-precision%29))
  (bind _brushstrikelocation (Variables|Default|GetBrushStrikeLocation))
  (bind _brushstrikelocation_2 (Variables|Default|GetBrushStrikeLocation))
  (bind _box (Variables|Default|GetBox))
  (bind _brushstrikelocation_3 (Variables|Default|GetBrushStrikeLocation))
  (bind _brushstrikelocation_4 (Variables|Default|GetBrushStrikeLocation))
  (bind _end_pos_y (Variables|Orientation|GetEnd%20Pos%20Y))
  (bind _end_pos_x (Variables|Orientation|GetEnd%20Pos%20X))
  (bind _brushstrikelocation_5 (Variables|Default|GetBrushStrikeLocation))
  (bind _returnvalue (Transformation|GetWorldLocation _brushstrikelocation_5))
  (bind _returnvalue_2 (Transformation|GetWorldLocation _brushstrikelocation))
  (bind _returnvalue_3 (Transformation|GetWorldLocation _brushstrikelocation_2))
  (bind _returnvalue_4 (Transformation|GetWorldLocation _brushstrikelocation_4))
  (bind _returnvalue_5 (Transformation|GetWorldLocation _brushstrikelocation_3))
  (bind _returnvalue_6 (Transformation|GetWorldLocation _box))
  ;[1 1 1] Event tick
  (Utilities|FlowControl|Gate true
    (:Exit
      (bind _outhit (Collision|SphereTraceByChannel _returnvalue_6 _returnvalue_6 (Variables|DrawRef|GetCrayonDistanceFromCanvas) "TraceTypeQuery1" false 0 "None"))
      (Utilities|Casting|CastToBP_canvas (.HitActor (Collision|BreakHitResult _outhit)))
      (bind _output_get (Variables|DrawRef|SetDistance (+ (Variables|DrawRef|GetDistance) (Math|Vector|Distance(Vector) (Variables|DrawRef|GetPreviousLocation) _returnvalue_2))))
      (Variables|DrawRef|SetPreviousLocation _returnvalue_2)
      (if (>= _output_get (Variables|DrawRef|GetSplineDistance))
        (Variables|DrawRef|SetDistance 0.0)
        (bind _returnvalue_7 (AddComponent|AddSplineMeshComponent false))
        (Rendering|Material|SetMaterial _returnvalue_7 0 (Variables|MaterialCrayon|GetMaterialPaint))
        (bind _returnvalue_8 (Utilities|Array|Add (Variables|DrawRef|GetDrawSpline) _returnvalue_7))
        (Utilities|Array|Add (Variables|DrawRef|GetTotalDrawnSpline) _returnvalue_7)
        (Utilities|Array|Add (Variables|DrawRef|GetTotalDrawnSplineImpactLocation) (.Location (Collision|BreakHitResult _outhit)))
        (if (Variables|Orientation|GetIsYOriented?)
          (SplineMesh|SetEndPosition _returnvalue_7 (Math|Vector|MakeVector (.x _returnvalue_5) _end_pos_y (.z _returnvalue_5)) true)
          (if (> _returnvalue_8 (Variables|DrawRef|GetLastPoint))
            (SplineMesh|SetStartPosition _returnvalue_7 (Math|Vector|MakeVector (.x (SplineMesh|GetEndPosition (Utilities|Array|Get(acopy) (Variables|DrawRef|GetDrawSpline) (- _returnvalue_8 1)))) _end_pos_y (.z (SplineMesh|GetEndPosition (Utilities|Array|Get(acopy) (Variables|DrawRef|GetDrawSpline) (- _returnvalue_8 1))))) true)
            (else
              (SplineMesh|SetStartPosition _returnvalue_7 (Math|Vector|MakeVector (.x _returnvalue_4) _end_pos_y (.z _returnvalue_4)) true)))
          (else
            (SplineMesh|SetEndPosition _returnvalue_7 (Math|Vector|MakeVector _end_pos_x (.y _returnvalue) (.z _returnvalue)) true)
            (if (> _returnvalue_8 (Variables|DrawRef|GetLastPoint))
              (SplineMesh|SetStartPosition _returnvalue_7 (Math|Vector|MakeVector _end_pos_x (.y (SplineMesh|GetEndPosition (Utilities|Array|Get(acopy) (Variables|DrawRef|GetDrawSpline) (- _returnvalue_8 1)))) (.z (SplineMesh|GetEndPosition (Utilities|Array|Get(acopy) (Variables|DrawRef|GetDrawSpline) (- _returnvalue_8 1))))) true)
              (else
                (SplineMesh|SetStartPosition _returnvalue_7 (Math|Vector|MakeVector (.x _returnvalue_3) _end_pos_x (.z _returnvalue_3)) true)))))))))

(fn ConstructionScript)