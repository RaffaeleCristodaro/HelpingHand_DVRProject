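; VR lever that opens the attic hatch (BP_AtticStair) and shifts the puzzle into a second illuminated room.
; While grabbed, a gated Tick pitches the rod from the hand's clamped height, releasing it if too distant.
; Past the snap threshold, it locks and one-time offsets both players, the hatch, death zones, grabbables and teleports vertically.
; An optional counterweight mode uses a re-arming timer to reset the rod after release.
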(event Custom|StartTracking
  (bind _rod (Variables|Default|GetRod))
  (bind _rod_2 (Variables|Default|GetRod))
  (bind _rod_3 (Variables|Default|GetRod))
  (bind _rod_4 (Variables|Default|GetRod))
  (bind _returnvalue (Transformation|GetWorldRotation _rod))
  (bind _returnvalue_2 (Transformation|GetWorldRotation _rod_2))
  (bind _returnvalue_3 (Transformation|GetWorldRotation _rod_3))
  (bind _returnvalue_4 (Transformation|GetWorldRotation _rod_4))
  ;[1 1 1] Event tick
  (if (Variables|Botola|GetCanOpenBotola?)
    (Utilities|FlowControl|Gate true) ; enters at Open
  ))

(event Custom|StopTracking
  (bind _rod (Variables|Default|GetRod))
  (bind _rod_2 (Variables|Default|GetRod))
  (bind _rod_3 (Variables|Default|GetRod))
  (bind _rod_4 (Variables|Default|GetRod))
  (bind _returnvalue (Transformation|GetWorldRotation _rod))
  (bind _returnvalue_2 (Transformation|GetWorldRotation _rod_2))
  (bind _returnvalue_3 (Transformation|GetWorldRotation _rod_3))
  (bind _returnvalue_4 (Transformation|GetWorldRotation _rod_4))
  ;[1 1 1] Event tick
  (if (Variables|Botola|GetCanOpenBotola?)
    (Utilities|FlowControl|Gate true) ; enters at Close
  ))

(event Custom|CheckHandleDistanceFromLeverEvent
  ;[1 1 1] Release hand from lever if too far
  (bind _pg1 (CallFunction|GetPlayer1))
  (if (!= (Variables|/Game/VRTemplate/Blueprints/VRPawn.VRPawn_C|GetHeldComponentLeft _pg1) 0)
    (if (>= (Math|Vector|VectorLength (- (Transformation|GetWorldLocation (Variables|/Game/VRTemplate/Blueprints/VRPawn.VRPawn_C|GetLeftHand _pg1)) (Transformation|GetWorldLocation (Variables|Default|GetRod)))) (Variables|LeverRef|GetLeverMaxDistanceFromHandBeforeRelease))
      (bind _pg1_2 (CallFunction|GetPlayer1))
      (Default|TryRelease (Variables|Default|GetGrabComponent) (Variables|/Game/VRTemplate/Blueprints/VRPawn.VRPawn_C|GetMotionControllerLeft _pg1_2))
      (CallFunction|StopTracking))
    (elif (!= (Variables|/Game/VRTemplate/Blueprints/VRPawn.VRPawn_C|GetHeldComponentRight _pg1) 0)
      (if (>= (Math|Vector|VectorLength (- (Transformation|GetWorldLocation (Variables|/Game/VRTemplate/Blueprints/VRPawn.VRPawn_C|GetRightHand _pg1)) (Transformation|GetWorldLocation (Variables|Default|GetRod)))) (Variables|LeverRef|GetLeverMaxDistanceFromHandBeforeRelease))
        (bind _pg1_3 (CallFunction|GetPlayer1))
        (Default|TryRelease (Variables|Default|GetGrabComponent) (Variables|/Game/VRTemplate/Blueprints/VRPawn.VRPawn_C|GetMotionControllerRight _pg1_3))
        (CallFunction|StopTracking)))))

(event Custom|CounterWeightEvent
  ;[1 1 1] CounterWeight Event
  (Utilities|Time|SetTimerbyEvent (delegate Custom|CounterWeightEventTimer) (Variables|CounterWeight|GetTimeCounterWeigth)))

(event Custom|CounterWeightEventTimer
  ;[1 1 1] CounterWeight Event
  (if (Variables|CounterWeight|GetIsCounterWeightPressed?)
    (CallFunction|CounterWeightEvent)
    (else
      (Transformation|SetWorldRotation (Variables|Default|GetRod) (Variables|LeverRef|GetLeverInitialRotation) false false))))

(event EventDrop
  ;[1 1 1] Pick up and drop events
  (CallFunction|StopTracking)
  (Variables|Default|SetHand 0)
  (if (Variables|CounterWeight|GetIsACounterWeight?)
    (Variables|CounterWeight|SetIsCounterWeightPressed? false)))

(event EventPickup
  (params (Component :type Scene%20Component%20Object%20Reference))
  ;[1 1 1] Pick up and drop events
  (Variables|Default|SetHand Component)
  (CallFunction|StartTracking)
  (if (Variables|CounterWeight|GetIsACounterWeight?)
    (CallFunction|CounterWeightEvent)
    (Variables|CounterWeight|SetIsCounterWeightPressed? true)))

(event EventBeginPlay
  (bind _rod (Variables|Default|GetRod))
  (bind _returnvalue (Transformation|GetWorldRotation _rod))
  ;[1 1 1] Initialize
  (Variables|LeverRef|SetLeverInitialRotation (Math|Rotator|MakeRotator (.roll _returnvalue) (.pitch _returnvalue) (.yaw _returnvalue)))
  (bind _returnvalue_2 (Actor|GetActorOfClass "/Game/Asset_Soffitta/Botola/BP_AtticStair.BP_AtticStair_C"))
  (Variables|Botola|SetBP_Botola _returnvalue_2)
  (bind _pg1 (CallFunction|GetPlayer1))
  (Variables|Default|SetPlayer1 _pg1)
  (bind _pg3 (CallFunction|GetPlayer3))
  (Variables|Default|SetPG3 _pg3))

(event EventTick
  (params (DeltaSeconds :type Float%20%28single-precision%29))
  (bind _rod (Variables|Default|GetRod))
  (bind _rod_2 (Variables|Default|GetRod))
  (bind _puzzle_sturalavandino (Variables|Default|GetPuzzle_Sturalavandino))
  (bind _rod_3 (Variables|Default|GetRod))
  (bind _rod_4 (Variables|Default|GetRod))
  (bind _returnvalue (Transformation|GetWorldRotation _rod))
  (bind _returnvalue_2 (Transformation|GetWorldRotation _rod_2))
  (bind _returnvalue_3 (Transformation|GetWorldRotation _rod_3))
  (bind _returnvalue_4 (Transformation|GetWorldRotation _rod_4))
  ;[1 1 1] Event tick
  (if (Variables|Botola|GetCanOpenBotola?)
    _
    (else
      (Utilities|IsValid _puzzle_sturalavandino
        (:Is%20Valid
          (Components|DestroyComponent _puzzle_sturalavandino))
        (:Is%20Not%20Valid
          _))))
  (Utilities|FlowControl|Gate true
    (:Exit
      (CallFunction|CheckHandleDistancefromLeverEvent)
      (bind _pg1 (CallFunction|GetPlayer1))
      (if (!= (Variables|/Game/VRTemplate/Blueprints/VRPawn.VRPawn_C|GetHeldComponentLeft _pg1) 0)
        (Transformation|SetWorldRotation _rod (Math|Rotator|MakeRotator (.roll _returnvalue) (Math|Float|Clamp(Float) (- (.z (Transformation|GetWorldLocation (Variables|/Game/VRTemplate/Blueprints/VRPawn.VRPawn_C|GetSphereLeft _pg1))) (Variables|LeverRef|GetGrabTreeshould)) (Variables|LeverRef|GetMinAngle) (Variables|LeverRef|GetMaxAngle)) (.yaw _returnvalue)) false false)
        (if (<= (Math|Float|Clamp(Float) (- (.z (Transformation|GetWorldLocation (Variables|/Game/VRTemplate/Blueprints/VRPawn.VRPawn_C|GetSphereLeft _pg1))) (Variables|LeverRef|GetGrabTreeshould)) (Variables|LeverRef|GetMinAngle) (Variables|LeverRef|GetMaxAngle)) (Variables|LeverRef|GetLevelSnapTreeshould))
          (Utilities|FlowControl|DoOnce false :!label _label
            (:Completed
              (Audio|PlaySound2D 0 1.0 1.0 0.0 0 0)
              (CallFunction|StopTracking)
              (Transformation|SetWorldRotation _rod_2 (Math|Rotator|MakeRotator (.roll _returnvalue_2) (Variables|LeverRef|GetLvFinalInclination) (.yaw _returnvalue_2)) false false)
              (Utilities|FlowControl|Sequence
                (:then_0
                  (if (Variables|Botola|GetCanOpenBotola?)
                    (Variables|Botola|SetCanOpenBotola? false)
                    (CallFunction|TeleportObjectinOtherIlluminatedRoom)))
                (:then_1
                  (Utilities|FlowControl|Delay 0.5)
                  (goto _label Reset))))))
        (elif (!= (Variables|/Game/VRTemplate/Blueprints/VRPawn.VRPawn_C|GetHeldComponentRight _pg1) 0)
          (Transformation|SetWorldRotation _rod_3 (Math|Rotator|MakeRotator (.roll _returnvalue_3) (Math|Float|Clamp(Float) (- (.z (Transformation|GetWorldLocation (Variables|/Game/VRTemplate/Blueprints/VRPawn.VRPawn_C|GetSphereRight _pg1))) (Variables|LeverRef|GetGrabTreeshould)) (Variables|LeverRef|GetMinAngle) (Variables|LeverRef|GetMaxAngle)) (.yaw _returnvalue_3)) false false)
          (if (<= (Math|Float|Clamp(Float) (- (.z (Transformation|GetWorldLocation (Variables|/Game/VRTemplate/Blueprints/VRPawn.VRPawn_C|GetSphereRight _pg1))) (Variables|LeverRef|GetGrabTreeshould)) (Variables|LeverRef|GetMinAngle) (Variables|LeverRef|GetMaxAngle)) (Variables|LeverRef|GetLevelSnapTreeshould))
            (Utilities|FlowControl|DoOnce false :!label _label_2
              (:Completed
                (Audio|PlaySound2D 0 1.0 1.0 0.0 0 0)
                (CallFunction|StopTracking)
                (Transformation|SetWorldRotation _rod_4 (Math|Rotator|MakeRotator (.roll _returnvalue_4) (Variables|LeverRef|GetLvFinalInclination) (.yaw _returnvalue_4)) false false)
                (Utilities|FlowControl|Sequence
                  (:then_0
                    (if (Variables|Botola|GetCanOpenBotola?)
                      (Variables|Botola|SetCanOpenBotola? false)
                      (CallFunction|TeleportObjectinOtherIlluminatedRoom)))
                  (:then_1
                    (Utilities|FlowControl|Delay 0.5)
                    (goto _label_2 Reset)))))))))))

(fn ConstructionScript)

(fn TeleportObjectinOtherIlluminatedRoom
  (bind _player1 (Variables|Default|GetPlayer1))
  (bind _heightzsecondroomdeathzones (Variables|TeleportSecondroomRef|GetHeightZSecondRoomDeathZones))
  (bind _player1_2 (Variables|Default|GetPlayer1))
  (bind _bp_botola (Variables|Botola|GetBP_Botola))
  (bind _heightzsecondroomteleports (Variables|TeleportSecondroomRef|GetHeightZSecondRoomTeleports))
  (bind _heightzsecondroomteleportsspawners (Variables|TeleportSecondroomRef|GetHeightZSecondRoomTeleportsSpawners))
  (bind _rod (Variables|Default|GetRod))
  (bind _canvasteleportedlocation (Variables|TeleportSecondroomRef|GetCanvasTeleportedLocation))
  (bind _pg3 (Variables|Default|GetPG3))
  (bind _returnvalue (Transformation|GetActorLocation _pg3))
  (bind _returnvalue_2 (Transformation|GetActorLocation _canvasteleportedlocation))
  (bind _returnvalue_3 (Transformation|GetActorLocation _bp_botola))
  (bind _returnvalue_4 (Transformation|GetWorldLocation _rod))
  (bind _returnvalue_5 (Transformation|GetActorRotation _player1))
  (bind _camera (Variables|/Game/VRTemplate/Blueprints/VRPawn.VRPawn_C|GetCamera _player1))
  (bind _returnvalue_6 (Transformation|GetWorldLocation _camera))
  ;[1 1 1] Special objects
  (Transformation|Teleport (Variables|Default|GetPlayer1) (Math|Vector|MakeVector (.x _returnvalue_6) (.y _returnvalue_6) (+ (.z _returnvalue_6) (Variables|TeleportSecondroomRef|GetHeightZSecondRoomTeleportPG1))) (Math|Rotator|MakeRotator (.roll _returnvalue_5) (.pitch _returnvalue_5) (.yaw _returnvalue_5)))
  (Transformation|SetActorLocationAndRotation _pg3 (Math|Vector|MakeVector (.x _returnvalue) (.y _returnvalue) (+ (.z _returnvalue) (Variables|TeleportSecondroomRef|GetHeightZSecondRoomTeleportPG3))) "0, 0, 0" false true)
  (Transformation|SetWorldLocationAndRotation _rod (Math|Vector|MakeVector (.x _returnvalue_4) (.y _returnvalue_4) (+ (.z _returnvalue_4) (Variables|TeleportSecondroomRef|GetHeightZSecondRoomGrabbables))) (Variables|TeleportSecondroomRef|GetLeverRotationTeleported) false false)
  (Transformation|SetActorLocation _bp_botola (Math|Vector|MakeVector (.x _returnvalue_3) (.y _returnvalue_3) (+ (.z _returnvalue_3) (Variables|TeleportSecondroomRef|GetHeightZSecondRoomGrabbables))) false false)
  (Default|EventOpenBotola (Variables|Botola|GetBP_Botola))
  (Transformation|SetActorLocation (Math|Vector|MakeVector (.x _returnvalue_2) (.y _returnvalue_2) (+ (.z _returnvalue_2) (Variables|TeleportSecondroomRef|GetHeightZSecondRoomGrabbables))) false false)
  ;[1 1 1] Deathzones
  (for _array_element (Variables|TeleportSecondroomRef|GetDeathZonesTeleported)
    (Transformation|SetActorLocation _array_element (Math|Vector|MakeVector (.x (Transformation|GetActorLocation _array_element)) (.y (Transformation|GetActorLocation _array_element)) (+ (.z (Transformation|GetActorLocation _array_element)) _heightzsecondroomdeathzones)) false true)
    (Variables|/Game/DeathZone/BP_Deathzone.BP_Deathzone_C|SetPG3RespawnLocation _array_element (Math|Vector|MakeVector (.x (Variables|/Game/DeathZone/BP_Deathzone.BP_Deathzone_C|GetPG3RespawnLocation _array_element)) (.y (Variables|/Game/DeathZone/BP_Deathzone.BP_Deathzone_C|GetPG3RespawnLocation _array_element)) (+ _heightzsecondroomdeathzones (.z (Variables|/Game/DeathZone/BP_Deathzone.BP_Deathzone_C|GetPG3RespawnLocation _array_element))))))
  ;[1 1 1] Grabbables
  (for _array_element_2 (Variables|TeleportSecondroomRef|GetGrabbablesTeleported)
    (Variables|/Game/Blueprint_Grabbable/BP_InteractiveGrabbablesParent.BP_InteractiveGrabbablesParent_C|SetActorStartLocation _array_element_2 (Math|Vector|MakeVector (.x (Variables|/Game/Blueprint_Grabbable/BP_InteractiveGrabbablesParent.BP_InteractiveGrabbablesParent_C|GetActorStartLocation _array_element_2)) (.y (Variables|/Game/Blueprint_Grabbable/BP_InteractiveGrabbablesParent.BP_InteractiveGrabbablesParent_C|GetActorStartLocation _array_element_2)) (+ (.z (Variables|/Game/Blueprint_Grabbable/BP_InteractiveGrabbablesParent.BP_InteractiveGrabbablesParent_C|GetActorStartLocation _array_element_2)) (Variables|TeleportSecondroomRef|GetHeightZSecondRoomGrabbables))))
    (Variables|/Game/Blueprint_Grabbable/BP_InteractiveGrabbablesParent.BP_InteractiveGrabbablesParent_C|SetPrimitiveComponentStartLocation _array_element_2 (Math|Vector|MakeVector (.x (Transformation|GetWorldLocation (Variables|/Game/Blueprint_Grabbable/BP_InteractiveGrabbablesParent.BP_InteractiveGrabbablesParent_C|GetStaticMesh _array_element_2))) (.y (Transformation|GetWorldLocation (Variables|/Game/Blueprint_Grabbable/BP_InteractiveGrabbablesParent.BP_InteractiveGrabbablesParent_C|GetStaticMesh _array_element_2))) (+ (.z (Transformation|GetWorldLocation (Variables|/Game/Blueprint_Grabbable/BP_InteractiveGrabbablesParent.BP_InteractiveGrabbablesParent_C|GetStaticMesh _array_element_2))) (Variables|TeleportSecondroomRef|GetHeightZSecondRoomGrabbables))))
    (Transformation|SetActorLocation _array_element_2 (Math|Vector|MakeVector (.x (Transformation|GetActorLocation _array_element_2)) (.y (Transformation|GetActorLocation _array_element_2)) (+ (.z (Transformation|GetActorLocation _array_element_2)) (Variables|TeleportSecondroomRef|GetHeightZSecondRoomGrabbables))) false true)
    (Transformation|SetWorldLocation (Variables|/Game/Blueprint_Grabbable/BP_InteractiveGrabbablesParent.BP_InteractiveGrabbablesParent_C|GetStaticMesh _array_element_2) (Math|Vector|MakeVector (.x (Transformation|GetWorldLocation (Variables|/Game/Blueprint_Grabbable/BP_InteractiveGrabbablesParent.BP_InteractiveGrabbablesParent_C|GetStaticMesh _array_element_2))) (.y (Transformation|GetWorldLocation (Variables|/Game/Blueprint_Grabbable/BP_InteractiveGrabbablesParent.BP_InteractiveGrabbablesParent_C|GetStaticMesh _array_element_2))) (+ (.z (Transformation|GetWorldLocation (Variables|/Game/Blueprint_Grabbable/BP_InteractiveGrabbablesParent.BP_InteractiveGrabbablesParent_C|GetStaticMesh _array_element_2))) (Variables|TeleportSecondroomRef|GetHeightZSecondRoomGrabbables))) false false))
  ;[1 1 1] Teleports
  (for _array_element_3 (Variables|TeleportSecondroomRef|GetTeleportsTeleported)
    (Transformation|SetActorLocation _array_element_3 (Math|Vector|MakeVector (.x (Transformation|GetActorLocation _array_element_3)) (.y (Transformation|GetActorLocation _array_element_3)) (+ (.z (Transformation|GetActorLocation _array_element_3)) _heightzsecondroomteleports)) false true)
    (Variables|/Game/Teleporters/BP_Teleport.BP_Teleport_C|SetPlayerNewLocation _array_element_3 (Math|Vector|MakeVector (.x (Variables|/Game/Teleporters/BP_Teleport.BP_Teleport_C|GetPlayerNewLocation _array_element_3)) (.y (Variables|/Game/Teleporters/BP_Teleport.BP_Teleport_C|GetPlayerNewLocation _array_element_3)) (+ (.z (Variables|/Game/Teleporters/BP_Teleport.BP_Teleport_C|GetPlayerNewLocation _array_element_3)) _heightzsecondroomteleports))))
  ;[1 1 1] Teleports Spawners
  (for _array_element_4 (Variables|TeleportSecondroomRef|GetTeleportsSpawnerTeleported)
    (Transformation|SetActorLocation _array_element_4 (Math|Vector|MakeVector (.x (Transformation|GetActorLocation _array_element_4)) (.y (Transformation|GetActorLocation _array_element_4)) (+ (.z (Transformation|GetActorLocation _array_element_4)) _heightzsecondroomteleportsspawners)) false true)
    (Variables|/Game/Teleporters/BP_TeleportSpawner.BP_TeleportSpawner_C|SetTeleportStartLocation _array_element_4 (Math|Vector|MakeVector (.x (Variables|/Game/Teleporters/BP_TeleportSpawner.BP_TeleportSpawner_C|GetTeleportStartLocation _array_element_4)) (.y (Variables|/Game/Teleporters/BP_TeleportSpawner.BP_TeleportSpawner_C|GetTeleportStartLocation _array_element_4)) (+ (.z (Variables|/Game/Teleporters/BP_TeleportSpawner.BP_TeleportSpawner_C|GetTeleportStartLocation _array_element_4)) _heightzsecondroomteleportsspawners)))
    (Variables|/Game/Teleporters/BP_TeleportSpawner.BP_TeleportSpawner_C|SetFinalTeleportLocation _array_element_4 (Math|Vector|MakeVector (.x (Variables|/Game/Teleporters/BP_TeleportSpawner.BP_TeleportSpawner_C|GetFinalTeleportLocation _array_element_4)) (.y (Variables|/Game/Teleporters/BP_TeleportSpawner.BP_TeleportSpawner_C|GetFinalTeleportLocation _array_element_4)) (+ (.z (Variables|/Game/Teleporters/BP_TeleportSpawner.BP_TeleportSpawner_C|GetFinalTeleportLocation _array_element_4)) _heightzsecondroomteleportsspawners))))
  ;[1 1 1] Fix PG1 grab bug
  (Variables|/Game/VRTemplate/Blueprints/VRPawn.VRPawn_C|SetHeldComponentRight _player1_2 0)
  (Variables|/Game/VRTemplate/Blueprints/VRPawn.VRPawn_C|SetHeldComponentLeft _player1_2 0)
  (return))