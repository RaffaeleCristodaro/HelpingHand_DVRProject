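; Playable pinball machine that Player 1 works by overlapping start, left and right button volumes.
; Tick animates buttons and flippers with MoveComponentTo, and the start button lowers a launch bar that resets after a delay.
; Hits on a held flipper add an impulse to the ball, and Fungis bumper hits add to a printed score, both throttled by DoOnce and Delay.
; A trigger area teleports the ball back to its respawn point.
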(event OnComponentBeginOverlap(RespawnBallArea)
  (params (OverlappedComponent :type Primitive%20Component%20Object%20Reference) (OtherActor :type Actor%20Object%20Reference) (OtherComp :type Primitive%20Component%20Object%20Reference) (OtherBodyIndex :type Integer) (bFromSweep :type Boolean) (SweepResult :type Hit%20Result%20Structure%20%28by%20ref%29))
  (bind _flipperball (Variables|Default|GetFlipperBall))
  ;[1 1 1] Respawn ball
  (if (== OtherActor _flipperball)
    (Transformation|SetWorldLocation (Variables|/Game/InteractionObjects/BP_FlipperBall.BP_FlipperBall_C|GetSphere _flipperball) (Transformation|GetWorldLocation (Variables|Default|GetRespawnBallScene)) false true)))

(event OnComponentHit(RightFlipper)
  (params (HitComponent :type Primitive%20Component%20Object%20Reference) (OtherActor :type Actor%20Object%20Reference) (OtherComp :type Primitive%20Component%20Object%20Reference) (NormalImpulse :type Vector :default "0, 0, 0") (Hit :type Hit%20Result%20Structure%20%28by%20ref%29))
  ;[1 1 1] Apply force to ball
  (if (Variables|ForceToApply|GetCanApplyForceRight?)
    (Utilities|FlowControl|DoOnce false :!label _label
      (:Completed
        (Physics|AddImpulse (Variables|/Game/InteractionObjects/BP_FlipperBall.BP_FlipperBall_C|GetSphere (Variables|Default|GetFlipperBall)) (Variables|ForceToApply|GetImpulse) "None" false)
        (Utilities|FlowControl|Delay 0.2)
        (goto _label Reset)))))

(event OnComponentHit(LeftFlipper)
  (params (HitComponent :type Primitive%20Component%20Object%20Reference) (OtherActor :type Actor%20Object%20Reference) (OtherComp :type Primitive%20Component%20Object%20Reference) (NormalImpulse :type Vector :default "0, 0, 0") (Hit :type Hit%20Result%20Structure%20%28by%20ref%29))
  ;[1 1 1] Apply force to ball
  (if (Variables|ForceToApply|GetCanApplyForceLeft?)
    (Utilities|FlowControl|DoOnce false :!label _label
      (:Completed
        (Physics|AddImpulse (Variables|/Game/InteractionObjects/BP_FlipperBall.BP_FlipperBall_C|GetSphere (Variables|Default|GetFlipperBall)) (Variables|ForceToApply|GetImpulse) "None" false)
        (Utilities|FlowControl|Delay 0.2)
        (goto _label Reset)))))

(event OnComponentHit(Fungis)
  (params (HitComponent :type Primitive%20Component%20Object%20Reference) (OtherActor :type Actor%20Object%20Reference) (OtherComp :type Primitive%20Component%20Object%20Reference) (NormalImpulse :type Vector :default "0, 0, 0") (Hit :type Hit%20Result%20Structure%20%28by%20ref%29))
  ;[1 1 1] Score
  (Utilities|Casting|CastToBP_FlipperBall OtherActor)
  (Utilities|FlowControl|DoOnce false :!label _label
    (:Completed
      (bind _output_get (Variables|Score|SetCurrentScore (+ (Variables|Score|GetCurrentScore) (Variables|Score|GetFungisAddScore))))
      (Development|PrintString (Utilities|String|ToString(Integer) _output_get))
      (Utilities|FlowControl|Delay 1.0)
      (goto _label Reset))))

(event EventBeginPlay
  ;[1 1 1] Initialize
  (bind _pg1 (CallFunction|GetPlayer1))
  (Variables|Default|SetPG1 _pg1))

(event EventTick
  (params (DeltaSeconds :type Float%20%28single-precision%29))
  (bind _startbarzlocationspeed (Variables|ButtonStart|GetStartBarZlocationSpeed))
  (bind _startbar (Variables|Default|GetStartBar))
  (bind _minoffsetbuttonstart (Variables|ButtonStart|GetMinOffsetButtonStart))
  (bind _maxoffsetbuttonstart (Variables|ButtonStart|GetMaxOffsetButtonStart))
  (bind _minoffsetbuttonstart_2 (Variables|ButtonStart|GetMinOffsetButtonStart))
  (bind _maxoffsetbuttonstart_2 (Variables|ButtonStart|GetMaxOffsetButtonStart))
  (bind _startbutton (Variables|Default|GetStartButton))
  (bind _startbutton_2 (Variables|Default|GetStartButton))
  (bind _rightbutton (Variables|Default|GetRightButton))
  (bind _rightbutton_2 (Variables|Default|GetRightButton))
  (bind _rightflipper (Variables|Default|GetRightFlipper))
  (bind _rightflipper_2 (Variables|Default|GetRightFlipper))
  (bind _lefttbutton (Variables|Default|GetLefttButton))
  (bind _leftflipper (Variables|Default|GetLeftFlipper))
  (bind _lefttbutton_2 (Variables|Default|GetLefttButton))
  (bind _leftflipper_2 (Variables|Default|GetLeftFlipper))
  (bind _returnvalue (Transformation|GetRelativeTransform _lefttbutton_2))
  (bind _returnvalue_2 (Transformation|GetRelativeTransform _lefttbutton))
  (bind _returnvalue_3 (Transformation|GetRelativeTransform _startbutton_2))
  (bind _returnvalue_4 (Transformation|GetRelativeTransform _startbutton))
  (bind _returnvalue_5 (Transformation|GetWorldLocation _startbar))
  (bind _returnvalue_6 (Transformation|GetRelativeTransform _rightbutton))
  (bind _returnvalue_7 (Transformation|GetRelativeTransform _rightbutton_2))
  (bind _returnvalue_8 (- (.location _returnvalue_2) "0.000000,3.000000,0.000000"))
  (bind _returnvalue_9 (+ (.location _returnvalue_4) "3.000000,0.000000,0.000000"))
  (bind _returnvalue_10 (- (.location _returnvalue_6) "0.000000,3.000000,0.000000"))
  (bind _returnvalue_11 (+ (.location _returnvalue_7) "0.000000,3.000000,0.000000"))
  (bind _returnvalue_12 (+ (.location _returnvalue) "0.000000,3.000000,0.000000"))
  (bind _returnvalue_13 (- (.location _returnvalue_3) "3.000000,0.000000,0.000000"))
  (bind _returnvalue_14 (- (.z _returnvalue_5) _startbarzlocationspeed))
  (bind _returnvalue_15 (Math|Float|Clamp(Float) (.x _returnvalue_9) _minoffsetbuttonstart_2 _maxoffsetbuttonstart_2))
  (bind _returnvalue_16 (Math|Float|Clamp(Float) (.x _returnvalue_13) _minoffsetbuttonstart _maxoffsetbuttonstart))
  ;[1 1 1] Event tick
  (Utilities|FlowControl|Sequence
    (:then_0
      (if (Collision|IsOverlappingActor (Variables|Default|GetStartButtonCollision) (Variables|Default|GetPG1) :!class /Script/Engine.PrimitiveComponent)
        (Components|MoveComponentTo _startbutton (Math|Vector|MakeVector _returnvalue_15 (.y _returnvalue_9) (.z _returnvalue_9)) (.rotation _returnvalue_4) false true (Variables|Default|GetOver%20Time) false)
        (if (<= _returnvalue_15 (Variables|ButtonStart|GetMaxOffsetButtonStart))
          (Utilities|FlowControl|DoOnce false :!label _label
            (:Completed
              (Variables|ButtonStart|SetCanStartBarGoDown? true))))
        (else
          (Components|MoveComponentTo _startbutton_2 (Math|Vector|MakeVector _returnvalue_16 (.y _returnvalue_13) (.z _returnvalue_13)) (.rotation _returnvalue_3) false true (Variables|Default|GetOver%20Time) false)
          (if (>= _returnvalue_16 (Variables|ButtonStart|GetMinOffsetButtonStart))
            (if (not (Variables|ButtonStart|GetCanStartBarGoDown?))
              (goto _label Reset))))))
    (:then_1
      (if (Variables|ButtonStart|GetCanStartBarGoDown?)
        (if (<= _returnvalue_14 (Variables|ButtonStart|GetStartBarMinZlocation))
          (Utilities|FlowControl|Delay (Variables|ButtonStart|GetStartBarDurationRespawn))
          (Variables|ButtonStart|SetCanStartBarGoDown? false)
          (Transformation|SetRelativeLocation (Variables|Default|GetStartBar) (Variables|ButtonStart|GetStartBarInitialTransform) false false)
          (else
            (Transformation|SetWorldLocation _startbar (Math|Vector|MakeVector (.x _returnvalue_5) (.y _returnvalue_5) _returnvalue_14) false false)))))
    (:then_2
      (if (Collision|IsOverlappingActor (Variables|Default|GetRightButtonCollision) (Variables|Default|GetPG1) :!class /Script/Engine.PrimitiveComponent)
        (Variables|ForceToApply|SetCanApplyForceRight? true)
        (Utilities|FlowControl|Sequence
          (:then_0
            (Components|MoveComponentTo _rightbutton (Math|Vector|MakeVector (.x _returnvalue_10) (Math|Float|Clamp(Float) (.y _returnvalue_10) (Variables|Levette|GetMinOffsetButtonLevettaRight) (Variables|Levette|GetMaxOffsetButtonLevettaRight)) (.z _returnvalue_10)) (.rotation _returnvalue_6) false true (Variables|Default|GetOver%20Time) false))
          (:then_1
            (Components|MoveComponentTo _rightflipper (Variables|/Script/Engine.SceneComponent|GetRelativeLocation _rightflipper) (Variables|Levette|GetLevettaRightPressedRotation) false true (Variables|Default|GetOver%20Time) false)))
        (else
          (Variables|ForceToApply|SetCanApplyForceRight? false)
          (Utilities|FlowControl|Sequence
            (:then_0
              (Components|MoveComponentTo _rightbutton_2 (Math|Vector|MakeVector (.x _returnvalue_11) (Math|Float|Clamp(Float) (.y _returnvalue_11) (Variables|Levette|GetMinOffsetButtonLevettaRight) (Variables|Levette|GetMaxOffsetButtonLevettaRight)) (.z _returnvalue_11)) (.rotation _returnvalue_7) false true (Variables|Default|GetOver%20Time) false))
            (:then_1
              (Components|MoveComponentTo _rightflipper_2 (Variables|/Script/Engine.SceneComponent|GetRelativeLocation _rightflipper_2) (Variables|Levette|GetLevettaRighReleasedRotation) false true (Variables|Default|GetOver%20Time) false))))))
    (:then_3
      (if (Collision|IsOverlappingActor (Variables|Default|GetLeftButtonCollision) (Variables|Default|GetPG1) :!class /Script/Engine.PrimitiveComponent)
        (Variables|ForceToApply|SetCanApplyForceLeft? true)
        (Utilities|FlowControl|Sequence
          (:then_0
            (Components|MoveComponentTo _lefttbutton_2 (Math|Vector|MakeVector (.x _returnvalue_12) (Math|Float|Clamp(Float) (.y _returnvalue_12) (Variables|Levette|GetMinOffsetButtonLevettaLeft) (Variables|Levette|GetMaxOffsetButtonLevettaLeft)) (.z _returnvalue_12)) (.rotation _returnvalue) false true (Variables|Default|GetOver%20Time) false))
          (:then_1
            (Components|MoveComponentTo _leftflipper (Variables|/Script/Engine.SceneComponent|GetRelativeLocation _leftflipper) (Variables|Levette|GetLevettaLeftPressedRotation) false true (Variables|Default|GetOver%20Time) false)))
        (else
          (Variables|ForceToApply|SetCanApplyForceLeft? false)
          (Utilities|FlowControl|Sequence
            (:then_0
              (Components|MoveComponentTo _lefttbutton (Math|Vector|MakeVector (.x _returnvalue_8) (Math|Float|Clamp(Float) (.y _returnvalue_8) (Variables|Levette|GetMinOffsetButtonLevettaLeft) (Variables|Levette|GetMaxOffsetButtonLevettaLeft)) (.z _returnvalue_8)) (.rotation _returnvalue_2) false true (Variables|Default|GetOver%20Time) false))
            (:then_1
              (Components|MoveComponentTo _leftflipper_2 (Variables|/Script/Engine.SceneComponent|GetRelativeLocation _leftflipper_2) (Variables|Levette|GetLevettaLeftReleasedRotation) false true (Variables|Default|GetOver%20Time) false))))))))

(fn ConstructionScript)