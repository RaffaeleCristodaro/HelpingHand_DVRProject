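; BP_CrouchingArea is a trigger volume that makes the PG3 player character crouch while inside it.
; On BeginPlay it caches the PG3 reference through GetPlayer3.
; Its Box overlap events call Crouching on PG3 at entry and Uncrouching at exit, ignoring all other actors.
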(event OnComponentBeginOverlap(Box)
  (params (OverlappedComponent :type Primitive%20Component%20Object%20Reference) (OtherActor :type Actor%20Object%20Reference) (OtherComp :type Primitive%20Component%20Object%20Reference) (OtherBodyIndex :type Integer) (bFromSweep :type Boolean) (SweepResult :type Hit%20Result%20Structure%20%28by%20ref%29))
  ;[1 1 1] Collision with player
  (if (== OtherActor (Variables|Default|GetPG3))
    (Default|Crouching (Variables|Default|GetPG3))))

(event OnComponentEndOverlap(Box)
  (params (OverlappedComponent :type Primitive%20Component%20Object%20Reference) (OtherActor :type Actor%20Object%20Reference) (OtherComp :type Primitive%20Component%20Object%20Reference) (OtherBodyIndex :type Integer))
  ;[1 1 1] Collision with player
  (if (== OtherActor (Variables|Default|GetPG3))
    (Default|Uncrouching (Variables|Default|GetPG3))))

(event EventBeginPlay
  ;[1 1 1] Initialize
  (bind _pg3 (CallFunction|GetPlayer3))
  (Variables|Default|SetPG3 _pg3))

(fn ConstructionScript)