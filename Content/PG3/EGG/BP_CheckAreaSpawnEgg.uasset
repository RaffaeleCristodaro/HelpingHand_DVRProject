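; Area checker for the PG3 egg's spawn zone that tracks whether it has been cleared of grabbable objects.
; Each Tick it counts grabbables overlapping its Box against NumberOfObjectLeft.
; At or below that threshold, a DoOnce clears the egg's HasNotBeenHatchedCorrectly flag and hides the tutorial UI.
; While above it, the tutorial UI rotates to face Player 1's camera.
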(event EventBeginPlay
  ;[1 1 1] Initialize
  (bind _returnvalue (Actor|GetActorOfClass "/Game/PG3/EGG/BPG_EggPG3.BPG_EggPG3_C"))
  (Variables|Default|SetEgg _returnvalue)
  (bind _pg1 (CallFunction|GetPlayer1))
  (Variables|Default|SetPG1 _pg1))

(event EventTick
  (params (DeltaSeconds :type Float%20%28single-precision%29))
  (bind _uitutorial (Variables|Default|GetUITutorial))
  (bind _uitutorial_2 (Variables|Default|GetUITutorial))
  (bind _pg1 (Variables|Default|GetPG1))
  (bind _returnvalue (Transformation|GetWorldLocation _uitutorial_2))
  (bind _camera (Variables|/Game/VRTemplate/Blueprints/VRPawn.VRPawn_C|GetCamera _pg1))
  (bind _returnvalue_2 (Transformation|GetWorldLocation _camera))
  (bind _returnvalue_3 (Math|Rotator|FindLookatRotation _returnvalue _returnvalue_2))
  ;[1 1 1] Overlap with grabbables
  (if (<= (Utilities|Array|Length (Collision|GetOverlappingActors (Variables|Default|GetBox) "/Game/Blueprint_Grabbable/BP_InteractiveGrabbablesParent.BP_InteractiveGrabbablesParent_C" :!class /Script/Engine.PrimitiveComponent)) (Variables|Default|GetNumberOfObjectLeft))
    (Utilities|FlowControl|DoOnce false
      (:Completed
        (Variables|/Game/PG3/EGG/BPG_EggPG3.BPG_EggPG3_C|SetHasNotBeenHatchedCorrectly? (Variables|Default|GetEgg) false)
        (Utilities|IsValid _uitutorial
          (:Is%20Valid
            (Development|SetHiddeninGame _uitutorial true false)))))
    (else
      (Transformation|SetWorldRotation _uitutorial_2 (Math|Rotator|MakeRotator (.roll _returnvalue_3) (.pitch _returnvalue_3) (.yaw _returnvalue_3)) false false))))

(fn ConstructionScript)