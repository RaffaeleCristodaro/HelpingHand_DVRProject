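; Trigger-box actor that controls when the jump tutorial UI shows on the PG3 player.
; Entering the box while CanShowJump is on removes the player's existing UITutorial component and enables the jump UI; leaving disables it.
; While the player stays inside, Tick starts a delayed check through a resettable DoOnce, showing the UI only if the player is nearly still.
; Turning CanShowJump off hides the prompt.
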(event OnComponentBeginOverlap(Box)
  (params (OverlappedComponent :type Primitive%20Component%20Object%20Reference) (OtherActor :type Actor%20Object%20Reference) (OtherComp :type Primitive%20Component%20Object%20Reference) (OtherBodyIndex :type Integer) (bFromSweep :type Boolean) (SweepResult :type Hit%20Result%20Structure%20%28by%20ref%29))
  (bind _pg3 (Variables|Default|GetPG3))
  (bind _uitutorial (Variables|/Game/PG3/BP_PG3.BP_PG3_C|GetUITutorial _pg3))
  ;[1 1 1] Collision with PG3
  (if (Variables|Default|GetCanShowJump?)
    (Utilities|IsValid _uitutorial
      (:Is%20Valid
        (Components|DestroyComponent _uitutorial)
        (Variables|/Game/PG3/BP_PG3.BP_PG3_C|SetCanShowJumpUI? _pg3 true)))))

(event OnComponentEndOverlap(Box)
  (params (OverlappedComponent :type Primitive%20Component%20Object%20Reference) (OtherActor :type Actor%20Object%20Reference) (OtherComp :type Primitive%20Component%20Object%20Reference) (OtherBodyIndex :type Integer))
  ;[1 1 1] Collision with PG3
  (Variables|/Game/PG3/BP_PG3.BP_PG3_C|SetCanShowJumpUI? (Variables|Default|GetPG3) false))

(event Custom|ShowUITutorial
  ;[1 1 1] Show UI jump
  (Utilities|Time|SetTimerbyEvent (delegate Custom|ShowUITutorialTimerEvent) (Variables|UI|GetTimeToShowUI)))

(event Custom|ShowUITutorialTimerEvent
  ;[1 1 1] Show UI jump
  (if (Variables|Default|GetCanShowJump?)
    (if (>= (Math|Vector|VectorLength (Transformation|GetVelocity (Variables|Default|GetPG3))) 0.1)
      (Variables|/Game/PG3/BP_PG3.BP_PG3_C|SetCanShowJumpUI? (Variables|Default|GetPG3) false)
      (else
        (Variables|/Game/PG3/BP_PG3.BP_PG3_C|SetCanShowJumpUI? (Variables|Default|GetPG3) true))))
  (CallFunction|RestorePG3CheckinUIJump))

(event Custom|RestorePG3CheckInUIJump
  ;[1 1 1] Event tick
  (Utilities|FlowControl|DoOnce false) ; enters at Reset
)

(event EventBeginPlay
  ;[1 1 1] Initialize
  (bind _pg3 (CallFunction|GetPlayer3))
  (Variables|Default|SetPG3 _pg3))

(event EventTick
  (params (DeltaSeconds :type Float%20%28single-precision%29))
  ;[1 1 1] Event tick
  (if (Variables|Default|GetCanShowJump?)
    (if (Collision|IsOverlappingActor (Variables|Default|GetBox) (Variables|Default|GetPG3) :!class /Script/Engine.PrimitiveComponent)
      (Utilities|FlowControl|DoOnce false
        (:Completed
          (CallFunction|ShowUITutorial)))
      (else
        (Variables|/Game/PG3/BP_PG3.BP_PG3_C|SetCanShowJumpUI? (Variables|Default|GetPG3) false)))
    (else
      (Utilities|FlowControl|DoOnce false
        (:Completed
          (Variables|/Game/PG3/BP_PG3.BP_PG3_C|SetCanShowJumpUI? (Variables|Default|GetPG3) false))))))

(fn ConstructionScript)