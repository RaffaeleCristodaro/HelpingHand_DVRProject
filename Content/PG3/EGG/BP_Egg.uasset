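; BP_Egg is an egg actor that enables the player's telekinesis, opens its tutorial panel and can hatch.
; Activate lets the static mesh simulate physics briefly, then freezes it, starts spawn Niagara, sets the controller's telekinesis flag and starts the VR pawn's check.
; Hatching stops that effect, disables mesh collision, plays the skeletal animation and fires a hatch effect.
; Disappear waits, then uses a timeline to shrink the actor to zero scale.
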(event Custom|Activate
  ;[1 1 1] Activate
  (Physics|SetSimulatePhysics (Variables|Default|GetStaticMesh) true)
  (Physics|SetPhysicsLinearVelocity (Variables|Default|GetStaticMesh) "0, 0, 0" false "None")
  (Utilities|FlowControl|Delay 1.5)
  (Components|Activation|Activate (Variables|Default|GetNiagara_Spawn) false)
  (Physics|SetPhysicsLinearVelocity (Variables|Default|GetStaticMesh) "0, 0, 0" false "None")
  (Physics|SetSimulatePhysics (Variables|Default|GetStaticMesh) false)
  (Variables|/Game/Managers/PlayerController/BPC_PlayerController_Default.BPC_PlayerController_Default_C|SetCanTelekinesis (CallFunction|GetPlayerController) true)
  (Default|StartCheckTelekinesis (Default|GetVRPawnRef (CallFunction|GetGameMode)))
  (Default|ActivateTutorialPanel (Variables|Ref|GetTutorialTelekinesis)))

(event Custom|Hatching
  ;[1 1 1] Egg Hatching
  (Components|Activation|Deactivate (Variables|Default|GetNiagara_Spawn))
  (Collision|SetCollisionEnabled (Variables|Default|GetStaticMesh) "NoCollision")
  (Components|Animation|PlayAnimation (Variables|Default|GetSkeletalMesh) "/Game/PG3/EGG/Uovo_Anim.Uovo_Anim" false)
  (Utilities|FlowControl|Delay 0.2)
  (Components|Activation|Activate (Variables|Default|GetNiagara_Hatch) false))

(event Custom|Disappear
  ;[1 1 1] Disappear
  (Utilities|FlowControl|Delay 2.0)
  (bind _scale (Timeline|Scale PlayFromStart)
    (:Update
      (Transformation|SetActorScale3D (Math|Vector|Lerp(Vector) (Transformation|GetActorScale3D) "0, 0, 0" _scale)))))

(fn ConstructionScript)