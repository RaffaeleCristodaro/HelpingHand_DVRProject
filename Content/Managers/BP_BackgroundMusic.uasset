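; BP_BackgroundMusic is a music manager with two audio tracks, meant to crossfade background music through ChangeMusic.
; ChangeMusic takes a sound, volume and fade duration, with helper checks to find the sole playing track and swap to the other.
; As wired, the "none playing" test passes unless both tracks play, so music always goes to MusicTrack1 and the crossfade branches cannot fire.
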(fn ConstructionScript)

(fn ChangeMusic
  (params (NewMusic :type Sound%20Base%20Object%20Reference) (Volume :type Float%20%28double-precision%29) (FadeDuration :type Float%20%28double-precision%29))
  (bind _musictrack_1 (Variables|Default|GetMusicTrack_1))
  (bind _musictrack_2 (Variables|Default|GetMusicTrack_2))
  (bind _musictrack_1_2 (Variables|Default|GetMusicTrack_1))
  (LocalVariables|SetMusic NewMusic)
  ;[1 1 1] Check if NONE is playing
  (if (not (and (Audio|Components|Audio|IsPlaying (Variables|Default|GetMusicTrack_2)) (Audio|Components|Audio|IsPlaying (Variables|Default|GetMusicTrack_1))))
    ;[1 1 1] First music set
    (Audio|Components|Audio|SetSound _musictrack_1 (LocalVariables|GetMusic))
    (Audio|Components|Audio|FadeIn _musictrack_1 FadeDuration 1.0 0.0 "Linear" :!class /Script/Engine.AudioComponent)
    (Audio|Components|Audio|SetVolumeMultiplier _musictrack_1 Volume :!class /Script/Engine.AudioComponent)
    (else
      (Utilities|FlowControl|Sequence
        (:then_0
          ;[1 1 1] Play 2 Track
          (if (CallFunction|IsPlayingFirstTrack?)
            (Audio|Components|Audio|SetSound _musictrack_2 (LocalVariables|GetMusic))
            (Audio|Components|Audio|FadeIn _musictrack_2 FadeDuration 1.0 0.0 "Linear" :!class /Script/Engine.AudioComponent)
            (Audio|Components|Audio|SetVolumeMultiplier _musictrack_2 Volume :!class /Script/Engine.AudioComponent)
            (Audio|Components|Audio|FadeOut (Variables|Default|GetMusicTrack_1) FadeDuration 0.0 "Linear" :!class /Script/Engine.AudioComponent)))
        (:then_1
          ;[1 1 1] Play 1 Track
          (if (CallFunction|IsPlayingSecondTrack?)
            (Audio|Components|Audio|SetSound _musictrack_1_2 (LocalVariables|GetMusic))
            (Audio|Components|Audio|FadeIn _musictrack_1_2 FadeDuration 1.0 0.0 "Linear" :!class /Script/Engine.AudioComponent)
            (Audio|Components|Audio|SetVolumeMultiplier _musictrack_1_2 Volume :!class /Script/Engine.AudioComponent)
            (Audio|Components|Audio|FadeOut (Variables|Default|GetMusicTrack_2) FadeDuration 0.0 "Linear" :!class /Script/Engine.AudioComponent)))))))

(fn IsPlayingFirstTrack?
  (return (and (Audio|Components|Audio|IsPlaying (Variables|Default|GetMusicTrack_1)) (not (Audio|Components|Audio|IsPlaying (Variables|Default|GetMusicTrack_2))))))

(fn IsPlayingSecondTrack?
  (return (and (Audio|Components|Audio|IsPlaying (Variables|Default|GetMusicTrack_2)) (not (Audio|Components|Audio|IsPlaying (Variables|Default|GetMusicTrack_1))))))