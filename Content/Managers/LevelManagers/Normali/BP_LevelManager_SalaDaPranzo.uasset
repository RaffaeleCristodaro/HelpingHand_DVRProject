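; BP_LevelManager_SalaDaPranzo is the level manager for the dining room level, restoring that room's special assets on respawn.
; RespawnSpecialAsset runs three passes: it resets destructible shelves (BP_MensolaDistruttibile), restores sinking objects and resets the mesh throw on monster spawn handlers.
; Each pass gathers its actors from the world, using class lookups for shelves and handlers and the BPI_SinkingObject interface for sinking objects.
; The construction script only calls its parent.
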(fn ConstructionScript
  (|CallParentFunction))

(fn RespawnSpecialAsset
  ;[1 1 1] Restore
  (Utilities|FlowControl|Sequence
    (:then_0
      (bind _outactors (Actor|GetAllActorsOfClass "/Game/Asset_SalaDaPranzo/BP/BP_MensolaDistruttibile.BP_MensolaDistruttibile_C"))
      (for _array_element _outactors
        (Utilities|IsValid _array_element
          (:Is%20Valid
            (Default|ResetMensolaEvent _array_element)))))
    (:then_1
      (bind _outactors_2 (Actor|GetAllActorswithInterface "/Game/Managers/BlueprintInterfaces/BPI_SinkingObject.BPI_SinkingObject_C"))
      (for _array_element_2 _outactors_2
        (Class|BPISinkingObject|RestoreSinking(Message) _array_element_2)))
    (:then_2
      (bind _outactors_3 (Actor|GetAllActorsOfClass "/Game/Asset_SalaDaPranzo/BP/MonsterSpawn/BP_MonsterSpawnHandler.BP_MonsterSpawnHandler_C"))
      (for _array_element_3 _outactors_3
        (Utilities|IsValid _array_element_3
          (:Is%20Valid
            (Default|ResetMeshThrow _array_element_3)))))))