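; BP_LevelManager_Bagno is the level manager for the Bagno (bathroom) level, which puts a mask on the VR player at start.
; On BeginPlay it runs the parent logic, then finds and stores the VRPawn.
; It adds a static mesh component to the pawn at runtime with the Maschera_LP mesh.
; The mask snaps to the pawn's MaskLocation, keeps world scale and has collision disabled.
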(event EventBeginPlay
  ;[1 0.07812 0.07812 1 50] Begin Play
  (|CallParentFunction)
  (bind _returnvalue (Actor|GetActorOfClass "/Game/Characters/VRPawn.VRPawn_C"))
  (bind _output_get (Variables|Default|SetVRPawn _returnvalue))
  (bind _returnvalue_2 (AddComponent|AddStaticMeshComponent _output_get false (Variables|Default|GetRelativeTransformMaskPlayer)))
  (bind _output_get_2 (Variables|Default|SetSM_Mask _returnvalue_2))
  (Components|StaticMesh|SetStaticMesh _output_get_2 "/Game/Asset_Bagno/Mesh/Maschera_LP.Maschera_LP")
  (Transformation|AttachComponentToComponent (Variables|Default|GetSM_Mask) (Variables|/Game/Characters/VRPawn.VRPawn_C|GetMaskLocation (Variables|Default|GetVRPawn)) "None" "SnapToTarget" "SnapToTarget" "KeepWorld" true)
  (Collision|SetCollisionEnabled (Variables|Default|GetSM_Mask) "NoCollision"))

(fn ConstructionScript
  (|CallParentFunction))