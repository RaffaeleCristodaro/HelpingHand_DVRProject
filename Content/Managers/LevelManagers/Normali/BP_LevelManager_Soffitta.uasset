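; Level manager for the Soffitta level, running the VR opening sequence from main menu through egg hatching to the PG3 tutorial.
; BeginPlay resets power-up save flags and restricts the player mostly to telekinesis, grab and snap rotation.
; Starting the game places and activates the egg; telekinesis on every listed item triggers hatching.
; When hatching finishes, it teleports PG3 and the VR pawn, enables movement and attaches PG3's tutorial widget.
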(event Custom|SetJumpTutorial_UI
  (bind _ref_tutorialwidgetpg3 (Variables|References|GetRef_TutorialWidgetPG3))
  ;[1 1 1] Set Jump Tutorial UI
  (Rendering|SetActorHiddenInGame _ref_tutorialwidgetpg3 false)
  (Default|SwitchTutorialType _ref_tutorialwidgetpg3 1))

(event Custom|SetMoveTutorial_UI
  (bind _ref_tutorialwidgetpg3 (Variables|References|GetRef_TutorialWidgetPG3))
  ;[1 1 1] Set Move Tutorial UI
  (Rendering|SetActorHiddenInGame _ref_tutorialwidgetpg3 false)
  (Default|SwitchTutorialType _ref_tutorialwidgetpg3))

(event Custom|Local_StartGame
  (bind _ref_egg (Variables|References|GetRef_Egg))
  ;[0 0 0 1 50] Custom Events
  ;;[1 1 1] Start Game
  (Transformation|SetActorLocation _ref_egg (Transformation|GetWorldLocation (Variables|Default|GetEggStartSpawnLocation)) false false)
  (Default|Activate _ref_egg))

(event Custom|OnEggHatchingFinish
  (bind (_pg3startlocation _pg3startrotation) (CallFunction|GetPG3Location&Rotation))
  ;[0 0 0 1 50] Custom Events
  ;;[1 1 1] On egg hatching Finish
  (Default|TeleportPG3 (CallFunction|GetGameMode) _pg3startlocation _pg3startrotation)
  (Variables|/Game/Managers/PlayerController/BPC_PlayerController_Default.BPC_PlayerController_Default_C|SetCanMove (CallFunction|GetPlayerController) true)
  (bind _returnvalue (Game|SpawnActorfromClass "/Game/Managers/UserInterface/BP_WidgetTutorialSpawner_PG3.BP_WidgetTutorialSpawner_PG3_C" (Math|Transform|MakeTransform "0, 0, 0" "0, 0, 0" "1.000000,1.000000,1.000000") "Undefined" 0 0))
  (bind _output_get (Variables|References|SetRef_TutorialWidgetPG3 _returnvalue))
  (Transformation|AttachActorToActor _returnvalue (Default|GetPG3Ref (CallFunction|GetGameMode)) "None" "SnapToTarget" "SnapToTarget" "KeepRelative" true)
  (Default|TeleportVRPawn (CallFunction|GetGameMode) (Variables|Editable|GetAfterStartLocation) (Variables|Editable|GetAfterStartRotation) false true)
  (CallFunction|SetMoveTutorialUI))

(event EventStartGame
  ;[1 0.03702 0.9005 1 50] Interface
  ;;[1 1 1] Start Game
  (CallFunction|LocalStartGame))

(event EventBeginPlay
  (bind _gameinstance (CallFunction|GetGameInstance))
  (bind _controllerref (CallFunction|GetPlayerController))
  (bind _currentsave (Default|GetCurrentSave _gameinstance))
  ;[1 0.07812 0.07812 1 50] Begin Play
  (|CallParentFunction)
  (Utilities|FlowControl|Delay 0.01)
  (Variables|/Game/Managers/SG_HelpingHand.SG_HelpingHand_C|SetHasPlayerUnclokedFirstPowerUp? _currentsave false)
  (Variables|/Game/Managers/SG_HelpingHand.SG_HelpingHand_C|SetHasPlayerUnclokedSecondPowerUp? _currentsave false)
  (Variables|/Game/Managers/SG_HelpingHand.SG_HelpingHand_C|SetHasPlayerUnclokedSecondThridPowerUp? _currentsave false)
  (Variables|/Game/Managers/VRGameMode.VRGameMode_C|SetCanPauseGame (CallFunction|GetGameMode) false)
  (Variables|/Game/Managers/PlayerController/BPC_PlayerController_Default.BPC_PlayerController_Default_C|SetCanTelekinesis _controllerref true)
  (Variables|/Game/Managers/PlayerController/BPC_PlayerController_Default.BPC_PlayerController_Default_C|SetCanSnapRotate _controllerref true)
  (Variables|/Game/Managers/PlayerController/BPC_PlayerController_Default.BPC_PlayerController_Default_C|SetCanJump _controllerref false)
  (Variables|/Game/Managers/PlayerController/BPC_PlayerController_Default.BPC_PlayerController_Default_C|SetCanMove _controllerref false)
  (Variables|/Game/Managers/PlayerController/BPC_PlayerController_Default.BPC_PlayerController_Default_C|SetCanGesture _controllerref false)
  (Variables|/Game/Managers/PlayerController/BPC_PlayerController_Default.BPC_PlayerController_Default_C|SetCanGrab _controllerref true)
  (bind _returnvalue (Actor|GetActorOfClass "/Game/PG3/EGG/BPG_EggPG3.BPG_EggPG3_C"))
  (Variables|References|SetRef_Egg _returnvalue)
  (bind _returnvalue_2 (Actor|GetActorOfClass "/Game/Managers/UserInterface/BP_MainMenu.BP_MainMenu_C"))
  (bind _output_get (Variables|References|SetRef_CurrentMainMenu _returnvalue_2))
  (Variables|References|SetRef_CurrentMainMenuWidget (Default|GetMenuWidget _output_get))
  (EventDispatchers|AssignOnTelekinesisStarted (CallFunction|GetPlayerController) (delegate OnTelekinesisStarted))
  (for _array_element (Variables|Editable|GetItemsToGrabForEggHatching)
    (if (Utilities|DoesObjectImplementInterface _array_element "/Game/Managers/BlueprintInterfaces/BPI_InteractiveGrabbable.BPI_InteractiveGrabbable_C")
      (bind _grabbable (Class|BPIInteractiveGrabbable|GetGrabbableParent(Message) _array_element))
      (EventDispatchers|AssignOnTelekinesis _grabbable (delegate OnTelekinesisStart)))))

(event EventActivateMenu
  ;[1 0.03702 0.9005 1 50] Interface
  ;;[1 1 1] Activate Menu
  (Default|ActivateMenu (Variables|References|GetRef_CurrentMainMenuWidget)))

(fn ConstructionScript
  (|CallParentFunction)
  (Transformation|SetRelativeLocation (Variables|Default|GetEggStartSpawnLocation) (Variables|Editable|GetEggSpawnLocation) false true)
  (Transformation|SetRelativeLocationAndRotation (Variables|Default|GetVRPawnAfterStartLocation) (Variables|Editable|GetAfterStartLocation) (Variables|Editable|GetAfterStartRotation) false false))

(event Custom|OnTelekinesis_Started_Event
  (params (RightHand? :type Boolean))
  (Default|DeactivateTutorialPanel (Variables|Editable|GetTutorialTelekinesis)))

(event Custom|OnGrabbed_Event
  (bind _currentgrabbedobjectsforegghatching (Variables|Default|GetCurrentGrabbedObjectsForEggHatching))
  (Math|Integer|IncrementInt _currentgrabbedobjectsforegghatching
    (:%20%20
      (EventDispatchers|UnbindEventfromOnTelekinesis (|Inputs) (delegate Custom|OnGrabbed_Event))
      (if (== _currentgrabbedobjectsforegghatching (Utilities|Array|Length (Variables|Editable|GetItemsToGrabForEggHatching)))
        (Default|Hatching (Variables|References|GetRef_Egg))))))

(fn GetManagerSoffitta
  (return self))