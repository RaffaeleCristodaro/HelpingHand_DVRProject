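; Master level manager for the VR game, configuring player start points, permissions and progress for a level.
; On BeginPlay it disables gestures on the game mode, starts a delayed camera fade-in, and copies power-up unlock flags and ability toggles to the save, game mode and player controller.
; It optionally attaches a world tips widget to the VR pawn.
; Getters expose PG3 and VR pawn spawn transforms, with PG3 yaw offset 90 degrees.
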(event EventBeginPlay
  ;[1 0.08229 0.08229 1 50] Begin Play
  (bind _gamemoderef (Class|BPIGameMode|GetGameModeRef(Message) (Game|GetGameMode)))
  (bind _output_get (Variables|References|SetRef_GameMode _gamemoderef))
  (Variables|/Game/Managers/VRGameMode.VRGameMode_C|SetCanUseGestures _output_get false)
  (Default|FadeVisual (Default|GetCameraFade (Variables|References|GetRef_GameMode)) 0.5 2.0 true)
  (CallFunction|SetVariablesLevelManager)
  (CallFunction|SpawnTipsWidget))

(fn ConstructionScript
  (Transformation|SetRelativeLocation (Variables|Default|GetPG3SpawnLocation) (Variables|Editables|GetPG3SpawnLocation_) false false))

(fn GetPG3Location&Rotation
  (bind _pg3spawnlocation (Variables|Default|GetPG3SpawnLocation))
  (bind _returnvalue (Transformation|GetWorldRotation _pg3spawnlocation))
  (return (Transformation|GetWorldLocation (Variables|Default|GetPG3SpawnLocation)) (Math|Rotator|MakeRotator (.roll _returnvalue) (.pitch _returnvalue) (+ (.yaw _returnvalue) 9e+01))))

(fn GetVRPawnLocation&Rotation
  (bind _vrpawnspawn (Variables|Default|GetVRPawnSpawn))
  (return (Transformation|GetWorldLocation _vrpawnspawn) (Transformation|GetWorldRotation _vrpawnspawn)))

(fn SetVariablesLevelManager
  (bind _gameinstance (CallFunction|GetGameInstance))
  (bind _controllerref (CallFunction|GetPlayerController))
  (bind _currentsave (Default|GetCurrentSave _gameinstance))
  (Variables|/Game/Managers/SG_HelpingHand.SG_HelpingHand_C|SetHasPlayerUnclokedFirstPowerUp? _currentsave (Variables|LevelManagerSettings|GetHasPlayerUnlockedFirstPowerUp?))
  (Variables|/Game/Managers/SG_HelpingHand.SG_HelpingHand_C|SetHasPlayerUnclokedSecondPowerUp? _currentsave (Variables|LevelManagerSettings|GetHasPlayerUnlockedSecondPowerUp?))
  (Variables|/Game/Managers/SG_HelpingHand.SG_HelpingHand_C|SetHasPlayerUnclokedSecondThridPowerUp? _currentsave (Variables|LevelManagerSettings|GetHasPlayerUnlockedThirdPowerUp?))
  (Variables|/Game/Managers/VRGameMode.VRGameMode_C|SetCanPauseGame (CallFunction|GetGameMode) (Variables|LevelManagerSettings|GetCan%20Pause%20Game))
  (Variables|/Game/Managers/PlayerController/BPC_PlayerController_Default.BPC_PlayerController_Default_C|SetCanTelekinesis _controllerref (Variables|LevelManagerSettings|GetCan%20Telekinesis))
  (Variables|/Game/Managers/PlayerController/BPC_PlayerController_Default.BPC_PlayerController_Default_C|SetCanSnapRotate _controllerref (Variables|LevelManagerSettings|GetCan%20Snap%20Rotate))
  (Variables|/Game/Managers/PlayerController/BPC_PlayerController_Default.BPC_PlayerController_Default_C|SetCanJump _controllerref (Variables|LevelManagerSettings|GetCan%20Jump))
  (Variables|/Game/Managers/PlayerController/BPC_PlayerController_Default.BPC_PlayerController_Default_C|SetCanMove _controllerref (Variables|LevelManagerSettings|GetCan%20Move))
  (Variables|/Game/Managers/PlayerController/BPC_PlayerController_Default.BPC_PlayerController_Default_C|SetCanGesture _controllerref (Variables|LevelManagerSettings|GetCan%20Gesture))
  (Variables|/Game/Managers/PlayerController/BPC_PlayerController_Default.BPC_PlayerController_Default_C|SetCanGrab _controllerref (Variables|LevelManagerSettings|GetCan%20Grab)))

(fn SpawnTipsWidget
  (if (Variables|Tips|GetCanUseTipsInThisLevel?)
    (bind _returnvalue (Game|SpawnActorfromClass "/Game/Managers/UserInterface/BP_Tips_World.BP_Tips_World_C" (Math|Transform|MakeTransform "0, 0, 0" "0, 0, 0" "1.000000,1.000000,1.000000") "Undefined" 0 0))
    (Transformation|AttachComponentToComponent _returnvalue (Variables|/Game/Characters/VRPawn.VRPawn_C|GetTipsWidgetLocation (Default|GetVRPawnRef (CallFunction|GetGameMode))) "None" "SnapToTarget" "KeepWorld" "KeepWorld" true)
    (Variables|/Game/Characters/VRPawn.VRPawn_C|SetCurrentLevelTips (Default|GetVRPawnRef (CallFunction|GetGameMode)) (Variables|Tips|GetTips_CurrentLevel))))