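; Animation notify that plays surface-specific footstep sounds for the animated mesh's owner.
; It line-traces down from the owner's location on the Visibility channel, ignoring an actor fetched from the game mode.
; The hit's physical surface type selects the sound cue played at that location, with wood as the fallback.
; No hit means no sound, and the Grass surface plays the Glass cue.
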(fn ReceivedNotify
  (params (MeshComp :type Skeletal%20Mesh%20Component%20Object%20Reference) (Animation :type Anim%20Sequence%20Base%20Object%20Reference) (EventReference :type Anim%20Notify%20Event%20Reference%20Structure%20%28by%20ref%29))
  (bind _returnvalue (Components|GetOwner MeshComp))
  (bind _returnvalue_2 (Transformation|GetActorLocation _returnvalue))
  (bind _pg3ref (Class|BPIPG3|GetPG3Ref(Message) (Game|GetGameMode)))
  (Utilities|Array|Add (Variables|Default|GetActors%20to%20Ignore) _pg3ref)
  (bind _output_get (LocalVariables|SetSoundLocation (Transformation|GetActorLocation _returnvalue)))
  (bind (_outhit _returnvalue_3) (Collision|LineTraceByChannel _output_get (Math|Vector|MakeVector (.x _returnvalue_2) (.y _returnvalue_2) (- (.z _returnvalue_2) (Variables|Default|GetZLocationToCheckFloor))) "TraceTypeQuery1" false (Variables|Default|GetActors%20to%20Ignore) "None"))
  (if _returnvalue_3
    (switch Utilities|FlowControl|Switch|SwitchonEPhysicalSurface (Collision|GetSurfaceType _outhit)
      (:SurfaceType_Default
        (Audio|PlaySoundatLocation "/Game/SoundSystem/DefinitiveSounds/PG3/Steps/SC_Step_Wood.SC_Step_Wood" (LocalVariables|GetSoundLocation) "0, 0, 0" 1.0 1.0 0.0 "/Game/SoundSystem/SoundAttenuator/SA_MainAttenuation.SA_MainAttenuation" 0 0 0 :!label _label))
      (:SurfaceType1
        (goto _label))
      (:SurfaceType2
        (Audio|PlaySoundatLocation "/Game/SoundSystem/DefinitiveSounds/PG3/Steps/SC_Step_Floor.SC_Step_Floor" (LocalVariables|GetSoundLocation) "0, 0, 0" 1.0 1.0 0.0 "/Game/SoundSystem/SoundAttenuator/SA_MainAttenuation.SA_MainAttenuation" 0 0 0))
      (:SurfaceType3
        (Audio|PlaySoundatLocation "/Game/SoundSystem/DefinitiveSounds/PG3/Steps/SC_Step_Water.SC_Step_Water" (LocalVariables|GetSoundLocation) "0, 0, 0" 1.0 1.0 0.0 "/Game/SoundSystem/SoundAttenuator/SA_MainAttenuation.SA_MainAttenuation" 0 0 0))
      (:SurfaceType4
        (Audio|PlaySoundatLocation "/Game/SoundSystem/DefinitiveSounds/PG3/Steps/SC_Step_Mud.SC_Step_Mud" (LocalVariables|GetSoundLocation) "0, 0, 0" 1.0 1.0 0.0 "/Game/SoundSystem/SoundAttenuator/SA_MainAttenuation.SA_MainAttenuation" 0 0 0))
      (:SurfaceType5
        (Audio|PlaySoundatLocation "/Game/SoundSystem/DefinitiveSounds/PG3/Steps/SC_Step_Metal.SC_Step_Metal" (LocalVariables|GetSoundLocation) "0, 0, 0" 1.0 1.0 0.0 "/Game/SoundSystem/SoundAttenuator/SA_MainAttenuation.SA_MainAttenuation" 0 0 0))
      (:SurfaceType6
        (Audio|PlaySoundatLocation "/Game/SoundSystem/DefinitiveSounds/PG3/Steps/SC_Step_Glass.SC_Step_Glass" (LocalVariables|GetSoundLocation) "0, 0, 0" 1.0 1.0 0.0 "/Game/SoundSystem/SoundAttenuator/SA_MainAttenuation.SA_MainAttenuation" 0 0 0))
      (:SurfaceType7
        (Audio|PlaySoundatLocation "/Game/SoundSystem/DefinitiveSounds/PG3/Steps/SC_Step_Soft.SC_Step_Soft" (LocalVariables|GetSoundLocation) "0, 0, 0" 1.0 1.0 0.0 "/Game/SoundSystem/SoundAttenuator/SA_MainAttenuation.SA_MainAttenuation" 0 0 0))
      (:SurfaceType8
        (Audio|PlaySoundatLocation "/Game/SoundSystem/DefinitiveSounds/PG3/Steps/SC_Step_Cardboard.SC_Step_Cardboard" (LocalVariables|GetSoundLocation) "0, 0, 0" 1.0 1.0 0.0 "/Game/SoundSystem/SoundAttenuator/SA_MainAttenuation.SA_MainAttenuation" 0 0 0))
      (:SurfaceType9
        (Audio|PlaySoundatLocation "/Game/SoundSystem/DefinitiveSounds/PG3/Steps/SC_Step_Plastic.SC_Step_Plastic" (LocalVariables|GetSoundLocation) "0, 0, 0" 1.0 1.0 0.0 "/Game/SoundSystem/SoundAttenuator/SA_MainAttenuation.SA_MainAttenuation" 0 0 0)))
    (return false)))