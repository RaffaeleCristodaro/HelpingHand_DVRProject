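; BP_GameManager is a central manager for save data, enemy spawning, music and level changes, and it uncaps the frame rate at start.
; LoadGame creates the Save_HelpingHand slot or restores PG3's finger and punch interaction unlocks from it.
; A camera-to-PG3 trace plus a line-of-sight check swaps PG3 to a see-through material when hidden.
; Other events spawn physics monsters, switch between random enemy and background music, and open levels after a delay.
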(event EventDeleteGame
  ;[1 1 1] Delete game data
  (SaveGame|DeleteGameinSlot "Save_HelpingHand"))

(event EventLoadGame
  ;[1 1 1] Load or Create game data
  (bind _returnvalue (SaveGame|DoesSaveGameExist "Save_HelpingHand"))
  (if _returnvalue
    (bind _returnvalue_2 (SaveGame|LoadGamefromSlot "Save_HelpingHand"))
    (bind _assg_helping_hand (Utilities|Casting|CastToSG_HelpingHand _returnvalue_2))
    (CallFunction|LoadingOldSaveSlot _assg_helping_hand)
    (else
      (bind _returnvalue_3 (SaveGame|CreateSaveGameObject "/Game/LoadingAndSaving/SG_HelpingHand.SG_HelpingHand_C"))
      (SaveGame|SaveGametoSlot _returnvalue_3 "Save_HelpingHand")
      (Variables|Default|SetSave%20Game%20Ref _returnvalue_3))))

(event EventPG3VisibleThroughWalls
  (params (PlayerCamera :type Camera%20Component%20Object%20Reference) (PG3 :type BP%20PG3%20Object%20Reference))
  ;[1 1 1] PG3 visible through walls
  (bind _outhit (Collision|LineTraceByChannel (Transformation|GetWorldLocation PlayerCamera) (Transformation|GetWorldLocation (Variables|/Script/Engine.Character|GetMesh PG3)) "TraceTypeQuery1" false (Variables|SeeThroughWallsPG3|GetActors%20to%20IgnoreForInvisibility) "None"))
  (Utilities|IsValid (.hitactor _outhit)
    (:Is%20Valid
      (if (Controller|LineOfSightTo (Game|GetPlayerController 0) (Variables|Default|GetPG3) "0, 0, 0" false)
        (Rendering|Material|SetMaterial (Variables|/Script/Engine.Character|GetMesh (Variables|Default|GetPG3)) 0 "/Game/GitIgnore/LearningKit_Games/Assets/Characters/Character/Material/M_EpicCharacter_Optimized.M_EpicCharacter_Optimized")
        (else
          (Rendering|Material|SetMaterial (Variables|/Script/Engine.Character|GetMesh (Variables|Default|GetPG3)) 0 "/Game/PG3/PG3_VisibilityThroughWalls/BP_SeeThroughV3.BP_SeeThroughV3"))))
    (:Is%20Not%20Valid
      (Rendering|Material|SetMaterial (Variables|/Script/Engine.Character|GetMesh (Variables|Default|GetPG3)) 0 "/Game/GitIgnore/LearningKit_Games/Assets/Characters/Character/Material/M_EpicCharacter_Optimized.M_EpicCharacter_Optimized"))))

(event EventChangeLevel
  (params (LevelToOpen :type Name :default "None") (LoadingTime :type Float%20%28double-precision%29))
  ;[1 1 1] Change Level
  (Utilities|FlowControl|Delay LoadingTime)
  (Game|OpenLevel(byName) LevelToOpen))

(event EventBeginPlay
  ;[1 1 1] Initialize
  (bind _returnvalue (Settings|GetGameUserSettings))
  (Class|GameUserSettings|SetFrameRateLimit _returnvalue 0.0)
  (bind _pg3 (CallFunction|GetPlayer3))
  (Variables|Default|SetPG3 _pg3))

(event EventSpawnNemicoFisico
  (params (SpawnPos :type Vector :default "0, 0, 0") (SpawnRotation :type Rotator :default "0, 0, 0"))
  ;[1 1 1] Spawn nemico fisico
  (Game|SpawnActorfromClass "/Game/Enemies/EnemyPhisyc/BP_PhysicMonster.BP_PhysicMonster_C" (Math|Transform|MakeTransform SpawnPos SpawnRotation "1.000000,1.000000,1.000000") "Undefined" 0 0))

(event EventChangeMusicEnemySpawn
  (params (BackgroundMusic :type Audio%20Component%20Object%20Reference))
  (bind _enemiesounds (Variables|NemicoFisico|GetEnemieSounds))
  ;[1 1 1] Change music when an enemy spawn
  (Audio|Components|Audio|Stop BackgroundMusic)
  (bind _returnvalue (Audio|SpawnSound2D (Utilities|Array|Get(acopy) _enemiesounds (Math|Random|RandomIntegerinRange 0 (- (Utilities|Array|Length _enemiesounds) 1))) 1.0 1.0 0.0 0))
  (Variables|NemicoFisico|SetChosenEnemyMusic _returnvalue))

(event EventReturnMusictoBackgroundMusic
  (params (BackGroundMusic :type Sound%20Base%20Object%20Reference))
  (bind _chosenenemymusic (Variables|NemicoFisico|GetChosenEnemyMusic))
  ;[1 1 1] Change music when an enemy spawn
  (Utilities|IsValid _chosenenemymusic
    (:Is%20Valid
      (Audio|Components|Audio|Stop _chosenenemymusic))
    (:Is%20Not%20Valid
      _))
  (bind _returnvalue (Audio|SpawnSound2D BackGroundMusic 1.0 1.0 0.0 0))
  (Variables|NemicoFisico|SetChosenBackgroundMusic _returnvalue))

(fn ConstructionScript)

(fn LoadingOldSaveSlot
  (params (SaveGameRef :type SG%20Helping%20Hand%20Object%20Reference))
  (bind _output_get (Variables|Default|SetSave%20Game%20Ref SaveGameRef))
  (Utilities|FlowControl|Sequence
    (:then_0
      (Variables|PlayerRef|SetHasPlayerUnlockedFingerInteractionWithPG3? (Variables|/Game/LoadingAndSaving/SG_HelpingHand.SG_HelpingHand_C|GetHasPlayerUnclokedFirstPowerUp? _output_get)))
    (:then_1
      (Variables|PlayerRef|SetHasPlayerUnlockedPunchInteractionWithPG3? (Variables|/Game/LoadingAndSaving/SG_HelpingHand.SG_HelpingHand_C|GetHasPlayerUnclokedSecondPowerUp? _output_get)))))