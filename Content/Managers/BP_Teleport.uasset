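; BP_Teleport is a teleport point that moves the VR pawn to its own location and rotation through the game mode.
; It starts at zero scale; an entrance timeline, run on begin play or through an interface call after a delay, scales it up.
; Activation, automatic or via interface, shows a Niagara effect and check sphere.
; Teleporting plays a sound and hides the cylinder; a separate event swaps its highlight material.
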(event Custom|Local_TeleportEntrance
  (params (Delay :type Float%20%28single-precision%29))
  ;[0 0 0 1 50] Custom Events
  ;;[1 1 1] Teleport Entrance
  (Utilities|FlowControl|Delay Delay)
  (Components|Timeline|SetPlayRate (Variables|Default|GetActivationAnimation) (Variables|Teleport|GetEntranceAnimPlayRate))
  (bind _activation (Timeline|ActivationAnimation PlayFromStart)
    (:Update
      (Transformation|SetActorScale3D (Math|Conversions|ToVector(Float) _activation)))
    (:Finished
      (if (Variables|Teleport|GetAutomaticActivation?)
        (CallFunction|LocalTeleportActivation)))))

(event Custom|Local_TeleportActivation
  ;[0 0 0 1 50] Custom Events
  ;;[1 1 1] Activation
  (Components|Activation|Activate (Variables|Default|GetNiagara) false)
  (Rendering|SetVisibility (Variables|Default|GetSphereCheck) true false))

(event Custom|OnTeleportPG
  ;[0 0 0 1 50] Custom Events
  ;;[1 1 1] Teleport player
  (Audio|PlaySound2D 0 1.0 1.0 0.0 0 0)
  (Default|TeleportVRPawn (CallFunction|GetGameMode) (Transformation|GetActorLocation) (Transformation|GetActorRotation) false false)
  (CallFunction|SetTeleportVisibility false)
  (Components|Activation|Deactivate (Variables|Default|GetNiagara))
  (CallFunction|SetOverlay false))

(event Custom|SetTeleportVisibility
  (params (bNewVisibility :type Boolean))
  (bind _niagara (Variables|Default|GetNiagara))
  ;[0 0 0 1 50] Custom Events
  ;;[1 1 1] Set Visibility
  (Rendering|SetVisibility (Variables|Default|GetCylinder) bNewVisibility false)
  (if bNewVisibility
    (Components|Activation|Activate _niagara false)
    (else
      (Components|Activation|Deactivate _niagara))))

(event EventTeleportEntrance
  (params (ActivationDelay :type Float%20%28double-precision%29))
  ;[1 0 0.8018 1 50] Interface
  ;;[1 1 1] Entrance
  (CallFunction|LocalTeleportEntrance ActivationDelay))

(event EventSetOverlay
  (params (Active? :type Boolean))
  (Rendering|Material|SetMaterial (Variables|Default|GetCylinder) 0 (select Active? "/Game/Materials/Materiale_magico/MI_Teleport_Highlight.MI_Teleport_Highlight" "/Game/Materials/Materiale_magico/MI_Teleport.MI_Teleport")))

(event EventBeginPlay
  ;[1 0.06146 0.06146 1 50] Begin Play
  (Transformation|SetActorScale3D "0, 0, 0")
  (if (Variables|Teleport|GetAutomaticActivation?)
    (CallFunction|LocalTeleportEntrance 0.0)
    (Transformation|SetRelativeLocation (Variables|Default|GetCylinder) "0, 0, 0" false false)))

(event EventTeleportActivation
  ;[1 0 0.8018 1 50] Interface
  ;;[1 1 1] Activation
  (CallFunction|LocalTeleportActivation))

(fn ConstructionScript)

(fn GetTelekinesisDistanceOverride
  (return 0.0))

(fn GetTeleport
  (return self))

(fn IsonTelekinesisEffect
  (return false))