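; Teleport spawner that brings an already-referenced Teleport actor into play when an actor implementing BPI_PG3 first enters its overlap volume.
; BeginPlay parks the Teleport at the start marker and prints a tip string built from the string table.
; Activation triggers the Teleport's entrance, slides it along a timeline curve to the end marker, then applies that rotation and sends an activation message.
; Meanwhile, a second timeline fades the symbol through a dynamic material, then hides it.
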(event OnComponentBeginOverlap(Overlap)
  (params (OverlappedComponent :type Primitive%20Component%20Object%20Reference) (OtherActor :type Actor%20Object%20Reference) (OtherComp :type Primitive%20Component%20Object%20Reference) (OtherBodyIndex :type Integer) (bFromSweep :type Boolean) (SweepResult :type Hit%20Result%20Structure%20%28by%20ref%29))
  ;[0 0.7187 1 1 50] Overlap
  ;;[1 1 1] Collsion with PG3
  (if (Utilities|DoesObjectImplementInterface OtherActor "/Game/Managers/BlueprintInterfaces/BPI_PG3.BPI_PG3_C")
    (Utilities|FlowControl|DoOnce false
      (:Completed
        (CallFunction|ActivateTeleport)))))

(event Custom|ActivateTeleport
  (bind _debug_teleportendtransform (Variables|Default|GetDebug_TeleportEndTransform))
  (bind _teleport (Variables|Teleport|GetTeleport))
  ;[0 0 0 1 50] Custom Events
  ;;[1 1 1] Activate Teleport
  (bind _teleport_2 (Variables|Teleport|GetTeleport)
    (:then
      (Transformation|SetActorLocation _teleport_2 (Transformation|GetWorldLocation (Variables|Default|GetDebug_TeleportStartTransform)) false true)
      (Components|Timeline|SetPlayRate (Variables|Default|GetTeleportActivation) (Variables|Settings|GetTeleportPositioningAnimationTime))
      (Default|LocalTeleportEntrance (Variables|Teleport|GetTeleport) 0.0)
      (CallFunction|SymbleDisappear)
      (bind _teleportanimationcurve (Timeline|TeleportActivation PlayFromStart)
        (:Update
          (Transformation|SetActorLocation _teleport (Math|Vector|Lerp(Vector) (Transformation|GetWorldLocation (Variables|Default|GetDebug_TeleportStartTransform)) (Transformation|GetWorldLocation _debug_teleportendtransform) _teleportanimationcurve) false false))
        (:Finished
          (Transformation|SetActorRotation _teleport (Transformation|GetWorldRotation _debug_teleportendtransform))
          (Class|BPITeleport|TeleportActivation(Message) (Variables|Teleport|GetTeleport)))))
    (:else)))

(event Custom|SymbleDisappear
  ;[0 0 0 1 50] Custom Events
  ;;[1 1 1] Disappear Symble
  (Rendering|SetVisibility (Variables|Default|GetSymble) true false)
  (Components|Timeline|SetPlayRate (Variables|Default|GetSymbleDisappearAnim) (Variables|Default|GetSymbleDisappearAnimRate))
  (bind _anim (Timeline|SymbleDisappearAnim PlayFromStart)
    (:Update
      (Rendering|Material|SetScalarParameterValue (Variables|Default|GetRef_Symble_DynamicMaterial) "OpacityMultiplier" _anim :!class /Script/Engine.MaterialInstanceDynamic))
    (:Finished
      (Rendering|SetVisibility (Variables|Default|GetSymble) false false))))

(event EventBeginPlay
  ;[1 0.09896 0.09896 1 50] Initialize
  (Variables|References|SetRef_GameMode (CallFunction|GetGameMode))
  (CallFunction|SymbleCreateDynamicMaterial)
  (bind _teleport (Variables|Teleport|GetTeleport)
    (:then
      (Transformation|SetActorLocation _teleport (CallFunction|GetTeleportStartLocation true) false false)
      (Development|PrintString (Class|KismetStringTableLibrary|GetTableEntrySourceString (.OutTableId (Class|KismetTextLibrary|StringTableIdandKeyfromText "tip_0")) (Utilities|String|Append (Variables|Default|GetKey) (Utilities|String|ToString(Integer) (Variables|Tips|GetTipsIndex)))) true true "(R=0.000000,G=0.660000,B=1.000000,A=1.000000)" 2e+01))
    (:else)))

(fn ConstructionScript
  (CallFunction|SymbleCreateDynamicMaterial)
  (Variables|Frameworks|SetTeleportStartLocation (Transformation|GetWorldLocation (Variables|Default|GetDebug_TeleportStartTransform)))
  (Variables|Frameworks|SetFinalTeleportLocation (Transformation|GetWorldLocation (Variables|Default|GetDebug_TeleportEndTransform))))

(fn SymbleCreateDynamicMaterial
  (bind _symble (Variables|Default|GetSymble))
  (bind _returnvalue (Rendering|Material|CreateDynamicMaterialInstance _symble 0 (Rendering|Material|GetMaterial _symble 0) "None" :!class /Script/Engine.PrimitiveComponent))
  (Variables|Default|SetRef_Symble_DynamicMaterial _returnvalue))

(fn GetTeleportStartLocation
  (params (World? :type Boolean))
  (bind _debug_teleportstarttransform (Variables|Default|GetDebug_TeleportStartTransform))
  (return (Math|Vector|SelectVector (Transformation|GetWorldLocation _debug_teleportstarttransform) (Variables|/Script/Engine.SceneComponent|GetRelativeLocation _debug_teleportstarttransform) World?)))

(fn GetTeleportEndLocation
  (params (World? :type Boolean))
  (bind _debug_teleportendtransform (Variables|Default|GetDebug_TeleportEndTransform))
  (return (Math|Vector|SelectVector (Transformation|GetWorldLocation _debug_teleportendtransform) (Variables|/Script/Engine.SceneComponent|GetRelativeLocation _debug_teleportendtransform) World?)))