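; BP_Rune_Fire is the fire rune pickup, a child Blueprint that extends a parent rune's animation and acquisition events.
; When the rune animation finishes, it flags the player's first power-up as unlocked in the current save and updates that save through the game instance.
; When acquisition finishes, it triggers a power message on the PG3 reference from the game mode and prints a debug string before calling the parent.
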(event EventOnFinishAcquirePowerRune
  (Class|BPIPG3|ActivatePower(Message) (Default|GetPG3Ref (CallFunction|GetGameMode)) "NewEnumerator1")
  (Development|PrintString "Did it!" true true "(R=0.000000,G=0.660000,B=1.000000,A=1.000000)" 5.0)
  (|CallParentFunction))

(event EventOnFinishRuneAnimation
  (bind _gameinstance (CallFunction|GetGameInstance))
  (|CallParentFunction)
  (Variables|/Game/Managers/SG_HelpingHand.SG_HelpingHand_C|SetHasPlayerUnclokedFirstPowerUp? (Default|GetCurrentSave _gameinstance) true)
  (Default|UpdateCurrentSave _gameinstance))

(fn ConstructionScript
  (|CallParentFunction))