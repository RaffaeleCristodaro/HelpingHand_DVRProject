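; BP_Rune is a VR power rune pickup that becomes queryable on Activate and is acquired through Interact.
; Interacting disables sphere collision once and starts a looping timer to interpolate the sphere toward HandLocation, intended as the telekinesis hand.
; On arrival it sets the pawn's rune tutorial flag, shrinks the sphere with the DisappearAnim timeline, then destroys itself.
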(event Custom|OnFinishRuneAnimation
  ;[1 1 1] On Finish Rune Animation
  (Variables|/Game/Characters/VRPawn.VRPawn_C|SetIsRuneModeTutorial? (Default|GetVRPawnRef (CallFunction|GetGameMode)) true)
  (bind _disappear (Timeline|DisappearAnim PlayFromStart)
    (:Update
      (Transformation|SetWorldScale3D (Variables|Default|GetSphere) (Math|Vector|Lerp(Vector) "0.200000,0.200000,0.200000" "0, 0, 0" _disappear)))
    (:Finished
      (CallFunction|OnFinishAcquirePowerRune))))

(event Custom|AnimationTimer
  (bind _returnvalue (Transformation|GetActorLocation))
  (bind _endloc (|HandLocation))
  ;[1 1 1] Animation Timer
  (Transformation|SetWorldLocation (Variables|Default|GetSphere) (Math|Interpolation|VInterpTo _returnvalue _endloc (Utilities|Time|GetWorldDeltaSeconds) 2.0) false false)
  (if (Utilities|Operators|EqualEqual _returnvalue _endloc 3.0)
    (Utilities|FlowControl|DoOnce false
      (:Completed
        (CallFunction|OnFinishRuneAnimation)))))

(event Custom|OnActivation
  ;[1 1 1] On Activation
  (Utilities|FlowControl|DoOnce false
    (:Completed
      (Collision|SetCollisionEnabled (Variables|Default|GetSphere) "NoCollision")
      (bind _returnvalue (Utilities|Time|SetTimerbyEvent (EventDispatchers|CreateEvent :!event Custom|AnimationTimer) 0.005 true))
      (Variables|Default|SetTimer_RuneActivation _returnvalue))))

(event Custom|OnFinishAcquirePowerRune
  (Actor|DestroyActor))

(event EventInteract
  ;[1 0 0.9837 1 50] Interfaces
  ;;[1 1 1] Interact
  (CallFunction|OnActivation))

(event EventActivate
  ;[1 0 0.9837 1 50] Interfaces
  ;;[1 1 1] Activate
  (Collision|SetCollisionEnabled (Variables|Default|GetSphere) "QueryOnly"))

(fn ConstructionScript)