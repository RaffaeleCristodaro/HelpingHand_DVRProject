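; BP_RuneModeSphereTutorial is a VR grabbable sphere that starts the rune mode tutorial and unlocks the player's first power-up.
; On grab, a one-time activation hides the sphere, disables its collision, flags the pawn's tutorial and saves the unlock.
; It then force-releases the grab and clears that hand's references.
; A separate event, not triggered here, plays PG3's power-acquisition montage and clears its surprised state.
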(event OnGrabbed(GrabComponent)
  ;[1 1 1] On Grabbed
  (CallFunction|OnActivation))

(event Custom|TutorialAnimationFirstTimeRuneFire
  ;[1 1 1] Tutorial anim
  (bind _returnvalue (Animation|PlayAnimMontage (Variables|References|GetRef_PG3) "/Game/PG3/PG3_Animations/AM_PG3_AcquisitionPower.AM_PG3_AcquisitionPower" 1.0 "None"))
  (Utilities|FlowControl|Delay _returnvalue)
  (Animation|StopAnimMontage (Variables|References|GetRef_PG3) "/Game/PG3/PG3_Animations/AM_PG3_AcquisitionPower.AM_PG3_AcquisitionPower")
  (Variables|/Game/PG3/BP_PG3.BP_PG3_C|SetIsSurprised? (Variables|References|GetRef_PG3) false))

(event Custom|OnActivation
  (bind _ref_gameinstance (Variables|References|GetRef_GameInstance))
  (bind _ref_vrpawn (Variables|References|GetRef_VRPawn))
  (bind _ref_vrpawn_2 (Variables|References|GetRef_VRPawn))
  (bind _currentsave (Default|GetCurrentSave _ref_gameinstance))
  ;[1 1 1] On Activation
  (Utilities|FlowControl|DoOnce false
    (:Completed
      (Development|SetHiddeninGame (Variables|Default|GetSphere) true false)
      (Collision|SetCollisionEnabled (Variables|Default|GetSphere) "NoCollision")
      (Variables|/Game/Characters/VRPawn.VRPawn_C|SetIsRuneModeTutorial? (Variables|References|GetRef_VRPawn) true)
      (Variables|/Game/Managers/SG_HelpingHand.SG_HelpingHand_C|SetHasPlayerUnclokedFirstPowerUp? _currentsave true)
      (SaveGame|SaveGametoSlot _currentsave "Save_HelpingHand")
      (if (== (Variables|/Game/Characters/VRPawn.VRPawn_C|GetHeldComponentLeft (Variables|References|GetRef_VRPawn)) (Variables|Default|GetGrabComponent))
        (Default|TryRelease (Variables|Default|GetGrabComponent))
        (Variables|/Game/Characters/VRPawn.VRPawn_C|SetHeldComponentLeft (Variables|References|GetRef_VRPawn) 0)
        (Utilities|IsValid (Variables|/Game/Characters/VRPawn.VRPawn_C|GetHit%20ActorLeft _ref_vrpawn_2)
          (:Is%20Valid
            (Variables|/Game/Characters/VRPawn.VRPawn_C|SetHit%20ActorLeft _ref_vrpawn_2 0)))
        (else
          (Default|TryRelease (Variables|Default|GetGrabComponent))
          (Variables|/Game/Characters/VRPawn.VRPawn_C|SetHeldComponentRight (Variables|References|GetRef_VRPawn) 0)
          (Utilities|IsValid (Variables|/Game/Characters/VRPawn.VRPawn_C|GetTelekinesis_CurrentActor_Right _ref_vrpawn)
            (:Is%20Valid
              (Variables|/Game/Characters/VRPawn.VRPawn_C|SetTelekinesis_CurrentActor_Right _ref_vrpawn 0))))))))

(event EventBeginPlay
  (bind _sphere (Variables|Default|GetSphere))
  ;[1 0.06979 0.06979 1 50] Begin Play
  (bind _gameinstance (Class|BPIGameInstance|GetGameInstanceRef(Message) (Game|GetGameInstance)))
  (Variables|References|SetRef_GameInstance _gameinstance)
  (bind _gamemoderef (Class|BPIGameMode|GetGameModeRef(Message) (Game|GetGameMode)))
  (bind _output_get (Variables|References|SetRef_GameMode _gamemoderef))
  (Variables|References|SetRef_PG3 (Default|GetPG3Ref _output_get))
  (Variables|References|SetRef_VRPawn (Default|GetVRPawnRef _output_get))
  (Variables|Default|SetIntialScale (Transformation|GetWorldScale (Variables|Default|GetSphere)))
  (Variables|Default|SetActorStartLocation (Transformation|GetActorLocation))
  (Variables|Default|SetActorStartRotation (Transformation|GetActorRotation))
  (Variables|Default|SetSphereStartLocation (Transformation|GetWorldLocation _sphere))
  (Variables|Default|SetSphereStartRotation (Transformation|GetWorldRotation _sphere)))

(fn ConstructionScript)