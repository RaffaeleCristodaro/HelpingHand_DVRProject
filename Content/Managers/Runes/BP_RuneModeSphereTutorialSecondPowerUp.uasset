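; Rune sphere pickup that unlocks the player's second power-up during the tutorial.
; A direct grab or telekinesis grab fires once, hiding the sphere, disabling its collision, activating Niagara and saving the unlock flag.
; It then forces a release and clears player 1's held and target references for that hand.
; A separate event plays player 3's rune-obtained montage, then clears their surprised state.
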(event OnGrabbed(GrabComponent)
  (bind _pg1 (Variables|Default|GetPG1))
  (bind _pg1_2 (Variables|Default|GetPG1))
  (bind _ref_gameinstance (Variables|Default|GetRef_GameInstance))
  (bind _currentsave (Default|GetCurrentSave _ref_gameinstance))
  ;[1 1 1] On Grabbed
  (Utilities|FlowControl|DoOnce false
    (:Completed
      (Development|SetHiddeninGame (Variables|Default|GetSphere) true false)
      (Collision|SetCollisionEnabled (Variables|Default|GetSphere) "NoCollision")
      (Components|Activation|Activate (Variables|Default|GetNiagaraSpawnRune) false)
      (Variables|/Game/Managers/SG_HelpingHand.SG_HelpingHand_C|SetHasPlayerUnclokedSecondPowerUp? _currentsave true)
      (SaveGame|SaveGametoSlot _currentsave "Save_HelpingHand")
      (if (== (Variables|/Game/Characters/VRPawn.VRPawn_C|GetHeldComponentLeft (Variables|Default|GetPG1)) (Variables|Default|GetGrabComponent))
        (Default|TryRelease (Variables|Default|GetGrabComponent))
        (Variables|/Game/Characters/VRPawn.VRPawn_C|SetHeldComponentLeft (Variables|Default|GetPG1) 0)
        (Utilities|IsValid (Variables|/Game/Characters/VRPawn.VRPawn_C|GetHit%20ActorLeft _pg1)
          (:Is%20Valid
            (Variables|/Game/Characters/VRPawn.VRPawn_C|SetHit%20ActorLeft _pg1 0)))
        (else
          (Default|TryRelease (Variables|Default|GetGrabComponent))
          (Variables|/Game/Characters/VRPawn.VRPawn_C|SetHeldComponentRight (Variables|Default|GetPG1) 0)
          (Utilities|IsValid (Variables|/Game/Characters/VRPawn.VRPawn_C|GetTelekinesis_CurrentActor_Right _pg1_2)
            (:Is%20Valid
              (Variables|/Game/Characters/VRPawn.VRPawn_C|SetTelekinesis_CurrentActor_Right _pg1_2 0))))))))

(event Custom|TutorialAnimationFirstTimeRuneStrenght
  ;[1 1 1] Tutorial anim
  (bind _returnvalue (Animation|PlayAnimMontage (Variables|Default|GetPG3) "/Game/PG3/PG3_Animations/PG_Ottiene_Runa_AnimMontage.PG_Ottiene_Runa_AnimMontage" 1.0 "None"))
  (Utilities|FlowControl|Delay _returnvalue)
  (Animation|StopAnimMontage (Variables|Default|GetPG3) "/Game/PG3/PG3_Animations/PG_Ottiene_Runa_AnimMontage.PG_Ottiene_Runa_AnimMontage")
  (Variables|/Game/PG3/BP_PG3.BP_PG3_C|SetIsSurprised? (Variables|Default|GetPG3) false))

(event Custom|TelekynesisGrab
  (bind _pg1 (Variables|Default|GetPG1))
  (bind _pg1_2 (Variables|Default|GetPG1))
  (bind _ref_gameinstance (Variables|Default|GetRef_GameInstance))
  (bind _currentsave (Default|GetCurrentSave _ref_gameinstance))
  ;[1 1 1] On Grabbed
  (Utilities|FlowControl|DoOnce false
    (:Completed
      (Development|SetHiddeninGame (Variables|Default|GetSphere) true false)
      (Collision|SetCollisionEnabled (Variables|Default|GetSphere) "NoCollision")
      (Components|Activation|Activate (Variables|Default|GetNiagaraSpawnRune) false)
      (Variables|/Game/Managers/SG_HelpingHand.SG_HelpingHand_C|SetHasPlayerUnclokedSecondPowerUp? _currentsave true)
      (SaveGame|SaveGametoSlot _currentsave "Save_HelpingHand")
      (if (== (Variables|/Game/Characters/VRPawn.VRPawn_C|GetHeldComponentLeft (Variables|Default|GetPG1)) (Variables|Default|GetGrabComponent))
        (Default|TryRelease (Variables|Default|GetGrabComponent))
        (Variables|/Game/Characters/VRPawn.VRPawn_C|SetHeldComponentLeft (Variables|Default|GetPG1) 0)
        (Utilities|IsValid (Variables|/Game/Characters/VRPawn.VRPawn_C|GetHit%20ActorLeft _pg1)
          (:Is%20Valid
            (Variables|/Game/Characters/VRPawn.VRPawn_C|SetHit%20ActorLeft _pg1 0)))
        (else
          (Default|TryRelease (Variables|Default|GetGrabComponent))
          (Variables|/Game/Characters/VRPawn.VRPawn_C|SetHeldComponentRight (Variables|Default|GetPG1) 0)
          (Utilities|IsValid (Variables|/Game/Characters/VRPawn.VRPawn_C|GetTelekinesis_CurrentActor_Right _pg1_2)
            (:Is%20Valid
              (Variables|/Game/Characters/VRPawn.VRPawn_C|SetTelekinesis_CurrentActor_Right _pg1_2 0))))))))

(event EventBeginPlay
  (bind _sphere (Variables|Default|GetSphere))
  ;[1 1 1] Initialize
  (bind _gameinstance (Class|BPIGameInstance|GetGameInstanceRef(Message) (Game|GetGameInstance)))
  (Variables|Default|SetRef_GameInstance _gameinstance)
  (bind _pg1 (CallFunction|GetPlayer1))
  (Variables|Default|SetPG1 _pg1)
  (bind _pg3 (CallFunction|GetPlayer3))
  (Variables|Default|SetPG3 _pg3)
  (Variables|Default|SetIntialScale (Transformation|GetWorldScale (Variables|Default|GetSphere)))
  (Variables|Default|SetActorStartLocation (Transformation|GetActorLocation))
  (Variables|Default|SetActorStartRotation (Transformation|GetActorRotation))
  (Variables|Default|SetSphereStartLocation (Transformation|GetWorldLocation _sphere))
  (Variables|Default|SetSphereStartRotation (Transformation|GetWorldRotation _sphere)))

(fn ConstructionScript)