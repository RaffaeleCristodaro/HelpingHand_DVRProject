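; BP_CullingBlueprint is a box-trigger culling volume that toggles the visibility of a list of actors as the VR pawn enters or leaves.
; Entering unhides every valid actor in BPToMakeInvisibles, and leaving hides them again.
; On exit, grabbables stay visible if held, matching player 1's left or right hit actor, or still overlapping the box.
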(event OnComponentBeginOverlap(Box)
  (params (OverlappedComponent :type Primitive%20Component%20Object%20Reference) (OtherActor :type Actor%20Object%20Reference) (OtherComp :type Primitive%20Component%20Object%20Reference) (OtherBodyIndex :type Integer) (bFromSweep :type Boolean) (SweepResult :type Hit%20Result%20Structure%20%28by%20ref%29))
  ;[1 1 1] Overlap with PG1
  (Utilities|Casting|CastToVRPawn OtherActor)
  (for _array_element (Variables|Default|GetBPToMakeInvisibles)
    (Utilities|IsValid _array_element
      (:Is%20Valid
        (Rendering|SetActorHiddenInGame _array_element false)))))

(event OnComponentEndOverlap(Box)
  (params (OverlappedComponent :type Primitive%20Component%20Object%20Reference) (OtherActor :type Actor%20Object%20Reference) (OtherComp :type Primitive%20Component%20Object%20Reference) (OtherBodyIndex :type Integer))
  (bind _pg1 (Variables|Default|GetPG1))
  ;[1 1 1] Overlap with PG1
  (Utilities|Casting|CastToVRPawn OtherActor)
  (for _array_element (Variables|Default|GetBPToMakeInvisibles)
    (Utilities|IsValid _array_element
      (:Is%20Valid
        (bind _asbp_interactive_grabbables_parent (Utilities|Casting|CastToBP_InteractiveGrabbablesParent _array_element)
          (:then
            (if (not (Variables|/Game/VRTemplate/Blueprints/GrabComponent.GrabComponent_C|GetbIsHeld (Variables|/Game/Blueprint_Grabbable/BP_InteractiveGrabbablesParent.BP_InteractiveGrabbablesParent_C|GetGrabComponent _asbp_interactive_grabbables_parent)))
              (if (not (or (== _array_element (Variables|/Game/VRTemplate/Blueprints/VRPawn.VRPawn_C|GetHit%20ActorRight _pg1)) (== _array_element (Variables|/Game/VRTemplate/Blueprints/VRPawn.VRPawn_C|GetHit%20ActorLeft _pg1))))
                (if (not (Collision|IsOverlappingActor (Variables|Default|GetBox) _array_element :!class /Script/Engine.PrimitiveComponent))
                  (Rendering|SetActorHiddenInGame _array_element true)))))
          (:CastFailed
            (Rendering|SetActorHiddenInGame _array_element true)))))))

(event EventBeginPlay
  ;[1 1 1] Initialize
  (bind _pg1 (CallFunction|GetPlayer1))
  (Variables|Default|SetPG1 _pg1))

(fn ConstructionScript)