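; Level-change trigger volume that sends the game to a configurable level when the PG3 character enters its box.
; BeginPlay caches the game mode, VR pawn, PG3 and game instance references, mostly through getters on the game mode.
; The first overlap by an actor implementing BPI_PG3 calls Death on the cached PG3, then has the game mode change level after a configurable delay.
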(event OnComponentBeginOverlap(Box)
  (params (OverlappedComponent :type Primitive%20Component%20Object%20Reference) (OtherActor :type Actor%20Object%20Reference) (OtherComp :type Primitive%20Component%20Object%20Reference) (OtherBodyIndex :type Integer) (bFromSweep :type Boolean) (SweepResult :type Hit%20Result%20Structure%20%28by%20ref%29))
  ;[0 0.739 1 1 50] Overlap
  ;;[1 1 1] Begin overlap "Box"
  (if (Utilities|DoesObjectImplementInterface OtherActor "/Game/Managers/BlueprintInterfaces/BPI_PG3.BPI_PG3_C")
    (Utilities|FlowControl|DoOnce false
      (:Completed
        (Default|Death (Variables|References|GetRef_PG3) "NewEnumerator0")
        (Default|ChangeLevelwithDelay (Variables|References|GetRef_GameMode) (Variables|Settings|GetLevel%20to%20Open) (Variables|Settings|GetOpenLevelDelay))))))

(event EventBeginPlay
  ;[1 0.07812 0.07812 1 50] Begin Play
  (bind _gamemoderef (Class|BPIGameMode|GetGameModeRef(Message) (Game|GetGameMode)))
  (bind _output_get (Variables|References|SetRef_GameMode _gamemoderef))
  (Variables|References|SetRef_VRPawn (Default|GetVRPawnRef _output_get))
  (Variables|References|SetRef_PG3 (Default|GetPG3Ref (Variables|References|GetRef_GameMode)))
  (bind _gameinstance (Class|BPIGameInstance|GetGameInstanceRef(Message) (Game|GetGameInstance)))
  (Variables|References|SetRef_GameInstance _gameinstance))

(fn ConstructionScript)