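; Level-change trigger for the Surreal Zone that sends the game to a configured level when an actor implementing BPI_PG3 enters its box.
; On BeginPlay, a GameInstance flag marking PG1's return from that zone is cleared and sets CanChangeArea to false, blocking the trigger.
; A valid overlap fires once, calling Death on PG3, activating Niagara and asking the GameMode for a delayed level change.
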(event OnComponentBeginOverlap(Box)
  (params (OverlappedComponent :type Primitive%20Component%20Object%20Reference) (OtherActor :type Actor%20Object%20Reference) (OtherComp :type Primitive%20Component%20Object%20Reference) (OtherBodyIndex :type Integer) (bFromSweep :type Boolean) (SweepResult :type Hit%20Result%20Structure%20%28by%20ref%29))
  ;[0 0.6419 1 1 50] Overlap
  ;;[1 1 1] Begin overlap "Box"
  (if (and (Utilities|DoesObjectImplementInterface OtherActor "/Game/Managers/BlueprintInterfaces/BPI_PG3.BPI_PG3_C") (Variables|Default|GetCanChangeArea?))
    (Utilities|FlowControl|DoOnce false
      (:Completed
        (Default|Death (Variables|Default|GetRef_PG3) "NewEnumerator3")
        (Components|Activation|Activate (Variables|Default|GetNiagara) false)
        (Default|ChangeLevelwithDelay (Variables|Default|GetRef_GameMode) (Variables|Default|GetLevel%20to%20Open) (Variables|Default|GetOpenLevelDelay))))))

(event EventBeginPlay
  ;[1 0.05729 0.05729 1 50] Begin Play
  (|CallParentFunction)
  (if (Variables|/Game/Managers/GI_HelpingHand.GI_HelpingHand_C|GetIsPG1ReturnedFromZonaSurreale? (Variables|Default|GetRef_GameInstance))
    (Variables|/Game/Managers/GI_HelpingHand.GI_HelpingHand_C|SetIsPG1ReturnedFromZonaSurreale? (Variables|Default|GetRef_GameInstance) false)
    (Variables|Default|SetCanChangeArea? false)))

(fn ConstructionScript
  (|CallParentFunction))