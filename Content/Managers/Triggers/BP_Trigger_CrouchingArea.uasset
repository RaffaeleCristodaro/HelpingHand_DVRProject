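; Trigger volume that makes the player character (PG3) crouch while inside its box.
; On BeginPlay it gets the game mode reference through an interface message and caches the PG3 reference from it.
; Box begin and end overlaps check that the other actor implements BPI_PG3, then call StartCrouching or StopCrouching on the cached PG3 rather than on the overlapping actor.
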(event OnComponentBeginOverlap(Box)
  (params (OverlappedComponent :type Primitive%20Component%20Object%20Reference) (OtherActor :type Actor%20Object%20Reference) (OtherComp :type Primitive%20Component%20Object%20Reference) (OtherBodyIndex :type Integer) (bFromSweep :type Boolean) (SweepResult :type Hit%20Result%20Structure%20%28by%20ref%29))
  ;[0 0.7082 1 1 50] Overlap
  ;;[1 1 1] On begin overlap
  (if (Utilities|DoesObjectImplementInterface OtherActor "/Game/Managers/BlueprintInterfaces/BPI_PG3.BPI_PG3_C")
    (Default|StartCrouching (Variables|Default|GetRef_PG3))))

(event OnComponentEndOverlap(Box)
  (params (OverlappedComponent :type Primitive%20Component%20Object%20Reference) (OtherActor :type Actor%20Object%20Reference) (OtherComp :type Primitive%20Component%20Object%20Reference) (OtherBodyIndex :type Integer))
  ;[0 0.7082 1 1 50] Overlap
  ;;[1 1 1] On end overlap
  (if (Utilities|DoesObjectImplementInterface OtherActor "/Game/Managers/BlueprintInterfaces/BPI_PG3.BPI_PG3_C")
    (Default|StopCrouching (Variables|Default|GetRef_PG3))))

(event EventBeginPlay
  ;[1 0.09479 0.09479 1 50] Begin Play
  (bind _gamemoderef (Class|BPIGameMode|GetGameModeRef(Message) (Game|GetGameMode)))
  (bind _output_get (Variables|Default|SetRef_GameMode _gamemoderef))
  (Variables|Default|SetRef_PG3 (Default|GetPG3Ref _output_get)))

(fn ConstructionScript)