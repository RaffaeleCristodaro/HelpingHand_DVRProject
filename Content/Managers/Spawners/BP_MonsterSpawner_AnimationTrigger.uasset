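; Trigger volume that makes a referenced PhysicMonster grab the third player character (PG3) while that character is inside its box.
; BeginPlay caches PG3, and the box overlap events react only to that actor.
; Entering copies SetMonsterGrabLocation into the monster's GrabPositionAnim and calls GrabPG3, while leaving stops the grab and zeroes that position.
; Despite the spawner name, the graph spawns nothing.
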(event OnComponentBeginOverlap(Box)
  (params (OverlappedComponent :type Primitive%20Component%20Object%20Reference) (OtherActor :type Actor%20Object%20Reference) (OtherComp :type Primitive%20Component%20Object%20Reference) (OtherBodyIndex :type Integer) (bFromSweep :type Boolean) (SweepResult :type Hit%20Result%20Structure%20%28by%20ref%29))
  (bind _physicmonster (Variables|Default|GetPhysicMonster))
  ;[1 1 1] Overlap with PG3
  (if (== OtherActor (Variables|Default|GetPG3))
    (Variables|/Game/Enemies/EnemyPhisyc/BP_PhysicMonster.BP_PhysicMonster_C|SetGrabPositionAnim _physicmonster (Variables|Default|GetSetMonsterGrabLocation))
    (Default|GrabPG3 _physicmonster "0, 0, 0")))

(event OnComponentEndOverlap(Box)
  (params (OverlappedComponent :type Primitive%20Component%20Object%20Reference) (OtherActor :type Actor%20Object%20Reference) (OtherComp :type Primitive%20Component%20Object%20Reference) (OtherBodyIndex :type Integer))
  (bind _physicmonster (Variables|Default|GetPhysicMonster))
  ;[1 1 1] Overlap with PG3
  (if (== OtherActor (Variables|Default|GetPG3))
    (Default|StopGrabPG3 _physicmonster)
    (Variables|/Game/Enemies/EnemyPhisyc/BP_PhysicMonster.BP_PhysicMonster_C|SetGrabPositionAnim _physicmonster "0, 0, 0")))

(event EventBeginPlay
  ;[1 1 1] Intialize
  (bind _pg3 (CallFunction|GetPlayer3))
  (Variables|Default|SetPG3 _pg3))

(fn ConstructionScript)