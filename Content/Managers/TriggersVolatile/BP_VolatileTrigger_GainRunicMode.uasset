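; One-shot volatile trigger, named for gaining Runic Mode, that reveals a rune when the VR pawn enters its box.
; On the first overlap by a BPI_VRPawn actor, it waits a delay, disables box collision and makes the SingleRune visible.
; A RunePopUp timeline lerps the rune to the EndRuneLocation component's position.
; When the timeline finishes, the rune's message and a Niagara spawn-sphere effect activate.
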(event OnComponentBeginOverlap(Box)
  (params (OverlappedComponent :type Primitive%20Component%20Object%20Reference) (OtherActor :type Actor%20Object%20Reference) (OtherComp :type Primitive%20Component%20Object%20Reference) (OtherBodyIndex :type Integer) (bFromSweep :type Boolean) (SweepResult :type Hit%20Result%20Structure%20%28by%20ref%29))
  ;[1 1 1] Overlap Box
  (if (Utilities|DoesObjectImplementInterface OtherActor "/Game/Managers/BlueprintInterfaces/BPI_VRPawn.BPI_VRPawn_C")
    (Utilities|FlowControl|DoOnce false
      (:Completed
        (Utilities|FlowControl|Delay (Variables|Settings|GetDelay))
        (Collision|SetCollisionEnabled (Variables|Default|GetBox) "NoCollision")
        (Rendering|SetVisibility (Variables|/Script/Engine.Actor|GetRootComponent (Variables|Settings|GetSingleRune)) true false)
        (Variables|Default|SetStartRuneLocation (Transformation|GetActorLocation (Variables|Settings|GetSingleRune)))
        (bind _anim (Timeline|RunePopUp PlayFromStart)
          (:Update
            (Transformation|SetActorLocation (Variables|Settings|GetSingleRune) (Math|Vector|Lerp(Vector) (Variables|Default|GetStartRuneLocation) (Transformation|GetWorldLocation (Variables|Default|GetEndRuneLocation)) _anim) false false))
          (:Finished
            (CallFunction|OnFinishPopUp)))))))

(event Custom|OnFinishPopUp
  ;[1 1 1] On Finish Popup
  (Class|BPITutorialRunes|Activate(Message) (Variables|Settings|GetSingleRune))
  (Components|Activation|Activate (Variables|Default|GetNiagaraSpawnSphere) false))

(fn ConstructionScript
  (|CallParentFunction))