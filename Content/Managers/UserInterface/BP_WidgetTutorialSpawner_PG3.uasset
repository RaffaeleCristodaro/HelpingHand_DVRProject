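; Actor that displays the PG3 tutorial widget in the world, floating above the PG3 character.
; A looping timer started on BeginPlay moves it to a height offset over PG3 and turns it toward the VR pawn's camera.
; SwitchTutorialType shows the selected panel and swaps player controller move and jump event bindings to match.
; A separate event hides the actor after a short delay.
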(event Custom|DeactivatePG3TutorialWidget
  ;[1 1 1] Deactivate Tutorial Widget
  (Utilities|FlowControl|Delay 1.0)
  (Rendering|SetActorHiddenInGame true))

(event Custom|GetWidgetTutorial
  ;[1 1 1] Get widget
  (bind _aswbp_widget_tutorial_pg3 (Utilities|Casting|CastToWBP_WidgetTutorial_PG3 (UserInterface|GetWidget (Variables|Default|GetWidget))))
  (Variables|Default|SetRef_Widget _aswbp_widget_tutorial_pg3))

(event Custom|SwitchTutorialType
  (params (Index :type Integer))
  (bind _controllerref (CallFunction|GetPlayerController))
  (bind _controllerref_2 (CallFunction|GetPlayerController))
  ;[1 1 1] SwitchTutorial Panel
  (Rendering|SetActorHiddenInGame false)
  (Default|SwitchTutorial (Variables|Default|GetRef_Widget) Index)
  (switch int Index
    (:0
      (EventDispatchers|UnbindEventfromOnJumpStarted _controllerref_2 (EventDispatchers|CreateEvent :!event Custom|DeactivatePG3TutorialWidget))
      (EventDispatchers|AssignOnMoveStarted _controllerref_2 (EventDispatchers|CreateEvent :!event Custom|DeactivatePG3TutorialWidget)))
    (:1
      (EventDispatchers|UnbindEventfromOnMoveStarted _controllerref (EventDispatchers|CreateEvent :!event Custom|DeactivatePG3TutorialWidget))
      (EventDispatchers|AssignOnJumpStarted _controllerref (EventDispatchers|CreateEvent :!event Custom|DeactivatePG3TutorialWidget)))))

(event Custom|FollowPG3
  ;[1 1 1] Follow PG3
  (bind _output_get (Variables|Components|SetCurrentLocation (+ (Transformation|GetActorLocation (Variables|Components|GetRef_PG3)) (Math|Vector|MakeVector 0.0 0.0 (Variables|Settings|GetHightOffset)))))
  (Transformation|SetActorLocation _output_get false false)
  (Transformation|SetActorRotation (Math|Rotator|FindLookatRotation (Variables|Components|GetCurrentLocation) (Transformation|GetWorldLocation (Variables|Default|GetRef_VRPawnCamera)))))

(event EventBeginPlay
  ;[1 0.06979 0.06979 1 50] Begin Play
  (CallFunction|GetWidgetTutorial)
  (bind _gamemoderef (Class|BPIGameMode|GetGameModeRef(Message) (Game|GetGameMode)))
  (Variables|Components|SetRef_PG3 (Default|GetPG3Ref _gamemoderef))
  (Variables|Default|SetRef_VRPawnCamera (Variables|/Game/Characters/VRPawn.VRPawn_C|GetCamera (Default|GetVRPawnRef _gamemoderef)))
  (bind _returnvalue (Utilities|Time|SetTimerbyEvent (delegate Custom|FollowPG3) 0.01 true))
  (Variables|Components|SetFollowPG3_TimerHandler _returnvalue))

(fn ConstructionScript)