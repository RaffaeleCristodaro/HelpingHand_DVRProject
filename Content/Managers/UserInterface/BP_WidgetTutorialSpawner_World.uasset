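; BP_WidgetTutorialSpawner_World is an actor that displays a world tutorial panel through its widget component.
; It caches the WBP_WidgetTutorial_World instance and passes it CurrentTutorialPanel to select the panel, both in the construction script and at BeginPlay.
; The panel is hidden at BeginPlay, and activate and deactivate events toggle the component's visibility without propagating to children.
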(event Custom|ActivateTutorialPanel
  ;[1 1 1] Activate Tutorial Panel
  (Rendering|SetVisibility (Variables|Default|GetWidget) true false))

(event Custom|GetWidget
  ;[1 1 1] Get Widget
  (bind _aswbp_widget_tutorial_world (Utilities|Casting|CastToWBP_WidgetTutorial_World (UserInterface|GetWidget (Variables|Default|GetWidget))))
  (Variables|Default|SetWidgetTutorial _aswbp_widget_tutorial_world))

(event Custom|DeactivateTutorialPanel
  ;[1 1 1] Deactivate Panel
  (Rendering|SetVisibility (Variables|Default|GetWidget) false false))

(event EventBeginPlay
  ;[1 0.08229 0.08229 1 50] Begin Play
  (CallFunction|GetWidget)
  (CallFunction|DeactivateTutorialPanel)
  (Default|UpdateCurrentIndex (Variables|Default|GetWidgetTutorial) (Variables|Settings|GetCurrentTutorialPanel)))

(fn ConstructionScript
  (CallFunction|GetWidget)
  (Default|UpdateCurrentIndex (Variables|Default|GetWidgetTutorial) (Variables|Settings|GetCurrentTutorialPanel)))