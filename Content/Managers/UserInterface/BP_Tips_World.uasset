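; BP_Tips_World is a world-space tips widget Blueprint that keeps its Widget component turned toward the VR player.
; Every Tick it runs WidgetLookAtPlayer, which sets the widget's world rotation with FindLookAtRotation toward the VR pawn's camera.
; The pawn reference comes from the Game Mode through GetVRPawnRef.
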(event EventTick
  (params (DeltaSeconds :type Float%20%28single-precision%29))
  ;[1 1 1] Event tick
  (CallFunction|WidgetLookatPlayer))

(fn ConstructionScript)

(fn WidgetLookatPlayer
  (Transformation|SetWorldRotation (Variables|Default|GetWidget) (Math|Rotator|FindLookatRotation (Transformation|GetWorldLocation (Variables|Default|GetWidget)) (Transformation|GetWorldLocation (Variables|/Game/Characters/VRPawn.VRPawn_C|GetCamera (Default|GetVRPawnRef (CallFunction|GetGameMode))))) false false))