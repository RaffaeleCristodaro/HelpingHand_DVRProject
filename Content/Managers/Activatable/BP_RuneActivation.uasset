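; Activatable manager that reveals a single rune with a pop-up animation when activated, firing only once.
; After a delay it makes the rune visible and a timeline lerps it from its current position to the EndRuneLocation component.
; When the pop-up finishes, it triggers the rune's message and a Niagara effect, then yaws the game mode's PG3 character toward the end location and plays its look-at-rune montage.
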(event Custom|OnFinishPopUp
  ;[1 1 1] On Finish Popup
  (Class|BPIRune|Activate(Message) (Variables|Settings|GetSingleRune))
  (Components|Activation|Activate (Variables|Default|GetNiagaraSpawnSphere) false)
  (Transformation|SetActorRotation (Default|GetPG3Ref (CallFunction|GetGameMode)) (Math|Rotator|MakeRotator 0.0 0.0 (.yaw (Math|Rotator|FindLookatRotation (Transformation|GetActorLocation (Default|GetPG3Ref (CallFunction|GetGameMode))) (Transformation|GetWorldLocation (Variables|Default|GetEndRuneLocation))))))
  (Animation|PlayAnimMontage (Default|GetPG3Ref (CallFunction|GetGameMode)) "/Game/PG3/PG3_Animations/AM_PG3_LookRune.AM_PG3_LookRune" 1.0 "None"))

(event EventActivate
  ;[1 1 1] Activate
  (Utilities|FlowControl|DoOnce false
    (:Completed
      (Utilities|FlowControl|Delay (Variables|Settings|GetDelay))
      (Rendering|SetVisibility (Variables|/Script/Engine.Actor|GetRootComponent (Variables|Settings|GetSingleRune)) true false)
      (Variables|Default|SetStartRuneLocation (Transformation|GetActorLocation (Variables|Settings|GetSingleRune)))
      (bind _anim (Timeline|RunePopUp PlayFromStart)
        (:Update
          (Transformation|SetActorLocation (Variables|Settings|GetSingleRune) (Math|Vector|Lerp(Vector) (Variables|Default|GetStartRuneLocation) (Transformation|GetWorldLocation (Variables|Default|GetEndRuneLocation)) _anim) false false))
        (:Finished
          (CallFunction|OnFinishPopUp))))))

(fn ConstructionScript)