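; Breakable plate actor built on a Geometry Collection that the player can grab with either hand and shatter.
; Once the player overlaps its Box, Tick teleports the plate to the pressed grab hand's sphere, left taking priority.
; On release it either enables physics and collision or clears the player's telekinesis reference.
; A Chaos break event stops the follow logic, disables plate telekinesis and destroys the Cube and Box components.
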(event OnChaosBreakEvent(GeometryCollection)
  (params (BreakEvent :type Chaos%20Break%20Event%20Structure%20%28by%20ref%29))
  (bind _cube (Variables|Default|GetCube))
  (bind _box (Variables|Default|GetBox))
  ;[1 1 1] Break event
  (Variables|/Game/VRTemplate/Blueprints/VRPawn.VRPawn_C|SetCanTelekynesisPlate? (Variables|Default|GetPG1) false)
  (Variables|Default|SetDestroyCondition true)
  (Utilities|IsValid _cube
    (:Is%20Valid
      (Components|DestroyComponent _cube))
    (:Is%20Not%20Valid
      _))
  (Utilities|IsValid _box
    (:Is%20Valid
      (Components|DestroyComponent _box))))

(event OnComponentBeginOverlap(Box)
  (params (OverlappedComponent :type Primitive%20Component%20Object%20Reference) (OtherActor :type Actor%20Object%20Reference) (OtherComp :type Primitive%20Component%20Object%20Reference) (OtherBodyIndex :type Integer) (bFromSweep :type Boolean) (SweepResult :type Hit%20Result%20Structure%20%28by%20ref%29))
  ;[1 1 1] Comment
  (if (== OtherActor (Variables|Default|GetPG1))
    (Variables|Default|SetCanFollowHand? true)))

(event EventBeginPlay
  ;[1 1 1] Initialize
  (Physics|SetSimulatePhysics (Variables|Default|GetGeometryCollection) false)
  (bind _pg1 (CallFunction|GetPlayer1))
  (Variables|Default|SetPG1 _pg1)
  (Variables|Default|SetInitialScalePiattogeometry (Transformation|GetWorldScale (Variables|Default|GetGeometryCollection))))

(event EventTick
  (params (DeltaSeconds :type Float%20%28single-precision%29))
  (bind _pg1 (Variables|Default|GetPG1))
  (bind _sphereleft (Variables|/Game/VRTemplate/Blueprints/VRPawn.VRPawn_C|GetSphereLeft _pg1))
  (bind _sphereright (Variables|/Game/VRTemplate/Blueprints/VRPawn.VRPawn_C|GetSphereRight _pg1))
  ;[1 1 1] Event tick
  (if (not (Variables|Default|GetDestroyCondition))
    (if (Variables|Default|GetCanFollowHand?)
      (if (Variables|/Game/VRTemplate/Blueprints/VRPawn.VRPawn_C|GetPressGrabLeft _pg1)
        (Transformation|SetWorldLocationAndRotation (Variables|Default|GetGeometryCollection) (Transformation|GetWorldLocation _sphereleft) (Transformation|GetWorldRotation _sphereleft) false true)
        (Variables|Default|SetGrabbedOnce? true :!label _label)
        (Variables|/Game/VRTemplate/Blueprints/VRPawn.VRPawn_C|SetCurrentPiattoGeometryGrabbed (Variables|Default|GetPG1) self)
        (elif (Variables|/Game/VRTemplate/Blueprints/VRPawn.VRPawn_C|GetPressGrabRight _pg1)
          (Transformation|SetWorldLocationAndRotation (Variables|Default|GetGeometryCollection) (Transformation|GetWorldLocation _sphereright) (Transformation|GetWorldRotation _sphereright) false true)
          (goto _label)
          (else
            ;;[0.08854 0.08854 0.08854] Grab release
            (if (Variables|Default|GetGrabbedOnce?)
              (if (== (Variables|/Game/VRTemplate/Blueprints/VRPawn.VRPawn_C|GetCurrentPiattoGeometrytelekynesisGrabbed _pg1) 0)
                (Physics|SetSimulatePhysics (Variables|Default|GetGeometryCollection) true)
                (Collision|SetCollisionEnabled (Variables|Default|GetGeometryCollection) "QueryAndPhysics")
                (else
                  (Variables|/Game/VRTemplate/Blueprints/VRPawn.VRPawn_C|SetCurrentPiattoGeometrytelekynesisGrabbed _pg1 0))))))))))

(fn ConstructionScript)