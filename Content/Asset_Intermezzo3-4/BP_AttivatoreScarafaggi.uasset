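; BP_AttivatoreScarafaggi is a one-shot trigger that releases a cockroach (scarafaggi) effect when Player 3 enters its box.
; The first overlap sets a flag that lets Tick activate the Niagara system once and play an optional sound at high volume.
; Tick also shrinks the Grumetto component at constant speed, then hides it and clears the flag once its scale nears zero.
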(event OnComponentBeginOverlap(Box)
  (params (OverlappedComponent :type Primitive%20Component%20Object%20Reference) (OtherActor :type Actor%20Object%20Reference) (OtherComp :type Primitive%20Component%20Object%20Reference) (OtherBodyIndex :type Integer) (bFromSweep :type Boolean) (SweepResult :type Hit%20Result%20Structure%20%28by%20ref%29))
  ;[1 1 1] Overlap with PG3
  (if (== OtherActor (Variables|Default|GetPG3))
    (Utilities|FlowControl|DoOnce false
      (:Completed
        (Variables|Default|SetCanActivate? true)))))

(event EventBeginPlay
  ;[1 1 1] Initialize
  (bind _pg3 (CallFunction|GetPlayer3))
  (Variables|Default|SetPG3 _pg3))

(event EventTick
  (params (DeltaSeconds :type Float%20%28single-precision%29))
  (bind _grumetto (Variables|Default|GetGrumetto))
  (bind _delta_time (Variables|FadeGrumetto|GetDelta%20Time))
  (bind _interp_speed (Variables|FadeGrumetto|GetInterp%20Speed))
  (bind _soundtoplay (Variables|FadeGrumetto|GetSoundToPlay))
  (bind _returnvalue (Transformation|GetWorldScale _grumetto))
  (bind _returnvalue_2 (Math|Interpolation|VInterptoConstant _returnvalue "0, 0, 0" _delta_time _interp_speed))
  ;[1 1 1] Event tick
  (if (Variables|Default|GetCanActivate?)
    (Utilities|FlowControl|Sequence
      (:then_0
        (Utilities|FlowControl|DoOnce false
          (:Completed
            (Components|Activation|Activate (Variables|Default|GetNiagara_Scarafaggi) false)
            (Utilities|IsValid _soundtoplay
              (:Is%20Valid
                (Audio|PlaySoundatLocation _soundtoplay "0, 0, 0" "0, 0, 0" 1e+02 1.0 0.0 0 0 0 0))))))
      (:then_1
        (Transformation|SetWorldScale3D _grumetto _returnvalue_2)
        (if (Utilities|Operators|EqualEqual :A _returnvalue_2 :ErrorTolerance 0.1)
          (Utilities|FlowControl|DoOnce false
            (:Completed
              (Development|SetHiddeninGame (Variables|Default|GetGrumetto) true false)
              (Variables|Default|SetCanActivate? false))))))))

(fn ConstructionScript)