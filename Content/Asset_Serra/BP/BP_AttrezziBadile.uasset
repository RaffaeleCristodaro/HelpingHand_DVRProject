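; BP_AttrezziBadile is a shovel tool that acts as a catapult, launching the PG3 character when the VR player triggers it.
; A VRPawn entering CollisionPG1 rotates the mesh's pitch through a timeline.
; CollisionPG3 tracks whether PG3 is in the throw zone; if so, PG3 from the GameMode is also launched.
; The IsRestoringBadileRot flag controls whether the finished timeline plays in reverse to restore the rotation.
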(event OnComponentBeginOverlap(CollisionPG1)
  (params (OverlappedComponent :type Primitive%20Component%20Object%20Reference) (OtherActor :type Actor%20Object%20Reference) (OtherComp :type Primitive%20Component%20Object%20Reference) (OtherBodyIndex :type Integer) (bFromSweep :type Boolean) (SweepResult :type Hit%20Result%20Structure%20%28by%20ref%29))
  ;[1 1 1] Collision PG1
  (Utilities|Casting|CastToVRPawn OtherActor)
  (if true
    (if (Variables|Default|GetPG3IsInCollisionToThrow)
      (CallFunction|RotateBadile)
      (Character|LaunchCharacter (Default|GetPG3Ref (CallFunction|GetGameMode)) (Variables|Badile|GetLaunchVelocityPG3FromBadile) false true)
      (else
        (CallFunction|RotateBadile)))))

(event OnComponentBeginOverlap(CollisionPG3)
  (params (OverlappedComponent :type Primitive%20Component%20Object%20Reference) (OtherActor :type Actor%20Object%20Reference) (OtherComp :type Primitive%20Component%20Object%20Reference) (OtherBodyIndex :type Integer) (bFromSweep :type Boolean) (SweepResult :type Hit%20Result%20Structure%20%28by%20ref%29))
  ;[1 1 1] Collision PG3
  (Utilities|Casting|CastToBP_PG3 OtherActor)
  (Variables|Default|SetPG3IsInCollisionToThrow true))

(event OnComponentEndOverlap(CollisionPG3)
  (params (OverlappedComponent :type Primitive%20Component%20Object%20Reference) (OtherActor :type Actor%20Object%20Reference) (OtherComp :type Primitive%20Component%20Object%20Reference) (OtherBodyIndex :type Integer))
  ;[1 1 1] Collision PG3
  (Utilities|Casting|CastToBP_PG3 OtherActor)
  (Variables|Default|SetPG3IsInCollisionToThrow false))

(event Custom|RestoreBadileRotation
  (bind _staticmesh (Variables|Default|GetStaticMesh))
  (bind _relativerotation (Variables|/Script/Engine.SceneComponent|GetRelativeRotation _staticmesh))
  ;[1 1 1] Rotate badile
  (Variables|Badile|SetIsRestoringBadileRot false)
  (bind _rotatebadilerotationy (Timeline|RotateBadileTimeline ReverseFromEnd)
    (:Update
      (Transformation|SetRelativeRotation _staticmesh (Math|Rotator|MakeRotator (.roll _relativerotation) _rotatebadilerotationy (.yaw _relativerotation)) false false))
    (:Finished
      (if (Variables|Badile|GetIsRestoringBadileRot)
        (CallFunction|RestoreBadileRotation)
        (else
          (Variables|Badile|SetIsRestoringBadileRot true))))))

(event Custom|RotateBadile
  (bind _staticmesh (Variables|Default|GetStaticMesh))
  (bind _relativerotation (Variables|/Script/Engine.SceneComponent|GetRelativeRotation _staticmesh))
  ;[1 1 1] Rotate badile
  (bind _rotatebadilerotationy (Timeline|RotateBadileTimeline PlayFromStart)
    (:Update
      (Transformation|SetRelativeRotation _staticmesh (Math|Rotator|MakeRotator (.roll _relativerotation) _rotatebadilerotationy (.yaw _relativerotation)) false false))
    (:Finished
      (if (Variables|Badile|GetIsRestoringBadileRot)
        (CallFunction|RestoreBadileRotation)
        (else
          (Variables|Badile|SetIsRestoringBadileRot true))))))

(fn ConstructionScript)