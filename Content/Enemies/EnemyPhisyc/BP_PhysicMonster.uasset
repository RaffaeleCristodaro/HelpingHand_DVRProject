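; Physical monster enemy character that follows, attacks, grabs and kills the player, with a rare shiny variant.
; Events drive AI states through inverted Blackboard bools, where false marks the active state.
; A velocity check with a short timer switches between following and idle, gating movement sounds.
; Nav-link jumps use projectile-arc launches; despawning can teleport it back to its starting position.
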(event Custom|ResetKillPlayer
  ;[1 1 1] Attack player if is in range
  (Utilities|FlowControl|DoOnce false) ; enters at Reset
)

(event Custom|RespawnMonster
  ;[1 1 1] Respawn Monster
  (CallFunction|SetIsFollowingPlayer)
  (CallFunction|ResetKillPlayer))

(event Custom|GrabPG3
  (params (LocationToGrab :type Vector))
  ;[1 1 1] Special animation
  (Variables|SpecialAnimation|SetGrabPositionAnim LocationToGrab)
  (Variables|SpecialAnimation|SetIsEnemyUsingSpecialAnim? true)
  (CallFunction|SetIsGrabbingPlayer))

(event Custom|AttackPlayer
  ;[1 1 1] Attack player if is in range
  (CallFunction|SetIsAttackingPlayer))

(event Custom|KillPlayer
  ;[1 1 1] Attack player if is in range
  (Utilities|FlowControl|DoOnce false
    (:Completed
      (Variables|CharacterStates|SetIsAttacking? true)
      (Default|LocalPlayerDeath (Variables|References|GetRef_GameMode) "NewEnumerator2"))))

(event Custom|CheckEnemySpeed
  ;[1 1 1] Check enemy speed
  (if (and (not (Variables|CharacterStates|GetIsDespawning?)) (not (Variables|SpecialAnimation|GetIsEnemyUsingSpecialAnim?)))
    (if (<= (Math|Vector|VectorLength (Transformation|GetVelocity)) 0.1)
      (Utilities|FlowControl|DoOnce true :!label _label
        (:Completed
          (Utilities|Time|SetTimerbyEvent (delegate Custom|CheckEnemySpeedTimerEvent) 0.05)))
      (elif (not (Variables|CharacterStates|GetIsJumping?))
        (CallFunction|SetIsFollowingPlayer)
        (Utilities|FlowControl|Sequence
          (:then_0
            (Utilities|FlowControl|DoOnce false
              (:Completed
                (Audio|PlaySoundatLocation 0 (Transformation|GetWorldLocation (Variables|Character|GetMesh)) "0, 0, 0" 1.0 1.0 0.0 0 0 0 0))))
          (:then_1
            (goto _label Reset)))))))

(event Custom|CheckEnemySpeedTimerEvent
  ;[1 1 1] Check enemy speed
  (if (<= (Math|Vector|VectorLength (Transformation|GetVelocity)) 0.1)
    (CallFunction|SetIsinIdle)
    (CallFunction|RestoreSnarl)
    (Utilities|FlowControl|DoOnce true) ; enters at Reset
    (else
      (CallFunction|SetIsFollowingPlayer)
      (Utilities|FlowControl|Sequence
        (:then_0
          (Utilities|FlowControl|DoOnce false
            (:Completed
              (Audio|PlaySoundatLocation 0 (Transformation|GetWorldLocation (Variables|Character|GetMesh)) "0, 0, 0" 1.0 1.0 0.0 0 0 0 0))))
        (:then_1
          (Utilities|FlowControl|DoOnce true) ; enters at Reset
        )))))

(event Custom|RestoreSnarl
  ;[1 1 1] Check enemy speed
  (Utilities|FlowControl|Sequence
    (:then_0
      (Utilities|FlowControl|DoOnce false) ; enters at Reset
    )
    (:then_1
      (Utilities|FlowControl|DoOnce false) ; enters at Reset
    )))

(event Custom|DespawnMonster
  ;[1 1 1] Despawn monster
  (CallFunction|SetIsDespawning)
  (Variables|CharacterStates|SetIsDespawning? true)
  (Variables|CharacterStates|SetIsAttacking? false))

(event Custom|SetDespawnMonsterLocation
  ;[1 1 1] Despawn monster
  (Transformation|SetActorLocation self (Variables|Settings|GetMosterStartingPos) false true)
  (Utilities|FlowControl|Delay 0.1)
  (CallFunction|SetIsFollowingPlayer)
  (Variables|CharacterStates|SetIsDespawning? false))

(event Custom|StopGrabPG3
  ;[1 1 1] Special animation
  (Variables|SpecialAnimation|SetGrabPositionAnim "0, 0, 0")
  (Variables|SpecialAnimation|SetIsEnemyUsingSpecialAnim? false)
  (CallFunction|SetIsFollowingPlayer)
  (Variables|SpecialAnimation|SetIsTryingToGrabPlayer? false))

(event EventTick
  (params (DeltaSeconds :type Float%20%28single-precision%29))
  ;[1 1 1] Update
  (CallFunction|CheckEnemySpeed))

(event EventNavLinkReached
  (params (Destination :type Vector :default "0, 0, 0") (JumpForce :type Float%20%28double-precision%29) (JumpDuration :type Float%20%28double-precision%29) (AlphaJumpXY :type Float%20%28double-precision%29))
  (bind (_x _y _z) (Math|Vector|BreakVector Destination))
  ;[1 1 1] Nav link reached jump
  (Variables|CharacterStates|SetIsJumping? true)
  (Variables|CalculateVelocityJump|SetJumpForce JumpForce)
  (Variables|CalculateVelocityJump|SetDestination Destination)
  (Variables|CalculateVelocityJump|SetAlpha%20Jump%20XY AlphaJumpXY)
  (CallFunction|SetIsJumping)
  (bind _outlaunchvelocity (Game|SuggestProjectileVelocityCustomArc (Transformation|GetWorldLocation (Variables|Character|GetMesh)) (Math|Vector|MakeVector _x _y (+ _z (Variables|CalculateVelocityJump|GetJumpForce))) 0.0 0.5))
  (Character|LaunchCharacter _outlaunchvelocity false true)
  (Utilities|FlowControl|Delay JumpDuration)
  (CallFunction|SetIsFollowingPlayer)
  (Variables|CharacterStates|SetIsJumping? false))

(event EventBeginPlay
  ;[1 1 1] Initialize
  (Variables|Settings|SetMosterStartingPos (Transformation|GetActorLocation))
  (bind _gamemoderef (Class|BPIGameMode|GetGameModeRef(Message) (Game|GetGameMode)))
  (Variables|References|SetRef_GameMode _gamemoderef)
  (CallFunction|SetIsFollowingPlayer)
  (CallFunction|SetShinyColor))

(fn ConstructionScript)

(fn CalculateVelocity
  (params (DestinationLocation :type Vector) (StartingLocation :type Vector) (Duration :type Float%20%28double-precision%29))
  (bind (_x _y _z) (Math|Vector|BreakVector StartingLocation))
  (bind (_x_2 _y_2 _z_2) (Math|Vector|BreakVector DestinationLocation))
  (Variables|CalculateVelocityJump|SetJumpDuration Duration)
  (return (/ (- _x_2 _x) (Variables|CalculateVelocityJump|GetJumpDuration)) (/ (- _y_2 _y) (Variables|CalculateVelocityJump|GetJumpDuration)) (/ (- _z_2 (+ _z (* (Math|Float|Square (Variables|CalculateVelocityJump|GetJumpDuration)) -0.5 (Variables|CalculateVelocityJump|GetGravity)))) (Variables|CalculateVelocityJump|GetJumpDuration))))

(fn SetIsinIdle
  (Variables|CharacterStates|SetIsFollowingPlayer? false)
  (return))

(fn SetIsFollowingPlayer
  (AI|Components|Blackboard|SetValueasBool (AI|GetBlackboard (AI|GetAIController self)) (Utilities|Name|MakeLiteralName "IsJumping?") true)
  (AI|Components|Blackboard|SetValueasBool (AI|GetBlackboard (AI|GetAIController self)) (Utilities|Name|MakeLiteralName "IsInIdle?") true)
  (AI|Components|Blackboard|SetValueasBool (AI|GetBlackboard (AI|GetAIController self)) (Utilities|Name|MakeLiteralName "IsAttacking?") true)
  (AI|Components|Blackboard|SetValueasBool (AI|GetBlackboard (AI|GetAIController self)) (Utilities|Name|MakeLiteralName "IsDespawning?") true)
  (AI|Components|Blackboard|SetValueasBool (AI|GetBlackboard (AI|GetAIController self)) (Utilities|Name|MakeLiteralName "IsTryingToGrabPlayer?") true)
  (AI|Components|Blackboard|SetValueasBool (AI|GetBlackboard (AI|GetAIController self)) (Utilities|Name|MakeLiteralName "IsFollowingPlayer?") false)
  (Variables|CharacterStates|SetIsFollowingPlayer? true)
  (return))

(fn SetIsAttackingPlayer
  (AI|Components|Blackboard|SetValueasBool (AI|GetBlackboard (AI|GetAIController self)) (Utilities|Name|MakeLiteralName "IsInIdle?") true)
  (AI|Components|Blackboard|SetValueasBool (AI|GetBlackboard (AI|GetAIController self)) (Utilities|Name|MakeLiteralName "IsJumping?") true)
  (AI|Components|Blackboard|SetValueasBool (AI|GetBlackboard (AI|GetAIController self)) (Utilities|Name|MakeLiteralName "IsFollowingPlayer?") true)
  (AI|Components|Blackboard|SetValueasBool (AI|GetBlackboard (AI|GetAIController self)) (Utilities|Name|MakeLiteralName "IsDespawning?") true)
  (AI|Components|Blackboard|SetValueasBool (AI|GetBlackboard (AI|GetAIController self)) (Utilities|Name|MakeLiteralName "IsTryingToGrabPlayer?") true)
  (AI|Components|Blackboard|SetValueasBool (AI|GetBlackboard (AI|GetAIController self)) (Utilities|Name|MakeLiteralName "IsAttacking?") false)
  (return))

(fn SetIsJumping
  (AI|Components|Blackboard|SetValueasBool (AI|GetBlackboard (AI|GetAIController self)) (Utilities|Name|MakeLiteralName "IsFollowingPlayer?") true)
  (AI|Components|Blackboard|SetValueasBool (AI|GetBlackboard (AI|GetAIController self)) (Utilities|Name|MakeLiteralName "IsInIdle?") true)
  (AI|Components|Blackboard|SetValueasBool (AI|GetBlackboard (AI|GetAIController self)) (Utilities|Name|MakeLiteralName "IsAttacking?") true)
  (AI|Components|Blackboard|SetValueasBool (AI|GetBlackboard (AI|GetAIController self)) (Utilities|Name|MakeLiteralName "IsJumping?") false)
  (return))

(fn SetShinyColor
  (if (or (== (Math|Random|RandomIntegerinRange 0 4095) 4095) (Variables|/Game/Managers/GI_HelpingHand.GI_HelpingHand_C|GetCanSpawnShiny (CallFunction|GetGameInstance)))
    (Rendering|Material|SetMaterial (Variables|Character|GetMesh) 0 "/Game/Asset_Cucina/M_Master_ShinyMonster.M_Master_ShinyMonster")
    (Components|Activation|Activate (Variables|Default|GetNiagara) false)
    (Variables|/Game/Managers/GI_HelpingHand.GI_HelpingHand_C|SetCanSpawnShiny (CallFunction|GetGameInstance) false)))

(fn SetIsDespawning
  (AI|Components|Blackboard|SetValueasBool (AI|GetBlackboard (AI|GetAIController self)) (Utilities|Name|MakeLiteralName "IsInIdle?") true)
  (AI|Components|Blackboard|SetValueasBool (AI|GetBlackboard (AI|GetAIController self)) (Utilities|Name|MakeLiteralName "IsJumping?") true)
  (AI|Components|Blackboard|SetValueasBool (AI|GetBlackboard (AI|GetAIController self)) (Utilities|Name|MakeLiteralName "IsFollowingPlayer?") true)
  (AI|Components|Blackboard|SetValueasBool (AI|GetBlackboard (AI|GetAIController self)) (Utilities|Name|MakeLiteralName "IsAttacking?") true)
  (AI|Components|Blackboard|SetValueasBool (AI|GetBlackboard (AI|GetAIController self)) (Utilities|Name|MakeLiteralName "IsTryingToGrabPlayer?") true)
  (AI|Components|Blackboard|SetValueasBool (AI|GetBlackboard (AI|GetAIController self)) (Utilities|Name|MakeLiteralName "IsDespawning?") false)
  (return))

(fn SetIsGrabbingPlayer
  (AI|Components|Blackboard|SetValueasBool (AI|GetBlackboard (AI|GetAIController self)) (Utilities|Name|MakeLiteralName "IsInIdle?") true)
  (AI|Components|Blackboard|SetValueasBool (AI|GetBlackboard (AI|GetAIController self)) (Utilities|Name|MakeLiteralName "IsJumping?") true)
  (AI|Components|Blackboard|SetValueasBool (AI|GetBlackboard (AI|GetAIController self)) (Utilities|Name|MakeLiteralName "IsFollowingPlayer?") true)
  (AI|Components|Blackboard|SetValueasBool (AI|GetBlackboard (AI|GetAIController self)) (Utilities|Name|MakeLiteralName "IsAttacking?") true)
  (AI|Components|Blackboard|SetValueasBool (AI|GetBlackboard (AI|GetAIController self)) (Utilities|Name|MakeLiteralName "IsDespawning?") true)
  (AI|Components|Blackboard|SetValueasBool (AI|GetBlackboard (AI|GetAIController self)) (Utilities|Name|MakeLiteralName "IsTryingToGrabPlayer?") false)
  (return))