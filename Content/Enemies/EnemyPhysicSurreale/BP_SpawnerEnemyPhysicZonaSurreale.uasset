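; Trigger volume in the surreal zone that stages an encounter with the giant physics monster (BP_PhysicMonsterGigante) when the player, BP_PG3, enters its box.
; Rather than spawning, it fires once to reveal and teleport the level's existing monster, briefly making its capsule Movable.
; It passes the monster an attack delay, player respawn data and one attack type, picked by priority from four flags.
; ReplayAnim re-arms the trigger.
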(event OnComponentBeginOverlap(Box)
  (params (OverlappedComponent :type Primitive%20Component%20Object%20Reference) (OtherActor :type Actor%20Object%20Reference) (OtherComp :type Primitive%20Component%20Object%20Reference) (OtherBodyIndex :type Integer) (bFromSweep :type Boolean) (SweepResult :type Hit%20Result%20Structure%20%28by%20ref%29))
  (bind _physicmonstergigante (Variables|Default|GetPhysicMonsterGigante))
  ;[1 1 1] Overlap with PG3
  (Utilities|Casting|CastToBP_PG3 OtherActor)
  (Utilities|FlowControl|DoOnce false
    (:Completed
      (Default|SetMeshVisible _physicmonstergigante (Variables|Default|GetVisibilityDelayDelay))
      (Transformation|SetMobility (Variables|/Script/Engine.Character|GetCapsuleComponent _physicmonstergigante) "Movable")
      (Transformation|SetActorLocationAndRotation _physicmonstergigante (Variables|Default|GetPhysicMonsterGiganteNewLocation) (Variables|Default|GetPhysicMonsterGiganteNewRotation) false true)
      (Variables|/Game/Enemies/EnemyPhysicSurreale/BP_PhysicMonsterGigante.BP_PhysicMonsterGigante_C|SetDelayAttack _physicmonstergigante (Variables|Default|GetDelay%20Attack))
      (Transformation|SetMobility (Variables|/Script/Engine.Character|GetCapsuleComponent _physicmonstergigante) "Static")
      (CallFunction|CheckMonsterGiganteAttack)
      (Variables|/Game/Enemies/EnemyPhysicSurreale/BP_PhysicMonsterGigante.BP_PhysicMonsterGigante_C|SetForced%20Teleport%20Where%20to%20Respawn _physicmonstergigante (Variables|Default|GetForced%20Teleport%20Where%20To%20Respawn))
      (Variables|/Game/Enemies/EnemyPhysicSurreale/BP_PhysicMonsterGigante.BP_PhysicMonsterGigante_C|SetPG3Location _physicmonstergigante (Variables|PG3|GetNewPG3Location))
      (Variables|/Game/Enemies/EnemyPhysicSurreale/BP_PhysicMonsterGigante.BP_PhysicMonsterGigante_C|SetPG3Rotation _physicmonstergigante (Variables|PG3|GetNewPG3Rotation)))))

(event Custom|ReplayAnim
  (bind _physicmonstergigante (Variables|Default|GetPhysicMonsterGigante))
  ;[1 1 1] Overlap with PG3
  (Utilities|FlowControl|DoOnce false) ; enters at Reset
)

(event EventBeginPlay
  ;[1 1 1] Intialize
  (bind _returnvalue (Actor|GetActorOfClass "/Game/Enemies/EnemyPhysicSurreale/BP_PhysicMonsterGigante.BP_PhysicMonsterGigante_C"))
  (Variables|Default|SetPhysicMonsterGigante _returnvalue)
  (bind _pg3 (CallFunction|GetPlayer3))
  (Variables|PG3|SetPG3 _pg3))

(fn ConstructionScript)

(fn CheckMonsterGiganteAttack
  (bind _physicmonstergigante (Variables|Default|GetPhysicMonsterGigante))
  (bind _physicmonstergigante_2 (Variables|Default|GetPhysicMonsterGigante))
  (bind _physicmonstergigante_3 (Variables|Default|GetPhysicMonsterGigante))
  (bind _physicmonstergigante_4 (Variables|Default|GetPhysicMonsterGigante))
  (if (Variables|Default|GetMustPhysicMonsterGiganteAttackWithLeftHand?)
    (Variables|/Game/Enemies/EnemyPhysicSurreale/BP_PhysicMonsterGigante.BP_PhysicMonsterGigante_C|SetMustAttackWithLeftHand? _physicmonstergigante_2 true)
    (Variables|/Game/Enemies/EnemyPhysicSurreale/BP_PhysicMonsterGigante.BP_PhysicMonsterGigante_C|SetMustAttackWithRightHand? _physicmonstergigante_2 false)
    (Variables|/Game/Enemies/EnemyPhysicSurreale/BP_PhysicMonsterGigante.BP_PhysicMonsterGigante_C|SetMustAttackWithBite? _physicmonstergigante_2 false)
    (Variables|/Game/Enemies/EnemyPhysicSurreale/BP_PhysicMonsterGigante.BP_PhysicMonsterGigante_C|SetMustTryToGrabPlayer? _physicmonstergigante_2 false)
    (elif (Variables|Default|GetMustPhysicMonsterGiganteAttackRigtHand?)
      (Variables|/Game/Enemies/EnemyPhysicSurreale/BP_PhysicMonsterGigante.BP_PhysicMonsterGigante_C|SetMustAttackWithRightHand? _physicmonstergigante_3 true)
      (Variables|/Game/Enemies/EnemyPhysicSurreale/BP_PhysicMonsterGigante.BP_PhysicMonsterGigante_C|SetMustAttackWithBite? _physicmonstergigante_3 false)
      (Variables|/Game/Enemies/EnemyPhysicSurreale/BP_PhysicMonsterGigante.BP_PhysicMonsterGigante_C|SetMustTryToGrabPlayer? _physicmonstergigante_3 false)
      (Variables|/Game/Enemies/EnemyPhysicSurreale/BP_PhysicMonsterGigante.BP_PhysicMonsterGigante_C|SetMustAttackWithLeftHand? _physicmonstergigante_3 false)
      (elif (Variables|Default|GetMustPhysicMonsterGiganteAttackWithBite?)
        (Variables|/Game/Enemies/EnemyPhysicSurreale/BP_PhysicMonsterGigante.BP_PhysicMonsterGigante_C|SetMustAttackWithBite? _physicmonstergigante_4 true)
        (Variables|/Game/Enemies/EnemyPhysicSurreale/BP_PhysicMonsterGigante.BP_PhysicMonsterGigante_C|SetMustAttackWithRightHand? _physicmonstergigante_4 false)
        (Variables|/Game/Enemies/EnemyPhysicSurreale/BP_PhysicMonsterGigante.BP_PhysicMonsterGigante_C|SetMustTryToGrabPlayer? _physicmonstergigante_4 false)
        (Variables|/Game/Enemies/EnemyPhysicSurreale/BP_PhysicMonsterGigante.BP_PhysicMonsterGigante_C|SetMustAttackWithLeftHand? _physicmonstergigante_4 false)
        (elif (Variables|Default|GetMustPhysicMonsterGiganteTryToGrabPlayer?)
          (Variables|/Game/Enemies/EnemyPhysicSurreale/BP_PhysicMonsterGigante.BP_PhysicMonsterGigante_C|SetMustAttackWithBite? _physicmonstergigante false)
          (Variables|/Game/Enemies/EnemyPhysicSurreale/BP_PhysicMonsterGigante.BP_PhysicMonsterGigante_C|SetMustAttackWithRightHand? _physicmonstergigante false)
          (Variables|/Game/Enemies/EnemyPhysicSurreale/BP_PhysicMonsterGigante.BP_PhysicMonsterGigante_C|SetMustTryToGrabPlayer? _physicmonstergigante true)
          (Variables|/Game/Enemies/EnemyPhysicSurreale/BP_PhysicMonsterGigante.BP_PhysicMonsterGigante_C|SetMustAttackWithLeftHand? _physicmonstergigante false)
          (else
            (return))))))
  (return))