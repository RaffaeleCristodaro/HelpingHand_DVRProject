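; Giant surreal physics monster enemy that kills player 3 on contact with its right arm.
; A capsule snapped to the right elbow socket triggers a guarded kill on overlap, respawning players through the GameManager and resetting the monster to its start position.
; It hides and teleports there after a BeginPlay delay, exposes visibility events and a blackboard state setter, and has a 1-in-4096 shiny material roll.
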(event OnComponentBeginOverlap(Capsule)
  (params (OverlappedComponent :type Primitive%20Component%20Object%20Reference) (OtherActor :type Actor%20Object%20Reference) (OtherComp :type Primitive%20Component%20Object%20Reference) (OtherBodyIndex :type Integer) (bFromSweep :type Boolean) (SweepResult :type Hit%20Result%20Structure%20%28by%20ref%29))
  ;[1 1 1] Collision with right hand
  (bind _asbp_pg3 (Utilities|Casting|CastToBP_PG3 OtherActor))
  (Utilities|FlowControl|DoOnce false :!label _label
    (:Completed
      (Variables|/Game/PG3/BP_PG3.BP_PG3_C|SetIsDying? _asbp_pg3 true)
      (Default|RespawnPlayers (Variables|Default|GetGame%20Manager) (Variables|RespawnPlayers|GetForced%20Teleport%20Where%20to%20Respawn) (Variables|RespawnPlayers|GetTeleport%20Where%20to%20Respawn) (Variables|RespawnPlayers|GetPG3Location) (Variables|RespawnPlayers|GetPG3Rotation))
      (Utilities|FlowControl|Delay 2.0)
      (Variables|/Game/PG3/BP_PG3.BP_PG3_C|SetIsDying? (Variables|Default|GetPG3) false)
      (Transformation|SetActorLocation (Variables|RespawnPlayers|GetMosterStartingPos) false true)
      (goto _label Reset))))

(event Custom|SetMeshVisible
  (params (Delay :type Float%20%28double-precision%29))
  ;[1 1 1] Mesh visibility
  (Utilities|FlowControl|Delay Delay)
  (Rendering|SetVisibility (Variables|Character|GetMesh) true false))

(event Custom|SetMeshInvisible
  (params (delay :type Float%20%28double-precision%29))
  ;[1 1 1] Mesh visibility
  (Utilities|FlowControl|Delay delay)
  (Rendering|SetVisibility (Variables|Character|GetMesh) false false)
  (Transformation|SetActorLocation (Variables|RespawnPlayers|GetMosterStartingPos) false true))

(event EventBeginPlay
  ;[1 1 1] Initialize
  (CallFunction|SetShinyColor)
  (bind _gamemanager (CallFunction|GetGameManager))
  (Variables|Default|SetGame%20Manager _gamemanager)
  (bind _pg3 (CallFunction|GetPlayer3))
  (Variables|Default|SetPG3 _pg3)
  (CallFunction|SetMeshInvisible (Variables|RespawnPlayers|GetDelayAttack)))

(fn ConstructionScript
  (Transformation|AttachComponentToComponent (Variables|Components|GetCapsule) (Variables|Character|GetMesh) "Elbow_RSocket" "SnapToTarget" "KeepRelative" "KeepRelative" true))

(fn SetIsJumping
  (AI|Components|Blackboard|SetValueasBool (AI|GetBlackboard (AI|GetAIController self)) (Utilities|Name|MakeLiteralName "IsFollowingPlayer?") true)
  (AI|Components|Blackboard|SetValueasBool (AI|GetBlackboard (AI|GetAIController self)) (Utilities|Name|MakeLiteralName "IsInIdle?") true)
  (AI|Components|Blackboard|SetValueasBool (AI|GetBlackboard (AI|GetAIController self)) (Utilities|Name|MakeLiteralName "IsAttacking?") true)
  (AI|Components|Blackboard|SetValueasBool (AI|GetBlackboard (AI|GetAIController self)) (Utilities|Name|MakeLiteralName "IsJumping?") false)
  (return))

(fn SetShinyColor
  (if (== (Math|Random|RandomIntegerinRange 0 4095) 4095)
    (Rendering|Material|SetMaterial (Variables|Character|GetMesh) 0 "/Game/Asset_Cucina/M_Master_ShinyMonster.M_Master_ShinyMonster"))
  (return))