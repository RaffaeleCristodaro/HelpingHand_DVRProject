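; VR pinball machine for the game room, played by physically pressing its start and flipper buttons.
; Tick polls the VR pawn's overlap with each button to slide it, rotate flippers, or briefly drop the start bar and reset the ball.
; Hits on a flipper while its button is held apply an impulse to the ball, throttled by DoOnce delays.
; Bumper hits add and print score, and a drain trigger teleports the ball to its spawn point.
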(event OnComponentBeginOverlap(RespawnBallArea)
  (params (OverlappedComponent :type Primitive%20Component%20Object%20Reference) (OtherActor :type Actor%20Object%20Reference) (OtherComp :type Primitive%20Component%20Object%20Reference) (OtherBodyIndex :type Integer) (bFromSweep :type Boolean) (SweepResult :type Hit%20Result%20Structure%20%28by%20ref%29))
  (bind _flipperball (Variables|Default|GetFlipperBall))
  ;[1 1 1] Respawn ball
  (if (== OtherActor _flipperball)
    (Transformation|SetWorldLocation (Variables|/Game/Asset_SalaGiochi/BP/BP_FlipperBall.BP_FlipperBall_C|GetSphere _flipperball) (Transformation|GetWorldLocation (Variables|Default|GetRespawnBallScene)) false true)
    (Variables|ButtonStart|SetCanStartBarGoDown? true)))

(event OnComponentHit(Fungis1)
  (params (HitComponent :type Primitive%20Component%20Object%20Reference) (OtherActor :type Actor%20Object%20Reference) (OtherComp :type Primitive%20Component%20Object%20Reference) (NormalImpulse :type Vector :default "0, 0, 0") (Hit :type Hit%20Result%20Structure%20%28by%20ref%29))
  ;[1 1 1] Score
  (CallFunction|FlipperAddScoreEvent OtherActor 1.0))

(event OnComponentHit(RightFlipper)
  (params (HitComponent :type Primitive%20Component%20Object%20Reference) (OtherActor :type Actor%20Object%20Reference) (OtherComp :type Primitive%20Component%20Object%20Reference) (NormalImpulse :type Vector :default "0, 0, 0") (Hit :type Hit%20Result%20Structure%20%28by%20ref%29))
  ;[1 1 1] Apply force when hitting ball
  (if (Variables|ForceToApply|GetCanApplyForceRight?)
    (Utilities|FlowControl|DoOnce false :!label _label
      (:Completed
        (Physics|AddImpulse (Variables|/Game/Asset_SalaGiochi/BP/BP_FlipperBall.BP_FlipperBall_C|GetSphere (Variables|Default|GetFlipperBall)) (Variables|ForceToApply|GetImpulse) "None" false)
        (Utilities|FlowControl|Delay (Variables|Levette|GetFlipperHitDelay))
        (goto _label Reset)))))

(event OnComponentHit(LeftFlipper)
  (params (HitComponent :type Primitive%20Component%20Object%20Reference) (OtherActor :type Actor%20Object%20Reference) (OtherComp :type Primitive%20Component%20Object%20Reference) (NormalImpulse :type Vector :default "0, 0, 0") (Hit :type Hit%20Result%20Structure%20%28by%20ref%29))
  ;[1 1 1] Apply force when hitting ball
  (if (Variables|ForceToApply|GetCanApplyForceLeft?)
    (Utilities|FlowControl|DoOnce false :!label _label
      (:Completed
        (Physics|AddImpulse (Variables|/Game/Asset_SalaGiochi/BP/BP_FlipperBall.BP_FlipperBall_C|GetSphere (Variables|Default|GetFlipperBall)) (Variables|ForceToApply|GetImpulse) "None" false)
        (Utilities|FlowControl|Delay (Variables|Levette|GetFlipperHitDelay))
        (goto _label Reset)))))

(event OnComponentHit(Fungis)
  (params (HitComponent :type Primitive%20Component%20Object%20Reference) (OtherActor :type Actor%20Object%20Reference) (OtherComp :type Primitive%20Component%20Object%20Reference) (NormalImpulse :type Vector :default "0, 0, 0") (Hit :type Hit%20Result%20Structure%20%28by%20ref%29))
  ;[1 1 1] Score
  (CallFunction|FlipperAddScoreEvent OtherActor 1.0))

(event OnComponentHit(Fungis2)
  (params (HitComponent :type Primitive%20Component%20Object%20Reference) (OtherActor :type Actor%20Object%20Reference) (OtherComp :type Primitive%20Component%20Object%20Reference) (NormalImpulse :type Vector :default "0, 0, 0") (Hit :type Hit%20Result%20Structure%20%28by%20ref%29))
  ;[1 1 1] Score
  (CallFunction|FlipperAddScoreEvent OtherActor 1.0))

(event Custom|FlipperAddScoreEvent
  (params (HitActor :type Actor%20Object%20Reference) (Delay :type Float%20%28double-precision%29))
  ;[1 1 1] Score
  (Utilities|Casting|CastToBP_FlipperBall HitActor)
  (Utilities|FlowControl|DoOnce false :!label _label
    (:Completed
      (bind _output_get (Variables|Score|SetCurrentScore (+ (Variables|Score|GetCurrentScore) (Variables|Score|GetFungisAddScore))))
      (Development|PrintString (Utilities|String|ToString(Integer) _output_get))
      (Utilities|FlowControl|Delay Delay)
      (goto _label Reset))))

(event Custom|StartBarEvent
  (bind _startbutton (Variables|Default|GetStartButton))
  (bind _minoffsetbuttonstart (Variables|ButtonStart|GetMinOffsetButtonStart))
  (bind _maxoffsetbuttonstart (Variables|ButtonStart|GetMaxOffsetButtonStart))
  (bind _startbutton_2 (Variables|Default|GetStartButton))
  (bind _returnvalue (Transformation|GetRelativeTransform _startbutton))
  (bind _returnvalue_2 (Transformation|GetRelativeTransform _startbutton_2))
  (bind _returnvalue_3 (+ (.location _returnvalue_2) "3.000000,0.000000,0.000000"))
  (bind _returnvalue_4 (- (.location _returnvalue) "3.000000,0.000000,0.000000"))
  (bind _returnvalue_5 (Math|Float|Clamp(Float) (.x _returnvalue_3) _minoffsetbuttonstart _maxoffsetbuttonstart))
  ;[1 1 1] Start bar
  (if (Collision|IsOverlappingActor (Variables|Default|GetStartButtonCollision) (Default|GetVRPawnRef (CallFunction|GetGameMode)) :!class /Script/Engine.PrimitiveComponent)
    (Components|MoveComponentTo _startbutton_2 (Math|Vector|MakeVector _returnvalue_5 (.y _returnvalue_3) (.z _returnvalue_3)) (.rotation _returnvalue_2) false true (Variables|Default|GetOver%20Time) false)
    (if (<= _returnvalue_5 (Variables|ButtonStart|GetMaxOffsetButtonStart))
      (Utilities|FlowControl|DoOnce false
        (:Completed
          (CallFunction|SetBarDown))))
    (elif (not (<= (.x (.location (Transformation|GetRelativeTransform (Variables|Default|GetStartButton)))) (Variables|ButtonStart|GetMinOffsetButtonStart)))
      (Components|MoveComponentTo _startbutton (Math|Vector|MakeVector (Math|Float|Clamp(Float) (.x _returnvalue_4) (Variables|ButtonStart|GetMinOffsetButtonStart) (Variables|ButtonStart|GetMaxOffsetButtonStart)) (.y _returnvalue_4) (.z _returnvalue_4)) (.rotation _returnvalue) false true (Variables|Default|GetOver%20Time) false))))

(event Custom|RightButtonEvent
  (bind _rightbutton (Variables|Default|GetRightButton))
  (bind _rightbutton_2 (Variables|Default|GetRightButton))
  (bind _rightflipper (Variables|Default|GetRightFlipper))
  (bind _rightflipper_2 (Variables|Default|GetRightFlipper))
  (bind _returnvalue (Transformation|GetRelativeTransform _rightbutton))
  (bind _returnvalue_2 (Transformation|GetRelativeTransform _rightbutton_2))
  (bind _returnvalue_3 (- (.location _returnvalue) "0.000000,3.000000,0.000000"))
  (bind _returnvalue_4 (+ (.location _returnvalue_2) "0.000000,3.000000,0.000000"))
  ;[1 1 1] Right button
  (if (Collision|IsOverlappingActor (Variables|Default|GetRightButtonCollision) (Default|GetVRPawnRef (CallFunction|GetGameMode)) :!class /Script/Engine.PrimitiveComponent)
    (Variables|ForceToApply|SetCanApplyForceRight? true)
    (Utilities|FlowControl|Sequence
      (:then_0
        (Components|MoveComponentTo _rightbutton (Math|Vector|MakeVector (.x _returnvalue_3) (Math|Float|Clamp(Float) (.y _returnvalue_3) (Variables|Levette|GetMinOffsetButtonLevettaRight) (Variables|Levette|GetMaxOffsetButtonLevettaRight)) (.z _returnvalue_3)) (.rotation _returnvalue) false true (Variables|Default|GetOver%20Time) false))
      (:then_1
        (Components|MoveComponentTo _rightflipper (Variables|/Script/Engine.SceneComponent|GetRelativeLocation _rightflipper) (Variables|Levette|GetLevettaRightPressedRotation) false true (Variables|Default|GetOver%20Time) false)))
    (else
      (Variables|ForceToApply|SetCanApplyForceRight? false)
      (if (>= (.y (.location (Transformation|GetRelativeTransform (Variables|Default|GetRightButton)))) (Variables|Levette|GetMinOffsetButtonLevettaRight))
        (Utilities|FlowControl|Sequence
          (:then_0
            (Components|MoveComponentTo _rightbutton_2 (Math|Vector|MakeVector (.x _returnvalue_4) (Math|Float|Clamp(Float) (.y _returnvalue_4) (Variables|Levette|GetMinOffsetButtonLevettaRight) (Variables|Levette|GetMaxOffsetButtonLevettaRight)) (.z _returnvalue_4)) (.rotation _returnvalue_2) false true (Variables|Default|GetOver%20Time) false))
          (:then_1
            (Components|MoveComponentTo _rightflipper_2 (Variables|/Script/Engine.SceneComponent|GetRelativeLocation _rightflipper_2) (Variables|Levette|GetLevettaRighReleasedRotation) false true (Variables|Default|GetOver%20Time) false)))))))

(event Custom|SetBarDown
  ;[1 1 1] Start bar
  (Transformation|SetRelativeLocation (Variables|Default|GetStartBar) (Variables|ButtonStart|GetStartBarFinalTransform) false false)
  (Transformation|SetWorldLocation (Variables|/Game/Asset_SalaGiochi/BP/BP_FlipperBall.BP_FlipperBall_C|GetSphere (Variables|Default|GetFlipperBall)) (Transformation|GetWorldLocation (Variables|Default|GetRespawnBallScene)) false true)
  (Utilities|FlowControl|Delay (Variables|ButtonStart|GetDelayStartBarRespawn))
  (Transformation|SetRelativeLocation (Variables|Default|GetStartBar) (Variables|ButtonStart|GetStartBarInitialTransform) false false)
  (Utilities|FlowControl|DoOnce false) ; enters at Reset
)

(event Custom|LeftButtonEvent
  (bind _leftbutton (Variables|Default|GetLeftButton))
  (bind _leftflipper (Variables|Default|GetLeftFlipper))
  (bind _leftbutton_2 (Variables|Default|GetLeftButton))
  (bind _leftflipper_2 (Variables|Default|GetLeftFlipper))
  (bind _returnvalue (Transformation|GetRelativeTransform _leftbutton_2))
  (bind _returnvalue_2 (Transformation|GetRelativeTransform _leftbutton))
  (bind _returnvalue_3 (- (.location _returnvalue_2) "0.000000,3.000000,0.000000"))
  (bind _returnvalue_4 (+ (.location _returnvalue) "0.000000,3.000000,0.000000"))
  ;[1 1 1] Left button
  (if (Collision|IsOverlappingActor (Variables|Default|GetLeftButtonCollision) (Default|GetVRPawnRef (CallFunction|GetGameMode)) :!class /Script/Engine.PrimitiveComponent)
    (Variables|ForceToApply|SetCanApplyForceLeft? true)
    (Utilities|FlowControl|Sequence
      (:then_0
        (Components|MoveComponentTo _leftbutton_2 (Math|Vector|MakeVector (.x _returnvalue_4) (Math|Float|Clamp(Float) (.y _returnvalue_4) (Variables|Levette|GetMinOffsetButtonLevettaLeft) (Variables|Levette|GetMaxOffsetButtonLevettaLeft)) (.z _returnvalue_4)) (.rotation _returnvalue) false true (Variables|Default|GetOver%20Time) false))
      (:then_1
        (Components|MoveComponentTo _leftflipper (Variables|/Script/Engine.SceneComponent|GetRelativeLocation _leftflipper) (Variables|Levette|GetLevettaLeftPressedRotation) false true (Variables|Default|GetOver%20Time) false)))
    (else
      (Variables|ForceToApply|SetCanApplyForceLeft? false)
      (if (>= (.y (.location (Transformation|GetRelativeTransform (Variables|Default|GetLeftButton)))) (Variables|Levette|GetMinOffsetButtonLevettaLeft))
        (Utilities|FlowControl|Sequence
          (:then_0
            (Components|MoveComponentTo _leftbutton (Math|Vector|MakeVector (.x _returnvalue_3) (Math|Float|Clamp(Float) (.y _returnvalue_3) (Variables|Levette|GetMinOffsetButtonLevettaLeft) (Variables|Levette|GetMaxOffsetButtonLevettaLeft)) (.z _returnvalue_3)) (.rotation _returnvalue_2) false true (Variables|Default|GetOver%20Time) false))
          (:then_1
            (Components|MoveComponentTo _leftflipper_2 (Variables|/Script/Engine.SceneComponent|GetRelativeLocation _leftflipper_2) (Variables|Levette|GetLevettaLeftReleasedRotation) false true (Variables|Default|GetOver%20Time) false)))))))

(event EventTick
  (params (DeltaSeconds :type Float%20%28single-precision%29))
  ;[0.5521 0.02147 0.05995] Event tick
  (CallFunction|StartBarEvent)
  (CallFunction|LeftButtonEvent)
  (CallFunction|RightButtonEvent))

(fn ConstructionScript)