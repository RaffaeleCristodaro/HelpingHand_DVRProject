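; Safe Blueprint for the game room that validates an entered code sequence against a stored password.
; CheckPassword compares both arrays position by position, sets IsCorrectPassword when the match count reaches the password length, and clears the entry either way.
; The match counter is not reset within the function, so matches accumulate across attempts unless reset elsewhere.
; SetNumbersOnDisplay and the construction script are empty stubs.
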(fn ConstructionScript)

(fn CheckPassword
  (for (_array_element _array_index) (Variables|Password|GetPasswordSequence)
    (if (== _array_element (Utilities|Array|Get(acopy) (Variables|Password|GetCurrentPasswordSequence) _array_index))
      (Math|Integer|IncrementInt (LocalVariables|GetIntSimilarity))))
  (if (>= (LocalVariables|GetIntSimilarity) (Utilities|Array|Length (Variables|Password|GetPasswordSequence)))
    (Variables|Password|SetIsCorrectPassword true)
    (Utilities|Array|Clear (Variables|Password|GetCurrentPasswordSequence))
    (else
      (Utilities|Array|Clear (Variables|Password|GetCurrentPasswordSequence)))))

(fn SetNumbersonDisplay)