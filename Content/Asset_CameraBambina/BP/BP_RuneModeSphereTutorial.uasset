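; Grabbable VR tutorial sphere that switches Player 1 into the rune mode tutorial when first picked up.
; A hand or telekinesis grab fires once, hiding the sphere, disabling its collision, flagging the tutorial, activating rune Niagara VFX and releasing the held hand.
; A separate event plays Player 3's fire-achievement montage, then clears its surprised state.
; BeginPlay caches both players and initial transforms.
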(event OnGrabbed(GrabComponent)
  (bind _pg1 (Variables|Default|GetPG1))
  ;[1 1 1] On Grabbed
  (Utilities|FlowControl|DoOnce false
    (:Completed
      (Development|SetHiddeninGame (Variables|Default|GetSphere) true false)
      (Collision|SetCollisionEnabled (Variables|Default|GetSphere) "NoCollision")
      (Variables|/Game/VRTemplate/Blueprints/VRPawn.VRPawn_C|SetIsRuneModeTutorial? (Variables|Default|GetPG1) true)
      (Components|Activation|Activate (Variables|Default|GetNiagaraSpawnRune) false)
      (if (== (Variables|/Game/VRTemplate/Blueprints/VRPawn.VRPawn_C|GetHeldComponentLeft _pg1) (Variables|Default|GetGrabComponent))
        (Default|TryRelease (Variables|Default|GetGrabComponent) (Variables|/Game/VRTemplate/Blueprints/VRPawn.VRPawn_C|GetMotionControllerLeft _pg1))
        (Variables|/Game/VRTemplate/Blueprints/VRPawn.VRPawn_C|SetHeldComponentLeft _pg1 0)
        (else
          (Default|TryRelease (Variables|Default|GetGrabComponent) (Variables|/Game/VRTemplate/Blueprints/VRPawn.VRPawn_C|GetMotionControllerRight _pg1))
          (Variables|/Game/VRTemplate/Blueprints/VRPawn.VRPawn_C|SetHeldComponentRight _pg1 0))))))

(event Custom|TutorialAnimationFirstTimeRuneFire
  ;[1 1 1] Tutorial anim
  (bind _returnvalue (Animation|PlayAnimMontage (Variables|Default|GetPG3) "/Game/PG3/PG3_Animations/PG_Fire_Achive_Montage.PG_Fire_Achive_Montage" 1.0 "None"))
  (Utilities|FlowControl|Delay _returnvalue)
  (Animation|StopAnimMontage (Variables|Default|GetPG3) "/Game/PG3/PG3_Animations/PG_Fire_Achive_Montage.PG_Fire_Achive_Montage")
  (Variables|/Game/PG3/BP_PG3.BP_PG3_C|SetIsSurprised? (Variables|Default|GetPG3) false))

(event Custom|TelekynesisGrab
  (bind _pg1 (Variables|Default|GetPG1))
  ;[1 1 1] On Grabbed
  (Utilities|FlowControl|DoOnce false
    (:Completed
      (Development|SetHiddeninGame (Variables|Default|GetSphere) true false)
      (Collision|SetCollisionEnabled (Variables|Default|GetSphere) "NoCollision")
      (Variables|/Game/VRTemplate/Blueprints/VRPawn.VRPawn_C|SetIsRuneModeTutorial? (Variables|Default|GetPG1) true)
      (Components|Activation|Activate (Variables|Default|GetNiagaraSpawnRune) false)
      (if (== (Variables|/Game/VRTemplate/Blueprints/VRPawn.VRPawn_C|GetHeldComponentLeft _pg1) (Variables|Default|GetGrabComponent))
        (Default|TryRelease (Variables|Default|GetGrabComponent) (Variables|/Game/VRTemplate/Blueprints/VRPawn.VRPawn_C|GetMotionControllerLeft _pg1))
        (Variables|/Game/VRTemplate/Blueprints/VRPawn.VRPawn_C|SetHeldComponentLeft _pg1 0)
        (else
          (Default|TryRelease (Variables|Default|GetGrabComponent) (Variables|/Game/VRTemplate/Blueprints/VRPawn.VRPawn_C|GetMotionControllerRight _pg1))
          (Variables|/Game/VRTemplate/Blueprints/VRPawn.VRPawn_C|SetHeldComponentRight _pg1 0))))))

(event EventBeginPlay
  (bind _sphere (Variables|Default|GetSphere))
  ;[1 1 1] Initialize
  (bind _pg1 (CallFunction|GetPlayer1))
  (Variables|Default|SetPG1 _pg1)
  (bind _pg3 (CallFunction|GetPlayer3))
  (Variables|Default|SetPG3 _pg3)
  (Variables|Default|SetIntialScale (Transformation|GetWorldScale (Variables|Default|GetSphere)))
  (Variables|Default|SetActorStartLocation (Transformation|GetActorLocation))
  (Variables|Default|SetActorStartRotation (Transformation|GetActorRotation))
  (Variables|Default|SetSphereStartLocation (Transformation|GetWorldLocation _sphere))
  (Variables|Default|SetSphereStartRotation (Transformation|GetWorldRotation _sphere)))

(fn ConstructionScript)