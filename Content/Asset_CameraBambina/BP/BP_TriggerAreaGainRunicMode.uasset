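; BP_TriggerAreaGainRunicMode is a one-shot trigger volume that stages the runic mode tutorial moment for player PG3.
; It caches PG3 on BeginPlay, and PG3's first overlap with the box calls a forced-location event for PG1 on a linked teleport object.
; After a configurable delay it flags PG3 as surprised, then spawns the rune mode tutorial sphere and activates its Niagara spawn effect.
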(event OnComponentBeginOverlap(Box)
  (params (OverlappedComponent :type Primitive%20Component%20Object%20Reference) (OtherActor :type Actor%20Object%20Reference) (OtherComp :type Primitive%20Component%20Object%20Reference) (OtherBodyIndex :type Integer) (bFromSweep :type Boolean) (SweepResult :type Hit%20Result%20Structure%20%28by%20ref%29))
  ;[1 1 1] Overlap with PG3
  (if (== OtherActor (Variables|Default|GetPG3))
    (Utilities|FlowControl|DoOnce false
      (:Completed
        (Default|PG1ForcedLocationEvent (Variables|Default|GetForcedTeleportToMovePlayer))
        (Utilities|FlowControl|Delay (Variables|Default|GetDelaySpawnRuneMode))
        (Variables|/Game/PG3/BP_PG3.BP_PG3_C|SetIsSurprised? (Variables|Default|GetPG3) true)
        (bind _returnvalue (Game|SpawnActorfromClass "/Game/Asset_CameraBambina/BP/BP_RuneModeSphereTutorial.BP_RuneModeSphereTutorial_C" (Math|Transform|MakeTransform (Variables|Default|GetSpawnLocationFireRune) "0, 0, 0" "1.000000,1.000000,1.000000") "Undefined" 0 0))
        (Components|Activation|Activate (Variables|/Game/Asset_CameraBambina/BP/BP_RuneModeSphereTutorial.BP_RuneModeSphereTutorial_C|GetNiagaraSpawnSphere _returnvalue) false)))))

(event EventBeginPlay
  ;[1 1 1] Initialize
  (bind _pg3 (CallFunction|GetPlayer3))
  (Variables|Default|SetPG3 _pg3))

(fn ConstructionScript)