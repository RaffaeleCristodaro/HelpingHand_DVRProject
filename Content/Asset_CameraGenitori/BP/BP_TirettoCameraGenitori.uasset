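; VR drawer (tiretto) for the parents' bedroom that the player slides along the world Y axis with a motion controller.
; Tick finds which of Player 1's hands holds this actor and moves the mesh to that controller's offset Y, clamped between limits.
; A controller straying beyond the maximum grab distance triggers a forced release through the grab component.
; Both OnGrabbed and OnDropped set IsGrabbed true; only the forced release clears it.
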(event OnGrabbed(GrabComponent)
  ;[1 1 1] On Grabbed
  (Variables|TirettoRef|SetIsGrabbed? true))

(event OnDropped(GrabComponent)
  ;[1 1 1] On Grabbed
  (Variables|TirettoRef|SetIsGrabbed? true))

(event Custom|ReleaseTirettoEvent
  (bind _pg1 (Variables|Default|GetPG1))
  (bind _pg1_2 (Variables|Default|GetPG1))
  (bind _heldcomponentleft (Variables|/Game/VRTemplate/Blueprints/VRPawn.VRPawn_C|GetHeldComponentLeft _pg1))
  (bind _heldcomponentright (Variables|/Game/VRTemplate/Blueprints/VRPawn.VRPawn_C|GetHeldComponentRight _pg1_2))
  ;[1 1 1] Release
  (Utilities|IsValid _heldcomponentleft
    (:Is%20Valid
      (if (== (Components|GetOwner _heldcomponentleft) self)
        (Default|TryRelease (Variables|Default|GetGrabComponent) (Variables|/Game/VRTemplate/Blueprints/VRPawn.VRPawn_C|GetMotionControllerLeft (Variables|Default|GetPG1)))
        (Variables|TirettoRef|SetIsGrabbed? false)))
    (:Is%20Not%20Valid
      (Utilities|IsValid _heldcomponentright
        (:Is%20Valid
          (if (== (Components|GetOwner _heldcomponentright) self)
            (Default|TryRelease (Variables|Default|GetGrabComponent) (Variables|/Game/VRTemplate/Blueprints/VRPawn.VRPawn_C|GetMotionControllerRight (Variables|Default|GetPG1)))
            (Variables|TirettoRef|SetIsGrabbed? false)))))))

(event EventBeginPlay
  ;[1 1 1] Initialize
  (bind _pg1 (CallFunction|GetPlayer1))
  (Variables|Default|SetPG1 _pg1)
  (Variables|Default|SetInitialScale (Transformation|GetWorldScale (Variables|Default|GetStaticMesh))))

(event EventTick
  (params (DeltaSeconds :type Float%20%28single-precision%29))
  (bind _grabtreeshold (Variables|TirettoRef|GetGrabTreeshold))
  (bind _maxylocation (Variables|TirettoRef|GetMaxYlocation))
  (bind _minylocation (Variables|TirettoRef|GetMinYLocation))
  (bind _maxylocation_2 (Variables|TirettoRef|GetMaxYlocation))
  (bind _staticmesh (Variables|Default|GetStaticMesh))
  (bind _pg1 (Variables|Default|GetPG1))
  (bind _pg1_2 (Variables|Default|GetPG1))
  (bind _minylocation_2 (Variables|TirettoRef|GetMinYLocation))
  (bind _pg1_3 (Variables|Default|GetPG1))
  (bind _staticmesh_2 (Variables|Default|GetStaticMesh))
  (bind _pg1_4 (Variables|Default|GetPG1))
  (bind _grabtreeshold_2 (Variables|TirettoRef|GetGrabTreeshold))
  (bind _returnvalue (Transformation|GetWorldLocation _staticmesh))
  (bind _returnvalue_2 (Transformation|GetWorldLocation _staticmesh_2))
  (bind _heldcomponentleft (Variables|/Game/VRTemplate/Blueprints/VRPawn.VRPawn_C|GetHeldComponentLeft _pg1))
  (bind _heldcomponentright (Variables|/Game/VRTemplate/Blueprints/VRPawn.VRPawn_C|GetHeldComponentRight _pg1_2))
  (bind _motioncontrollerright (Variables|/Game/VRTemplate/Blueprints/VRPawn.VRPawn_C|GetMotionControllerRight _pg1_3))
  (bind _motioncontrollerleft (Variables|/Game/VRTemplate/Blueprints/VRPawn.VRPawn_C|GetMotionControllerLeft _pg1_4))
  (bind _returnvalue_3 (Transformation|GetWorldLocation _motioncontrollerleft))
  (bind _returnvalue_4 (Transformation|GetWorldLocation _motioncontrollerright))
  (bind _returnvalue_5 (- (.y _returnvalue_3) _grabtreeshold))
  (bind _returnvalue_6 (- (.y _returnvalue_4) _grabtreeshold_2))
  (bind _returnvalue_7 (Math|Float|Clamp(Float) _returnvalue_6 _minylocation_2 _maxylocation))
  (bind _returnvalue_8 (Math|Float|Clamp(Float) _returnvalue_5 _minylocation _maxylocation_2))
  ;[1 1 1] Event tick
  (if (Variables|TirettoRef|GetIsGrabbed?)
    (Utilities|IsValid _heldcomponentleft
      (:Is%20Valid
        (if (== (Components|GetOwner _heldcomponentleft) self)
          (if (Variables|TirettoRef|GetIsTesting?)
            (Development|PrintString (Utilities|String|ToString(Float) _returnvalue_8)))
          (Transformation|SetWorldLocation _staticmesh_2 (Math|Vector|MakeVector (.x _returnvalue_2) _returnvalue_8 (.z _returnvalue_2)) false false)
          (if (> (Math|Vector|Distance(Vector) (Transformation|GetWorldLocation (Variables|/Game/VRTemplate/Blueprints/VRPawn.VRPawn_C|GetMotionControllerLeft (Variables|Default|GetPG1))) (Transformation|GetWorldLocation (Variables|Default|GetStaticMesh))) (Variables|TirettoRef|GetMaxDistanceGrab))
            (CallFunction|ReleaseTirettoEvent))
          (else
            (Utilities|IsValid _heldcomponentright :!label _label
              (:Is%20Valid
                (if (== (Components|GetOwner _heldcomponentright) self)
                  (Development|PrintString "Hello")
                  (if (Variables|TirettoRef|GetIsTesting?)
                    (Development|PrintString (Utilities|String|ToString(Float) _returnvalue_7) true true "(R=1.000000,G=0.958813,B=0.000000,A=1.000000)"))
                  (Transformation|SetWorldLocation _staticmesh (Math|Vector|MakeVector (.x _returnvalue) _returnvalue_7 (.z _returnvalue)) false false)
                  (if (> (Math|Vector|Distance(Vector) (Transformation|GetWorldLocation (Variables|/Game/VRTemplate/Blueprints/VRPawn.VRPawn_C|GetMotionControllerRight (Variables|Default|GetPG1))) (Transformation|GetWorldLocation (Variables|Default|GetStaticMesh))) (Variables|TirettoRef|GetMaxDistanceGrab))
                    (CallFunction|ReleaseTirettoEvent))))))))
      (:Is%20Not%20Valid
        (goto _label)))))

(fn ConstructionScript)